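; BP_SplittingTool is a tool actor for the cataract removal part of an eye surgery game that slices BP_SliceMesh actors it touches.
; A static mesh overlap casts to BP_SliceMesh and calls CallSlice with a zero-location transform, rolled 90 degrees and yawed along the heading from that actor to the tool's Sphere.
; A DoOnce gate, reset by a short timer, rate-limits slicing and is consumed before the cast, so any overlap triggers the cooldown.
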(event OnComponentBeginOverlap(StaticMeshComponent)
  (params (OverlappedComponent :type Primitive%20Component%20Object%20Reference) (OtherActor :type Actor%20Object%20Reference) (OtherComp :type Primitive%20Component%20Object%20Reference) (OtherBodyIndex :type Integer) (bFromSweep :type Boolean) (SweepResult :type Hit%20Result%20Structure%20%28by%20ref%29))
  (Development|PrintString "Hello")
  (Utilities|FlowControl|DoOnce false
    (:Completed
      (Utilities|Time|SetTimerbyEvent (delegate Custom|EnableSliceAgain) 2.0)
      (bind _asbp_slice_mesh (Utilities|Casting|CastToBP_SliceMesh OtherActor))
      (Default|CallSlice (Math|Transform|MakeTransform "0, 0, 0" (Math|Rotator|MakeRotator 9e+01 0.0 (Math|Trig|RadiansToDegrees (Class|KismetMathLibrary|VectorHeadingAngle (- (Transformation|GetWorldLocation (Variables|Default|GetSphere)) (Transformation|GetActorLocation _asbp_slice_mesh))))))))))

(event Custom|EnableSliceAgain
  (Utilities|FlowControl|DoOnce false) ; enters at Reset
)

(event EventBeginPlay
  (|CallParentFunction) ; This node is disabled and will not be called.\nDrag off pins to build functionality.
)

(event Collision|EventActorBeginOverlap
  (params (OtherActor :type Actor%20Object%20Reference))
  (|CallParentFunction OtherActor) ; This node is disabled and will not be called.\nDrag off pins to build functionality.
)

(event EventTick
  (params (DeltaSeconds :type Float%20%28single-precision%29))
  (|CallParentFunction DeltaSeconds) ; This node is disabled and will not be called.\nDrag off pins to build functionality.
)

(fn ConstructionScript
  (|CallParentFunction))