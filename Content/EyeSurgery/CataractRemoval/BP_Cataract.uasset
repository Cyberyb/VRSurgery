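; BP_Cataract is a generated dynamic mesh actor representing the cataract in an eye surgery cataract removal game.
; On mesh rebuild it copies a static sphere into its dynamic mesh, applies PN tessellation and enables complex-as-simple collision.
; The ToSlicingMesh input spawns a BP_SliceMesh at its transform, passing it the mesh object, then destroys the actor.
; Component hit and overlap events only print debug strings.
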(event OnComponentHit(DynamicMeshComponent)
  (params (HitComponent :type Primitive%20Component%20Object%20Reference) (OtherActor :type Actor%20Object%20Reference) (OtherComp :type Primitive%20Component%20Object%20Reference) (NormalImpulse :type Vector :default "0, 0, 0") (Hit :type Hit%20Result%20Structure%20%28by%20ref%29))
  (Development|PrintString "Hello"))

(event OnComponentBeginOverlap(DynamicMeshComponent)
  (params (OverlappedComponent :type Primitive%20Component%20Object%20Reference) (OtherActor :type Actor%20Object%20Reference) (OtherComp :type Primitive%20Component%20Object%20Reference) (OtherBodyIndex :type Integer) (bFromSweep :type Boolean) (SweepResult :type Hit%20Result%20Structure%20%28by%20ref%29))
  (Development|PrintString "overlapping"))

(event EventBeginPlay)

(event Collision|EventActorBeginOverlap
  (params (OtherActor :type Actor%20Object%20Reference)))

(event EventTick
  (params (DeltaSeconds :type Float%20%28single-precision%29)))

(event Events|EventOnRebuildGeneratedMesh
  (params (TargetMesh :type Dynamic%20Mesh%20Object%20Reference))
  (Utilities|FlowControl|Sequence
    (:then_0
      (bind _returnvalue (DynamicMeshComponent|GetDynamicMesh (Variables|DynamicMeshActor|GetDynamicMeshComponent)))
      (Variables|Default|SetDynamicMeshObj _returnvalue))
    (:then_1
      (bind _returnvalue_2 (GeometryScript|StaticMesh|CopyMeshFromStaticMesh :FromStaticMeshAsset "/Engine/BasicShapes/Sphere.Sphere" :ToDynamicMesh (Variables|Default|GetDynamicMeshObj) :Debug 0)
        (:Success
          (Class|GeometryScriptLibraryMeshSubdivideFunctions|ApplyPNTessellation :TargetMesh _returnvalue_2 :Debug 0)
          (Class|DynamicMeshComponent|EnableComplexasSimpleCollision (Variables|DynamicMeshActor|GetDynamicMeshComponent)))))))

(event Input|ActionEvents|InputActionToSlicingMesh
  (params (Key :type Key%20Structure :default "None"))
  (:Pressed
    (CallFunction|CreateSlicingMesh (Math|Transform|MakeTransform "0, 0, 0"))
    (Actor|DestroyActor)
    (Development|PrintString "To Slicing Mesh")))

(fn ConstructionScript)

(fn CreateSlicingMesh
  (params (RelativeTransform :type Transform))
  (bind _returnvalue (Game|SpawnActorfromClass "/Game/EyeSurgery/CataractRemoval/BP_SliceMesh.BP_SliceMesh_C" (Math|Transform|ComposeTransforms (Transformation|GetActorTransform) RelativeTransform) "Undefined" 0 (Variables|Default|GetDynamicMeshObj) 0 0))
  (return _returnvalue))