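; BP_Ball is a sliceable dynamic-mesh sphere actor in the eye surgery cataract removal content.
; It uses Geometry Script to copy a static Sphere into its mesh on rebuild and caches that mesh.
; The ShrinkParts input cuts the mesh with a fixed angled, gapped plane and splits it by components.
; Each piece is copied into a newly spawned BP_Ball, with DestroyActor on the original called inside that loop.
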(event EventBeginPlay)

(event Collision|EventActorBeginOverlap
  (params (OtherActor :type Actor%20Object%20Reference)))

(event EventTick
  (params (DeltaSeconds :type Float%20%28single-precision%29)))

(event Events|EventOnRebuildGeneratedMesh
  (params (TargetMesh :type Dynamic%20Mesh%20Object%20Reference))
  (bind _returnvalue (GeometryScript|StaticMesh|CopyMeshFromStaticMesh :FromStaticMeshAsset "/Engine/BasicShapes/Sphere.Sphere" :ToDynamicMesh TargetMesh :Debug 0)
    (:Success
      (Variables|Default|SetRootDynamicMeshObj _returnvalue))))

(event Input|ActionEvents|InputActionShrinkParts
  (params (Key :type Key%20Structure :default "None"))
  (:Pressed
    (bind _returnvalue (Class|GeometryScriptLibraryMeshBooleanFunctions|ApplyMeshPlaneSlice (Variables|Default|GetRootDynamicMeshObj) (Math|Transform|MakeTransform "0, 0, 0" "75.000000,0.000000,0.000000" "1.000000,1.000000,1.000000") (Utilities|Struct|MakeGeometryScriptMeshPlaneSliceOptions true true 1.0 1.0) 0))
    (bind _componentmeshes (Class|GeometryScriptLibraryMeshDecompositionFunctions|SplitMeshbyComponents _returnvalue (Variables|Default|GetMeshPool) 0))
    (for _array_element _componentmeshes
      (bind _returnvalue_2 (Game|SpawnActorfromClass "BP_Ball_C" (Transformation|GetActorTransform) "Undefined" 0 0))
      (bind _returnvalue_3 (DynamicMeshComponent|GetDynamicMesh (Variables|/Script/GeometryFramework.DynamicMeshActor|GetDynamicMeshComponent _returnvalue_2)))
      (GeometryScript|Decomposition|CopyMeshtoMesh _array_element _returnvalue_3 0)
      (Actor|DestroyActor))))

(fn ConstructionScript)