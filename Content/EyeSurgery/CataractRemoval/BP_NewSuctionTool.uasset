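; VR suction tool actor for the cataract removal eye surgery, which carves away cataract mesh where its sphere touches it.
; Sphere overlap events set an overlap flag and cache the BP_NewCataract reference.
; While overlapping, Tick copies a sphere static mesh into a dynamic mesh and boolean-subtracts it from the cataract's mesh at runtime.
; The right trigger toggles an Active flag that does not gate the cutting.
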(event OnComponentBeginOverlap(Sphere)
  (params (OverlappedComponent :type Primitive%20Component%20Object%20Reference) (OtherActor :type Actor%20Object%20Reference) (OtherComp :type Primitive%20Component%20Object%20Reference) (OtherBodyIndex :type Integer) (bFromSweep :type Boolean) (SweepResult :type Hit%20Result%20Structure%20%28by%20ref%29))
  (Variables|Default|SetOverlapping true)
  (bind _asbp_new_cataract (Utilities|Casting|CastToBP_NewCataract OtherActor))
  (Variables|Default|SetCataract _asbp_new_cataract)
  (Development|PrintString "Overlap begins"))

(event OnComponentEndOverlap(Sphere)
  (params (OverlappedComponent :type Primitive%20Component%20Object%20Reference) (OtherActor :type Actor%20Object%20Reference) (OtherComp :type Primitive%20Component%20Object%20Reference) (OtherBodyIndex :type Integer))
  (Variables|Default|SetOverlapping false)
  (Development|PrintString "Overlap ends"))

(event EventBeginPlay
  (|CallParentFunction) ; 此节点被禁用，将不会被调用。\n从引脚连出引线来编译功能。
)

(event Collision|EventActorBeginOverlap
  (params (OtherActor :type Actor%20Object%20Reference))
  (|CallParentFunction OtherActor) ; 此节点被禁用，将不会被调用。\n从引脚连出引线来编译功能。
)

(event EventTick
  (params (DeltaSeconds :type Float%20%28single-precision%29))
  (|CallParentFunction DeltaSeconds)
  (if (Variables|Default|GetOverlapping)
    (bind _cataract (Variables|Default|GetCataract)
      (:then
        (bind _returnvalue (GeometryScript|StaticMesh|CopyMeshFromStaticMesh :FromStaticMeshAsset "/Engine/BasicShapes/Sphere.Sphere" :ToDynamicMesh (Variables|Default|GetTo%20Dynamic%20Mesh) :Debug 0)
          (:Success
            (GeometryScript|Booleans|ApplyMeshBoolean :TargetMesh (Variables|/Game/EyeSurgery/CataractRemoval/BP_NewCataract.BP_NewCataract_C|GetDynamicMeshObj (Variables|Default|GetCataract)) :TargetTransform (Math|Transform|MakeTransform (.Location (Math|Transform|BreakTransform (Transformation|GetWorldTransform (Variables|/Game/EyeSurgery/CataractRemoval/BP_NewCataract.BP_NewCataract_C|GetDynamicMesh _cataract)))) (.Rotation (Math|Transform|BreakTransform (Transformation|GetWorldTransform (Variables|/Game/EyeSurgery/CataractRemoval/BP_NewCataract.BP_NewCataract_C|GetDynamicMesh _cataract)))) (.Scale (Math|Transform|BreakTransform (Transformation|GetWorldTransform (Variables|/Game/EyeSurgery/CataractRemoval/BP_NewCataract.BP_NewCataract_C|GetDynamicMesh _cataract))))) :ToolMesh _returnvalue :ToolTransform (Transformation|GetWorldTransform (Variables|Default|GetSphere)) :Operation "Subtract" :Debug 0)
            (Development|PrintString "Subtraction"))))
      (:else
        (Development|PrintString "invalid cataract ref")))))

(event Input|ActionEvents|InputActionMotionControllerTriggerRight
  (params (Key :type Key%20Structure :default "None"))
  (:Pressed
    (Variables|Default|SetActive true))
  (:Released
    (Variables|Default|SetActive false)))

(fn ConstructionScript
  (|CallParentFunction))