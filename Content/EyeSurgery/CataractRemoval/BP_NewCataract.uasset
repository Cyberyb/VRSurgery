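; BP_NewCataract is a cataract mesh actor for the eye surgery cataract removal section, built on a DynamicMesh component.
; Its construction script fills the mesh from InitDynamicMeshComp if valid, otherwise from InitStaticMesh.
; It then applies PN tessellation and enables complex-as-simple collision on the mesh.
; The event graph has no active logic: overlap handlers are empty and their debug prints are disconnected.
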(event OnComponentBeginOverlap(DynamicMesh)
  (params (OverlappedComponent :type Primitive%20Component%20Object%20Reference) (OtherActor :type Actor%20Object%20Reference) (OtherComp :type Primitive%20Component%20Object%20Reference) (OtherBodyIndex :type Integer) (bFromSweep :type Boolean) (SweepResult :type Hit%20Result%20Structure%20%28by%20ref%29)))

(event OnComponentEndOverlap(DynamicMesh)
  (params (OverlappedComponent :type Primitive%20Component%20Object%20Reference) (OtherActor :type Actor%20Object%20Reference) (OtherComp :type Primitive%20Component%20Object%20Reference) (OtherBodyIndex :type Integer)))

(event EventBeginPlay)

(event Collision|EventActorBeginOverlap
  (params (OtherActor :type Actor%20Object%20Reference)))

(event EventTick
  (params (DeltaSeconds :type Float%20%28single-precision%29)))

(fn ConstructionScript
  (bind _initstaticmesh (Variables|Default|GetInitStaticMesh))
  (bind _initdynamicmeshcomp (Variables|Default|GetInitDynamicMeshComp))
  (Utilities|FlowControl|Sequence
    (:then_0
      (bind _returnvalue (DynamicMeshComponent|GetDynamicMesh (Variables|Default|GetDynamicMesh)))
      (Variables|Default|SetDynamicMeshObj _returnvalue))
    (:then_1
      (Utilities|IsValid _initdynamicmeshcomp
        (:Is%20Valid
          (GeometryScript|Scene|CopyMeshfromComponent :Component _initdynamicmeshcomp :ToDynamicMesh (Variables|Default|GetDynamicMeshObj) :Debug 0))
        (:Is%20Not%20Valid
          (Utilities|IsValid _initstaticmesh
            (:Is%20Valid
              (GeometryScript|StaticMesh|CopyMeshFromStaticMesh :FromStaticMeshAsset _initstaticmesh :ToDynamicMesh (Variables|Default|GetDynamicMeshObj) :Debug 0))))))
    (:then_2
      (Class|GeometryScriptLibraryMeshSubdivideFunctions|ApplyPNTessellation :TargetMesh (Variables|Default|GetDynamicMeshObj) :Debug 0)
      (Class|DynamicMeshComponent|EnableComplexasSimpleCollision (Variables|Default|GetDynamicMesh)))))