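; Sliceable mesh actor for cataract-removal eye surgery that breaks into shrinkable fragments.
; Construction fills a dynamic mesh from an initial static or dynamic mesh.
; The Slice input or BP_SplittingTool plane-slices all pieces with Geometry Script, splitting them into overlap-enabled components with complex-as-simple collision.
; Tick shrinks pieces overlapping BP_ShrinkTool until destroyed, while ToCataract input copies each piece into a new BP_Cataract and destroys this actor.
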(event Custom|OnHitBySplittingTool
  (params (CutFrame :type Transform))
  (Transformation|SetRelativeTransform (Variables|Default|GetPlane) CutFrame false false)
  (Development|PrintString "Hello")
  (CallFunction|SliceAllMeshes CutFrame)
  (for _array_element (Variables|Default|GetDynamicMeshes)
    (Utilities|FlowControl|Sequence
      (:then_0
        (Collision|BindEventtoOnComponentBeginOverlap _array_element (delegate Custom|ShrinkStart)))
      (:then_1
        (Collision|BindEventtoOnComponentEndOverlap _array_element (delegate Custom|ShrinkStop))))))

(event Custom|ShrinkStart
  (params (OverlappedComponent :type Primitive%20Component%20Object%20Reference) (OtherActor :type Actor%20Object%20Reference) (OtherComp :type Primitive%20Component%20Object%20Reference) (OtherBodyIndex :type Integer) (bFromSweep :type Boolean) (SweepResult :type Hit%20Result%20Structure%20%28by%20ref%29))
  (Utilities|Casting|CastToBP_ShrinkTool OtherActor)
  (bind _asdynamic_mesh_component (Utilities|Casting|CastToDynamicMeshComponent OverlappedComponent))
  (Utilities|Set|Add (Variables|Default|GetOverlappingComponents) _asdynamic_mesh_component))

(event Custom|ShrinkStop
  (params (OverlappedComponent :type Primitive%20Component%20Object%20Reference) (OtherActor :type Actor%20Object%20Reference) (OtherComp :type Primitive%20Component%20Object%20Reference) (OtherBodyIndex :type Integer))
  (Utilities|Casting|CastToBP_ShrinkTool OtherActor)
  (bind _asdynamic_mesh_component (Utilities|Casting|CastToDynamicMeshComponent OverlappedComponent))
  (Utilities|Set|Remove (Variables|Default|GetOverlappingComponents) _asdynamic_mesh_component))

(event EventBeginPlay
  (bind _returnvalue (Actor|GetActorOfClass "/Game/EyeSurgery/CataractRemoval/BP_SplittingTool.BP_SplittingTool_C"))
  (EventDispatchers|BindEventtoSlice _returnvalue (delegate Custom|OnHitBySplittingTool)))

(event EventTick
  (params (DeltaSeconds :type Float%20%28single-precision%29))
  (bind _result (Utilities|Set|ToArray (Variables|Default|GetOverlappingComponents)))
  (for _array_element _result
    (if (< (.X (Math|Vector|BreakVector (Variables|/Script/Engine.SceneComponent|GetRelativeScale3D _array_element))) 0.2)
      (Utilities|Array|RemoveItem (Variables|Default|GetDynamicMeshes) _array_element)
      (Components|DestroyComponent _array_element)
      (else
        (Transformation|SetRelativeScale3D _array_element (- (Variables|/Script/Engine.SceneComponent|GetRelativeScale3D _array_element) "0.010000,0.010000,0.010000"))))))

(event Input|ActionEvents|InputActionSlice
  (params (Key :type Key%20Structure :default "None"))
  (:Pressed
    (Transformation|SetRelativeTransform (Variables|Default|GetPlane) (stale Custom|OnHitBySplittingTool CutFrame) false false)
    (Development|PrintString "Hello")
    (CallFunction|SliceAllMeshes (stale Custom|OnHitBySplittingTool CutFrame))
    (for _array_element (Variables|Default|GetDynamicMeshes)
      (Utilities|FlowControl|Sequence
        (:then_0
          (Collision|BindEventtoOnComponentBeginOverlap _array_element (delegate Custom|ShrinkStart)))
        (:then_1
          (Collision|BindEventtoOnComponentEndOverlap _array_element (delegate Custom|ShrinkStop)))))))

(event Input|ActionEvents|InputActionToCataract
  (params (Key :type Key%20Structure :default "None"))
  (:Pressed
    (CallFunction|CreateCataracts (Math|Transform|MakeTransform "0, 0, 0"))
    (Actor|DestroyActor)
    (Development|PrintString "To Cataract")))

(fn ConstructionScript
  (bind _dynamicmeshes (Variables|Default|GetDynamicMeshes))
  (Utilities|FlowControl|Sequence
    (:then_0
      (bind _returnvalue (AddComponent|AddStaticMeshComponent false))
      (bind _output_get (LocalVariables|SetStaticMeshComp _returnvalue))
      (Components|StaticMesh|SetStaticMesh _output_get (Variables|Default|GetInitStaticMesh)))
    (:then_1
      (bind _returnvalue_2 (DynamicMeshComponent|GetDynamicMesh (Variables|Default|GetDynamicMesh)))
      (bind _initdynamicmeshobject (Variables|Default|GetInitDynamicMeshObject)
        (:then
          (GeometryScript|Decomposition|CopyMeshtoMesh _initdynamicmeshobject _returnvalue_2 0))
        (:else
          (GeometryScript|Scene|CopyMeshfromComponent :Component (LocalVariables|GetStaticMeshComp) :ToDynamicMesh _returnvalue_2 :Debug 0))))
    (:then_2
      (Components|DestroyComponent (LocalVariables|GetStaticMeshComp))
      (Utilities|Array|Clear _dynamicmeshes)
      (Utilities|Array|Add _dynamicmeshes (Variables|Default|GetDynamicMesh)))))

(fn SliceAllMeshes
  (params (CutFrame :type Transform))
  (Utilities|Array|Clear (LocalVariables|GetTotalSlicedMeshCompoents))
  (for _array_element (Variables|Default|GetDynamicMeshes)
    (bind _slicedmeshcomponents (CallFunction|SliceMeshComponent _array_element CutFrame (Utilities|Struct|MakeGeometryScriptMeshPlaneSliceOptions true true 1.0 1.0)))
    (Utilities|Array|AppendArray (LocalVariables|GetTotalSlicedMeshCompoents) _slicedmeshcomponents))
  (Utilities|Array|Clear (Variables|Default|GetDynamicMeshes))
  (Variables|Default|SetDynamicMeshes (LocalVariables|GetTotalSlicedMeshCompoents)))

(fn SliceMeshComponent
  (params (DynamicMeshCompoent :type Dynamic%20Mesh%20Component%20Object%20Reference) (CutFrame :type Transform) (Options :type Geometry%20Script%20Mesh%20Plane%20Slice%20Options%20Structure))
  (bind _returnvalue (DynamicMeshComponent|GetDynamicMesh DynamicMeshCompoent))
  (bind _returnvalue_2 (Class|GeometryScriptLibraryMeshBooleanFunctions|ApplyMeshPlaneSlice _returnvalue CutFrame Options 0))
  (bind _componentmeshes (Class|GeometryScriptLibraryMeshDecompositionFunctions|SplitMeshbyComponents _returnvalue_2 0 0))
  (for _array_element _componentmeshes
    (bind _dynamicmeshcomponent (CallFunction|CreateDynamicMeshComponent _array_element))
    (Utilities|SetCollision _dynamicmeshcomponent
      (:Out
        (Class|DynamicMeshComponent|UpdateCollision _dynamicmeshcomponent false) ; w/o this no collision will happen. OnlyIfPending must be turned off
        (Utilities|Array|Add (LocalVariables|GetMeshComponents) _dynamicmeshcomponent))))
  (Components|DestroyComponent DynamicMeshCompoent)
  (return (LocalVariables|GetMeshComponents)))

(fn CreateDynamicMeshComponent
  (params (DynamicMesh :type Dynamic%20Mesh%20Object%20Reference))
  (bind _returnvalue (AddComponent|AddDynamicMeshComponent false))
  (bind _output_get (LocalVariables|SetDynamicMeshComp _returnvalue))
  (bind _returnvalue_2 (DynamicMeshComponent|GetDynamicMesh _output_get))
  (GeometryScript|Decomposition|CopyMeshtoMesh DynamicMesh _returnvalue_2 0)
  (return (LocalVariables|GetDynamicMeshComp)))

(fn PrintAllChildren
  (for _array_element (Components|GetChildrenComponents (Variables|Default|GetDefaultSceneRoot) false)
    (Development|PrintString (Utilities|GetDisplayName _array_element))))

(fn CreateCataracts
  (params (RelativeTransform :type Transform))
  (for _array_element (Variables|Default|GetDynamicMeshes)
    (bind _returnvalue (Game|SpawnActorfromClass "/Game/EyeSurgery/CataractRemoval/BP_Cataract.BP_Cataract_C" (Math|Transform|ComposeTransforms (Transformation|GetActorTransform) RelativeTransform) "Undefined" 0 0))
    (bind _returnvalue_2 (DynamicMeshComponent|GetDynamicMesh (Variables|/Script/GeometryFramework.DynamicMeshActor|GetDynamicMeshComponent _returnvalue)))
    (bind _returnvalue_3 (DynamicMeshComponent|GetDynamicMesh _array_element))
    (GeometryScript|Decomposition|CopyMeshtoMesh _returnvalue_3 _returnvalue_2 0)))