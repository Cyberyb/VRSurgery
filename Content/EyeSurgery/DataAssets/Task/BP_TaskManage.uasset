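; Task manager for the eye surgery levels that sequences each level's ordered steps from a task data asset.
; BeginPlay resets the asset's finished flags and starts task 0; TaskFinished requires the previous task done, then broadcasts and advances CurTask.
; TaskInit maps the asset to a level index and runs per-task setup toggling gaze, selection and board widgets or respawning the doctor.
; An out-of-range task ID returns to the start level.
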(event Custom|BackToStartLevel
  ;[1 1 1] 返回开始界面
  (bind _gameinstance (CallFunction|GetMainGameInstance self))
  (Default|SwitchLevel _gameinstance "/Game/EyeSurgery/DataAssets/Level/DA_Level_开始.DA_Level_开始" true true))

(event EventBeginPlay
  (CallFunction|InitAllTasks)
  (CallFunction|TaskInit))

(event Collision|EventActorBeginOverlap
  (params (OtherActor :type Actor%20Object%20Reference)))

(event EventTick
  (params (DeltaSeconds :type Float%20%28single-precision%29)))

(fn ConstructionScript)

(fn GetPreNode
  (params (CurNodeIndex :type Integer))
  (bind _taskarraypda (Variables|Default|GetTaskArrayPDA))
  (bind _taskarray (Variables|/Game/EyeSurgery/DataAssets/Task/PDA_TaskArray.PDA_TaskArray_C|GetTaskArray _taskarraypda))
  (bind (_value _index) (Utilities|ArrayPrevIndex _taskarray CurNodeIndex false))
  (if (> CurNodeIndex 0)
    (return _value _index)
    (else
      (Development|PrintString "无前置节点，返回当前节点")
      (return (Utilities|Array|Get(acopy) _taskarray CurNodeIndex) 0))))

(fn GetNextNode
  (params (CurNodeIndex :type Integer))
  (bind _taskarraypda (Variables|Default|GetTaskArrayPDA))
  (bind _taskarray (Variables|/Game/EyeSurgery/DataAssets/Task/PDA_TaskArray.PDA_TaskArray_C|GetTaskArray _taskarraypda))
  (bind (_value _index) (Utilities|ArrayNextIndex _taskarray CurNodeIndex false))
  (if (< CurNodeIndex (- (Utilities|Array|Length _taskarray) 1))
    (return _value _index)
    (else
      (Development|PrintString "无后置节点，返回当前节点")
      (return (Utilities|Array|Get(acopy) _taskarray CurNodeIndex) CurNodeIndex))))

(fn TaskFinished
  (params (TaskID :type Integer))
  (bind _taskarraypda (Variables|Default|GetTaskArrayPDA))
  (bind _taskarray (Variables|/Game/EyeSurgery/DataAssets/Task/PDA_TaskArray.PDA_TaskArray_C|GetTaskArray _taskarraypda))
  (bind _output (Utilities|Array|Get(acopy) _taskarray TaskID))
  (if (== TaskID 0)
    (Utilities|IsValid _taskarraypda
      (:Is%20Valid
        _))
    (else
      (bind _prenodeindex (CallFunction|GetPreNode TaskID))
      (bind _isfinished (CallFunction|IsTaskFinished _prenodeindex))
      (if _isfinished
        _
        (else
          (Development|PrintString "前置任务未完成，无法完成当前任务")
          (return false)))))
  (Utilities|Struct|SetmembersinS_TaskNode _output true)
  (Development|PrintString (Utilities|String|Append "完成任务：" (Utilities|String|ToString(Text) (Utilities|Struct|BreakS_TaskNode _output))))
  (Default|CallTaskFinished TaskID)
  (Variables|Default|SetCurTask (+ TaskID 1))
  (return true))

(fn IsTaskFinished
  (params (TaskID :type Integer))
  (return (Utilities|Struct|BreakS_TaskNode (Utilities|Array|Get(acopy) (Variables|/Game/EyeSurgery/DataAssets/Task/PDA_TaskArray.PDA_TaskArray_C|GetTaskArray (Variables|Default|GetTaskArrayPDA)) TaskID))))

(fn InitAllTasks
  (bind _taskarraypda (Variables|Default|GetTaskArrayPDA))
  (bind _taskarray (Variables|/Game/EyeSurgery/DataAssets/Task/PDA_TaskArray.PDA_TaskArray_C|GetTaskArray _taskarraypda))
  (for (_ _array_index) _taskarray
    (Utilities|Struct|SetmembersinS_TaskNode (Utilities|Array|Get(acopy) _taskarray _array_index) false))
  (Development|PrintString "初始化任务完成"))

(fn TaskInit
  (params (TaskID :type Integer))
  (bind _taskarraypda (Variables|Default|GetTaskArrayPDA))
  (bind _level2intmap (Variables|Default|GetLevel2IntMap))
  (bind (_value _returnvalue) (Utilities|Map|Find _level2intmap _taskarraypda))
  ;[1 1 1] 根据当前Map、当前Task来进行任务初始化工作
  (if (>= TaskID (Utilities|Array|Length (Variables|/Game/EyeSurgery/DataAssets/Task/PDA_TaskArray.PDA_TaskArray_C|GetTaskArray (Variables|Default|GetTaskArrayPDA))))
    (CallFunction|BacktoStartLevel)
    (elif _returnvalue
      (switch int _value
        (:0
          (switch int TaskID
            (:0
              (|Level1Task0Init))
            (:1
              (|Level1Task1Init))
            (:2
              (|Level1Task2Init))
            (:4
              (|Level1Task4Init))))
        (:1
          (switch int TaskID
            (:0
              (|Level2Task0Init))
            (:1
              (|Level2Task1Init))))
        (:3
          (switch int TaskID
            (:0
              (|Level4Task0Init))
            (:1
              (|Level4Task1Init))))))))