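; Task manager Blueprint for EyeSurgery that tracks an ordered queue of task nodes and enforces their completion order.
; On BeginPlay it clears the finished flag on every node in TaskNode's TaskQue.
; TaskFinished converts a 1-based ID to an index and marks that task done only if it is first or its predecessor is finished.
; Helpers fetch neighbouring nodes, returning the current one at either end, with debug prints for feedback.
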(event EventBeginPlay
  (CallFunction|InitAllTasks))

(event Collision|EventActorBeginOverlap
  (params (OtherActor :type Actor%20Object%20Reference)))

(event EventTick
  (params (DeltaSeconds :type Float%20%28single-precision%29)))

(fn ConstructionScript)

(fn GetPreNode
  (params (CurNodeIndex :type Integer))
  (bind _tasknode (Variables|Default|GetTaskNode))
  (bind _taskque (Variables|/Game/EyeSurgery/DataAssets/Level/PDA_TaskList.PDA_TaskList_C|GetTaskQue _tasknode))
  (bind (_value _index) (Utilities|ArrayPrevIndex _taskque CurNodeIndex false))
  (if (> CurNodeIndex 0)
    (return _value _index)
    (else
      (Development|PrintString "无前置节点，返回当前节点")
      (return (Utilities|Array|Get(acopy) _taskque CurNodeIndex) CurNodeIndex))))

(fn GetNextNode
  (params (CurNodeIndex :type Integer))
  (bind _tasknode (Variables|Default|GetTaskNode))
  (bind _taskque (Variables|/Game/EyeSurgery/DataAssets/Level/PDA_TaskList.PDA_TaskList_C|GetTaskQue _tasknode))
  (bind (_value _index) (Utilities|ArrayNextIndex _taskque CurNodeIndex false))
  (if (< CurNodeIndex (- (Utilities|Array|Length _taskque) 1))
    (return _value _index)
    (else
      (Development|PrintString "无后置节点，返回当前节点")
      (return (Utilities|Array|Get(acopy) _taskque CurNodeIndex) CurNodeIndex))))

(fn TaskFinished
  (params (TaskID :type Integer))
  (bind _returnvalue (- TaskID 1))
  (if (== _returnvalue 0)
    (Utilities|Struct|SetmembersinS_TaskQueNode (Utilities|Array|Get(acopy) (Variables|/Game/EyeSurgery/DataAssets/Level/PDA_TaskList.PDA_TaskList_C|GetTaskQue (Variables|Default|GetTaskNode)) _returnvalue) true :!label _label)
    (Development|PrintString (Utilities|String|Append "完成任务，ID:" (Utilities|String|ToString(Integer) _returnvalue)))
    (else
      (bind _prenodeindex (CallFunction|GetPreNode _returnvalue))
      (bind _isfinished (CallFunction|IsTaskFinished _prenodeindex))
      (if _isfinished
        (goto _label)
        (else
          (Development|PrintString "前置任务未完成，无法完成当前任务"))))))

(fn IsTaskFinished
  (params (TaskID :type Integer))
  (return (Utilities|Struct|BreakS_TaskQueNode (Utilities|Array|Get(acopy) (Variables|/Game/EyeSurgery/DataAssets/Level/PDA_TaskList.PDA_TaskList_C|GetTaskQue (Variables|Default|GetTaskNode)) TaskID))))

(fn InitAllTasks
  (bind _tasknode (Variables|Default|GetTaskNode))
  (bind _taskque (Variables|/Game/EyeSurgery/DataAssets/Level/PDA_TaskList.PDA_TaskList_C|GetTaskQue _tasknode))
  (for (_ _array_index) _taskque
    (Utilities|Struct|SetmembersinS_TaskQueNode (Utilities|Array|Get(acopy) _taskque _array_index) false))
  (Development|PrintString "初始化任务完成")
  (for _array_element _taskque
    (if (.isfinished _array_element)
      (Development|PrintString "TTTTTTTrue"))))