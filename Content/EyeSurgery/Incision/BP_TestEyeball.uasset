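; BP_TestEyeball is a test eyeball actor for the eye surgery incision feature that positions and scales a decal on its surface.
; PlaceDecal moves the decal to a given world location and orients it along the direction from the eyeball center, with a fixed local rotation correction.
; ScaleDecal sets the decal's relative scale from the given value.
; Its event graph and construction script are empty, so callers drive both functions.
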(event EventBeginPlay)

(event Collision|EventActorBeginOverlap
  (params (OtherActor :type Actor%20Object%20Reference)))

(event EventTick
  (params (DeltaSeconds :type Float%20%28single-precision%29)))

(fn ConstructionScript)

(fn PlaceDecal
  (params (WorldLocation :type Vector))
  (bind _decal (Variables|Default|GetDecal))
  (Utilities|FlowControl|Sequence
    (:then_0
      (LocalVariables|SetProjectionDir (- WorldLocation (Transformation|GetWorldLocation (Variables|Default|GetEyeball)))))
    (:then_1
      (Transformation|SetWorldLocationAndRotation _decal WorldLocation (Math|Conversions|RotationFromXVector (LocalVariables|GetProjectionDir)) false false)
      (Transformation|AddLocalRotation _decal "0,180.000000,90.000000" false false))))

(fn ScaleDecal
  (params (Scale :type Float%20%28double-precision%29))
  (Transformation|SetRelativeScale3D (Variables|Default|GetDecal) (Math|Conversions|ToVector(Float) Scale)))