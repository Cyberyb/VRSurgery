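; BP_IncisionToolLimiter keeps the incision tool's tip within a spherical boundary during an incision in the eye surgery game.
; The incision tool's begin and end events switch the limiter on and off.
; While enabled, Tick tests whether the tip has left the sphere component's scaled radius.
; If so, it offsets the whole tool actor without sweep so the tip lands on the nearest point of the sphere's surface.
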(event Custom|Enable
  (Variables|Default|SetEnabled true))

(event Custom|Disable
  (Variables|Default|SetEnabled false))

(event EventBeginPlay
  (bind _incisiontool (Variables|Default|GetIncisionTool)
    (:then
      (EventDispatchers|BindEventtoIncisionBegin _incisiontool (delegate Custom|Enable))
      (EventDispatchers|BindEventtoIncisionEnd _incisiontool (delegate Custom|Disable)))
    (:else)))

(event EventTick
  (params (DeltaSeconds :type Float%20%28single-precision%29))
  (if (Variables|Default|GetEnabled)
    (if (not (CallFunction|ToolInsideSphere))
      (CallFunction|LimitToolLocation))))

(fn ConstructionScript)

(fn ToolInsideSphere
  (bind _sphere (Variables|Default|GetSphere))
  (return (< (Math|Vector|Distance(Vector) (Default|TipWorldLocation (Variables|Default|GetIncisionTool)) (Transformation|GetWorldLocation _sphere)) (Components|Sphere|GetScaledSphereRadius _sphere))))

(fn LimitToolLocation
  (bind _incisiontool (Variables|Default|GetIncisionTool))
  (bind _sphere (Variables|Default|GetSphere))
  (bind _location (Default|TipWorldLocation _incisiontool))
  (Transformation|AddActorWorldOffset (Variables|Default|GetIncisionTool) (- (CallFunction|ProjecttoSphere _location (Transformation|GetWorldLocation _sphere) (Components|Sphere|GetScaledSphereRadius _sphere)) _location))
  (return))

(fn ProjecttoSphere
  (params (Point :type Vector) (Center :type Vector) (Radius :type Float%20%28double-precision%29))
  (return (+ (* (Math|Vector|Normalize (- Point Center)) Radius) Center)))