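; Sliceable ball actor in the CataractRemoval2 folder that cuts itself into pieces with Geometry Script.
; The construction script copies a static sphere mesh into a dynamic mesh component, then destroys the static one.
; Each Slice input plane-slices every tracked mesh at a fixed angle with a gap, then splits it by connected components.
; Each piece becomes a new dynamic mesh component, replacing its source for later slices.
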(event EventBeginPlay)

(event Collision|EventActorBeginOverlap
  (params (OtherActor :type Actor%20Object%20Reference)))

(event EventTick
  (params (DeltaSeconds :type Float%20%28single-precision%29)))

(event Input|ActionEvents|InputActionSlice
  (params (Key :type Key%20Structure))
  (:Pressed
    (CallFunction|SliceAllMeshes)))

(fn ConstructionScript
  (bind _dynamicmeshes (Variables|Default|GetDynamicMeshes))
  (Utilities|FlowControl|Sequence
    (:then_0
      (bind _returnvalue (AddComponent|AddStaticMeshComponent false))
      (bind _output_get (LocalVariables|SetStaticMeshComp _returnvalue))
      (Components|StaticMesh|SetStaticMesh _output_get "/Engine/BasicShapes/Sphere.Sphere"))
    (:then_1
      (bind _returnvalue_2 (AddComponent|AddDynamicMeshComponent false))
      (bind _returnvalue_3 (DynamicMeshComponent|GetDynamicMesh _returnvalue_2))
      (GeometryScript|Scene|CopyMeshfromComponent :Component (LocalVariables|GetStaticMeshComp) :ToDynamicMesh _returnvalue_3 :Debug 0
        (:Success
          (Components|DestroyComponent (LocalVariables|GetStaticMeshComp)))))
    (:then_2
      (Utilities|Array|Clear _dynamicmeshes)
      (Utilities|Array|Add _dynamicmeshes _returnvalue_2))))

(fn SliceAllMeshes
  (Utilities|Array|Clear (LocalVariables|GetTotalSlicedMeshCompoents))
  (for _array_element (Variables|Default|GetDynamicMeshes)
    (bind _slicedmeshcomponents (CallFunction|SliceMeshComponent _array_element (Math|Transform|MakeTransform "0, 0, 0" "75.000000, 0, 0" "1.000000,1.000000,1.000000") (Utilities|Struct|MakeGeometryScriptMeshPlaneSliceOptions true true 1.0 1.0)))
    (Utilities|Array|AppendArray _slicedmeshcomponents (LocalVariables|GetTotalSlicedMeshCompoents))
    (Components|DestroyComponent _array_element))
  (Utilities|Array|Clear (Variables|Default|GetDynamicMeshes))
  (Variables|Default|SetDynamicMeshes (LocalVariables|GetTotalSlicedMeshCompoents)))

(fn SliceMeshComponent
  (params (DynamicMeshCompoent :type Dynamic%20Mesh%20Component%20Object%20Reference) (CutFrame :type Transform) (Options :type Geometry%20Script%20Mesh%20Plane%20Slice%20Options%20Structure))
  (bind _returnvalue (DynamicMeshComponent|GetDynamicMesh DynamicMeshCompoent))
  (bind _returnvalue_2 (Class|GeometryScriptLibraryMeshBooleanFunctions|ApplyMeshPlaneSlice _returnvalue CutFrame Options 0))
  (bind _componentmeshes (Class|GeometryScriptLibraryMeshDecompositionFunctions|SplitMeshbyComponents _returnvalue_2 0 0))
  (for _array_element _componentmeshes
    (bind _dynamicmeshcomponent (CallFunction|CreateDynamicMeshComponent _array_element))
    (Utilities|Array|Add (LocalVariables|GetMeshComponents) _dynamicmeshcomponent))
  (return (LocalVariables|GetMeshComponents)))

(fn CreateDynamicMeshComponent
  (params (DynamicMesh :type Dynamic%20Mesh%20Object%20Reference))
  (bind _returnvalue (AddComponent|AddDynamicMeshComponent false))
  (bind _output_get (LocalVariables|SetDynamicMeshComp _returnvalue))
  (bind _returnvalue_2 (DynamicMeshComponent|GetDynamicMesh _output_get))
  (GeometryScript|Decomposition|CopyMeshtoMesh DynamicMesh _returnvalue_2 0)
  (return (LocalVariables|GetDynamicMeshComp)))