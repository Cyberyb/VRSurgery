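; BP_SuctionTool is a VR eye-surgery tool that carves away cataract material with its sphere while the right motion controller trigger is held.
; Sphere overlap events track contact and cache the BP_Cataract reference.
; While active and overlapping, Tick copies the sphere into a pooled compute mesh and boolean-subtracts it from the cataract's dynamic mesh using Geometry Script.
; Releasing the trigger frees the cataract's compute meshes.
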(event OnComponentBeginOverlap(Sphere)
  (params (OverlappedComponent :type Primitive%20Component%20Object%20Reference) (OtherActor :type Actor%20Object%20Reference) (OtherComp :type Primitive%20Component%20Object%20Reference) (OtherBodyIndex :type Integer) (bFromSweep :type Boolean) (SweepResult :type Hit%20Result%20Structure%20%28by%20ref%29))
  (Variables|Default|SetOverlapping true)
  (bind _asbp_cataract (Utilities|Casting|CastToBP_Cataract OtherActor))
  (Variables|Default|SetCataract _asbp_cataract))

(event OnComponentEndOverlap(Sphere)
  (params (OverlappedComponent :type Primitive%20Component%20Object%20Reference) (OtherActor :type Actor%20Object%20Reference) (OtherComp :type Primitive%20Component%20Object%20Reference) (OtherBodyIndex :type Integer))
  (Variables|Default|SetOverlapping false))

(event EventBeginPlay
  (|CallParentFunction) ; 此节点被禁用，将不会被调用。\n从引脚连出引线来编译功能。
)

(event Collision|EventActorBeginOverlap
  (params (OtherActor :type Actor%20Object%20Reference))
  (|CallParentFunction OtherActor) ; 此节点被禁用，将不会被调用。\n从引脚连出引线来编译功能。
)

(event EventTick
  (params (DeltaSeconds :type Float%20%28single-precision%29))
  (|CallParentFunction DeltaSeconds)
  (if (and (Variables|Default|GetOverlapping) (Variables|Default|GetActive))
    (bind _cataract (Variables|Default|GetCataract)
      (:then
        (bind _returnvalue (DynamicMeshActor|AllocateComputeMesh _cataract))
        (bind _returnvalue_2 (GeometryScript|StaticMesh|CopyMeshFromStaticMesh :FromStaticMeshAsset "/Engine/BasicShapes/Sphere.Sphere" :ToDynamicMesh _returnvalue :Debug 0)
          (:Success
            (GeometryScript|Booleans|ApplyMeshBoolean :TargetMesh (Variables|/Game/EyeSurgery/CataractRemoval2/BP_Cataract.BP_Cataract_C|GetDynamicMeshObj (Variables|Default|GetCataract)) :TargetTransform (Transformation|GetWorldTransform (Variables|/Script/GeometryFramework.DynamicMeshActor|GetDynamicMeshComponent _cataract)) :ToolMesh _returnvalue_2 :ToolTransform (Transformation|GetWorldTransform (Variables|Default|GetSphere)) :Operation "Subtract" :Debug 0))))
      (:else
        (Development|PrintString "invalid cataract ref")))))

(event Input|ActionEvents|InputActionMotionControllerTriggerRight
  (params (Key :type Key%20Structure))
  (:Pressed
    (Variables|Default|SetActive true))
  (:Released
    (Variables|Default|SetActive false)
    (DynamicMeshActor|ReleaseAllComputeMeshes (Variables|Default|GetCataract))))

(fn ConstructionScript
  (|CallParentFunction))