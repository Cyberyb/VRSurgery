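; BP_CataractOverlap is a slice-tool helper for cataract surgery that tracks which parts of a dynamic cataract it touches.
; CollisionComponent overlaps cache the BP_DynamicCataract and maintain a set of its touched DynamicMeshComponents.
; A separate Tip collider records the last mesh component it enters as the slice target, which is not cleared on exit.
; Getters expose overlap state, count, cataract and slice component.
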(event OnComponentBeginOverlap(CollisionComponent)
  (params (OverlappedComponent :type Primitive%20Component%20Object%20Reference) (OtherActor :type Actor%20Object%20Reference) (OtherComp :type Primitive%20Component%20Object%20Reference) (OtherBodyIndex :type Integer) (bFromSweep :type Boolean) (SweepResult :type Hit%20Result%20Structure%20%28by%20ref%29))
  (bind _asbp_dynamic_cataract (Utilities|Casting|CastToBP_DynamicCataract OtherActor))
  (Variables|Default|SetCataract _asbp_dynamic_cataract)
  (bind _asdynamic_mesh_component (Utilities|Casting|CastToDynamicMeshComponent OtherComp))
  (Utilities|Set|Add (Variables|Default|GetOverlappingComponents) _asdynamic_mesh_component))

(event OnComponentEndOverlap(CollisionComponent)
  (params (OverlappedComponent :type Primitive%20Component%20Object%20Reference) (OtherActor :type Actor%20Object%20Reference) (OtherComp :type Primitive%20Component%20Object%20Reference) (OtherBodyIndex :type Integer))
  (bind _asdynamic_mesh_component (Utilities|Casting|CastToDynamicMeshComponent OtherComp))
  (Utilities|Set|Remove (Variables|Default|GetOverlappingComponents) _asdynamic_mesh_component))

(event OnComponentBeginOverlap(Tip)
  (params (OverlappedComponent :type Primitive%20Component%20Object%20Reference) (OtherActor :type Actor%20Object%20Reference) (OtherComp :type Primitive%20Component%20Object%20Reference) (OtherBodyIndex :type Integer) (bFromSweep :type Boolean) (SweepResult :type Hit%20Result%20Structure%20%28by%20ref%29))
  (bind _asdynamic_mesh_component (Utilities|Casting|CastToDynamicMeshComponent OtherComp))
  (Variables|Default|SetSliceComponent _asdynamic_mesh_component))

(event OnComponentEndOverlap(Tip)
  (params (OverlappedComponent :type Primitive%20Component%20Object%20Reference) (OtherActor :type Actor%20Object%20Reference) (OtherComp :type Primitive%20Component%20Object%20Reference) (OtherBodyIndex :type Integer)))

(event EventTick
  (params (DeltaSeconds :type Float%20%28single-precision%29)))

(fn ConstructionScript)

(fn IsOverlapping
  (return (Utilities|Set|IsNotEmpty (Variables|Default|GetOverlappingComponents))))

(fn GetOverlap
  (return (CallFunction|GetCataract) (CallFunction|GetSliceComponent)))

(fn GetOverlapCount
  (return (Utilities|Set|Length (Variables|Default|GetOverlappingComponents))))

(fn GetCataract
  (return (Variables|Default|GetCataract)))

(fn GetSliceComponent
  (return (Variables|Default|GetSliceComponent)))