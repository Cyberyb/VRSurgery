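; A trigger volume actor for the cataract removal surgery that detects the suction tool entering its collision component.
; On begin overlap it stores the BP_SuctionTool reference and disables the tool; on end overlap it re-enables the tool and clears the reference.
; Helper functions report whether a tool is currently inside and whether that tool is triggered.
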(event OnComponentBeginOverlap(CollisionComponent)
  (params (OverlappedComponent :type Primitive%20Component%20Object%20Reference) (OtherActor :type Actor%20Object%20Reference) (OtherComp :type Primitive%20Component%20Object%20Reference) (OtherBodyIndex :type Integer) (bFromSweep :type Boolean) (SweepResult :type Hit%20Result%20Structure%20%28by%20ref%29))
  (bind _asbp_suction_tool (Utilities|Casting|CastToBP_SuctionTool OtherActor))
  (bind _output_get (Variables|Default|SetSuctionTool _asbp_suction_tool))
  (Default|Disable _output_get))

(event OnComponentEndOverlap(CollisionComponent)
  (params (OverlappedComponent :type Primitive%20Component%20Object%20Reference) (OtherActor :type Actor%20Object%20Reference) (OtherComp :type Primitive%20Component%20Object%20Reference) (OtherBodyIndex :type Integer))
  (bind _asbp_suction_tool (Utilities|Casting|CastToBP_SuctionTool OtherActor))
  (Default|Enable _asbp_suction_tool)
  (Variables|Default|SetSuctionTool 0))

(event EventBeginPlay)

(event Collision|EventActorBeginOverlap
  (params (OtherActor :type Actor%20Object%20Reference)))

(event EventTick
  (params (DeltaSeconds :type Float%20%28single-precision%29)))

(fn ConstructionScript)

(fn IsSuctionToolValid
  (return (Utilities|IsValid (Variables|Default|GetSuctionTool))))

(fn IsTriggered
  (bind _suctiontool (Variables|Default|GetSuctionTool)
    (:then
      (return (Default|IsTriggered _suctiontool)))
    (:else
      (return false))))