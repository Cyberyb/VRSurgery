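; BP_ShrinkTool gradually shrinks marked dynamic mesh components in the cataract-removal eye surgery until they disappear.
; MarkShrink and UnmarkShrink maintain the tracked components, and Tick scales each one's mesh geometry down by a fixed fraction per frame, independent of delta time.
; Once a mesh's bounding-box diagonal drops below ThresholdRadius, its owning BP_DynamicCataract is told to delete that component.
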(event EventTick
  (params (DeltaSeconds :type Float%20%28single-precision%29))
  (bind _result (Utilities|Set|ToArray (Variables|Default|GetCompToShrink)))
  (for _array_element _result
    (CallFunction|Shrink _array_element 0.01)
    (CallFunction|DestroyifTooSmall _array_element)))

(fn ConstructionScript)

(fn MarkShrink
  (params (DynamicMeshComponent :type Dynamic%20Mesh%20Component%20Object%20Reference))
  (Utilities|Set|Add (Variables|Default|GetCompToShrink) DynamicMeshComponent))

(fn UnmarkShrink
  (params (DynamicMeshComponent :type Dynamic%20Mesh%20Component%20Object%20Reference))
  (Utilities|Set|Remove (Variables|Default|GetCompToShrink) DynamicMeshComponent))

(fn Shrink
  (params (DynamicMeshComponent :type Dynamic%20Mesh%20Component%20Object%20Reference) (DeltaScale :type Float%20%28double-precision%29))
  (bind _returnvalue (DynamicMeshComponent|GetDynamicMesh DynamicMeshComponent))
  (Class|GeometryScriptLibraryMeshTransformFunctions|ScaleMesh _returnvalue (Math|Conversions|ToVector(Float) (- 1.0 DeltaScale)) 0)
  (return))

(fn DestroyifTooSmall
  (params (DynamicMeshComponent :type Dynamic%20Mesh%20Component%20Object%20Reference))
  (bind _returnvalue (DynamicMeshComponent|GetDynamicMesh DynamicMeshComponent))
  (if (< (Math|Vector|Distance(Vector) (.min (Class|GeometryScriptLibraryMeshQueryFunctions|GetMeshBoundingBox _returnvalue)) (.max (Class|GeometryScriptLibraryMeshQueryFunctions|GetMeshBoundingBox _returnvalue))) (Variables|Default|GetThresholdRadius))
    (bind _asbp_dynamic_cataract (Utilities|Casting|CastToBP_DynamicCataract (Components|GetOwner DynamicMeshComponent)))
    (Default|DeleteComponent _asbp_dynamic_cataract DynamicMeshComponent)))