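; Grabbable surgical tool that slices the dynamic-mesh cataract in the eye surgery game.
; Trigger input enables it and switches mode; UpdateToolBehavior prioritizes translate, rotate, then slice, using limiter, overlap and suction-tool checks.
; Slicing requires cataract overlap and a nearby, triggered suction tool, both detected through child actors.
; DoSlice cuts one component or all, along the tool's free plane or an axis-constrained plane angled toward the overlap point.
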(event GrabKeyInput(Comp_Grab)
  (params (MComp :type BP%20M%20Comp%20Object%20Reference) (Key :type Enum_Controller_Buttons%20Enum :default "NewEnumerator1") (Set :type Boolean))
  (switch Utilities|FlowControl|Switch|SwitchonEnum_Controller_Buttons Key
    (:NewEnumerator0
      (bind _output_get (Variables|Default|SetIsTriggered Set))
      (if _output_get
        (CallFunction|Enable)
        (CallFunction|SwitchMode "NewEnumerator0")))))

(event EventBeginPlay
  (Utilities|FlowControl|Sequence
    (:then_0
      (bind _returnvalue (Actor|GetActorOfClass "/Game/EyeSurgery/CataractRemovalNew/BP_DynamicCataract.BP_DynamicCataract_C"))
      (Utilities|IsValid _returnvalue
        (:Is%20Valid
          (Variables|Default|SetCataractToTransform _returnvalue)
          (Variables|Default|SetBehavior "NewEnumerator2"))))))

(event EventTick
  (params (DeltaSeconds :type Float%20%28single-precision%29))
  (|CallParentFunction DeltaSeconds))

(fn ConstructionScript)

(fn SlicewithFreePlane
  (params (Cataract :type BP%20Dynamic%20Cataract%20Object%20Reference) (ComponentToSlice :type Dynamic%20Mesh%20Component%20Object%20Reference))
  (bind _returnvalue (Transformation|GetActorRotation))
  (bind _returnvalue_2 (Transformation|GetActorLocation Cataract))
  (bind _gapwidth (Variables|Slice|GetGapWidth))
  (bind _cataractoverlap (Variables|Default|GetCataractOverlap))
  (bind _returnvalue_3 (Transformation|GetWorldLocation _cataractoverlap))
  (bind _returnvalue_4 (- _returnvalue_3 _returnvalue_2))
  (if (Variables|Slice|GetSliceThroughAllComponents)
    (Default|SliceAll Cataract (Math|Transform|MakeTransform _returnvalue_4 _returnvalue "1.000000,1.000000,1.000000") (Utilities|Struct|MakeGeometryScriptMeshPlaneSliceOptions true true _gapwidth 1.0))
    (else
      (Default|SliceComponent Cataract ComponentToSlice (Math|Transform|MakeTransform _returnvalue_4 _returnvalue "1.000000,1.000000,1.000000") (Utilities|Struct|MakeGeometryScriptMeshPlaneSliceOptions true true _gapwidth 1.0)))))

(fn SlicewithDirection
  (params (Cataract :type BP%20Dynamic%20Cataract%20Object%20Reference) (ComponentToSlice :type Dynamic%20Mesh%20Component%20Object%20Reference) (PlaneVec :type Vector))
  (bind _rotation (CallFunction|GetSliceRotationAlongY PlaneVec))
  (bind _rotation_2 (CallFunction|GetSliceRotationAlongZ PlaneVec))
  (bind _rotation_3 (CallFunction|GetSliceRotationAlongX PlaneVec))
  (bind _totalmeshlocaltransform (Variables|/Game/EyeSurgery/CataractRemovalNew/BP_DynamicCataract.BP_DynamicCataract_C|GetTotalMeshLocalTransform Cataract))
  (bind _slicedirection (Variables|Slice|GetSliceDirection))
  (bind _gapwidth (Variables|Slice|GetGapWidth))
  (bind _returnvalue (Utilities|Select :Index _slicedirection :NewEnumerator0 _rotation_3 :NewEnumerator1 _rotation :NewEnumerator2 _rotation_2))
  (bind _returnvalue_2 (Math|Transform|MakeTransform (.location _totalmeshlocaltransform) _returnvalue))
  (if (Variables|Slice|GetSliceThroughAllComponents)
    (Default|SliceAll Cataract _returnvalue_2 (Utilities|Struct|MakeGeometryScriptMeshPlaneSliceOptions true true _gapwidth 1.0))
    (else
      (Default|SliceComponent Cataract ComponentToSlice _returnvalue_2 (Utilities|Struct|MakeGeometryScriptMeshPlaneSliceOptions true true _gapwidth 1.0)))))

(fn GetSliceRotationAlongX
  (params (PlaneVec :type Vector))
  (bind (_x _y _z) (Math|Vector|BreakVector PlaneVec))
  (return (Math|Rotator|MakeRotator (* (CallFunction|AngleBetweenTwoVectors (Math|Vector|MakeVector 0.0 _y _z) "0,1.000000, 0") (* (Math|Float|Sign(Float) _z) -1.0)) 0.0 0.0)))

(fn GetSliceRotationAlongY
  (params (PlaneVec :type Vector))
  (bind (_x _y _z) (Math|Vector|BreakVector PlaneVec))
  (return (Math|Rotator|MakeRotator 0.0 (* (CallFunction|AngleBetweenTwoVectors (Math|Vector|MakeVector _x 0.0 _z) "1.000000,0.000000, 0") (Math|Float|Sign(Float) _z)) 0.0)))

(fn GetSliceRotationAlongZ
  (params (PlaneVec :type Vector))
  (bind (_x _y) (Math|Vector|BreakVector PlaneVec))
  (return (Math|Rotator|MakeRotator 9e+01 0.0 (* (CallFunction|AngleBetweenTwoVectors (Math|Vector|MakeVector _x _y 0.0) "1.000000,0.000000, 0") (Math|Float|Sign(Float) _y)))))

(fn SliceToolTriggered
  (return (Variables|Default|GetIsTriggered)))

(fn SuctionToolIsNear
  (bind _asbp_suction_tool_detection (Utilities|Casting|CastToBP_SuctionToolDetection (Variables|/Script/Engine.ChildActorComponent|GetChildActor (Variables|Default|GetSuctionToolDetection))))
  (return (Default|IsSuctionToolValid _asbp_suction_tool_detection)))

(fn SuctionToolTriggered
  (bind _asbp_suction_tool_detection (Utilities|Casting|CastToBP_SuctionToolDetection (Variables|/Script/Engine.ChildActorComponent|GetChildActor (Variables|Default|GetSuctionToolDetection))))
  (return (Default|IsTriggered _asbp_suction_tool_detection)))

(fn OverlappingwithCataract
  (bind _asbp_cataract_overlap (Utilities|Casting|CastToBP_CataractOverlap (Variables|/Script/Engine.ChildActorComponent|GetChildActor (Variables|Default|GetCataractOverlap))))
  (return (Default|IsOverlapping _asbp_cataract_overlap)))

(fn CanTranslate
  (return (and (Variables|Default|GetTranslateMode) (CallFunction|OverlappingwithCataract))))

(fn CanRotate
  (return (and (not (CallFunction|SuctionToolIsNear)) (CallFunction|IsInsideLimiter))))

(fn CanSlice
  (return (Math|Boolean|ANDBoolean (CallFunction|SuctionToolIsNear) (CallFunction|SuctionToolTriggered) (CallFunction|OverlappingwithCataract))))

(fn DoSlice
  (Utilities|FlowControl|Sequence
    (:then_0
      (bind _asbp_cataract_overlap (Utilities|Casting|CastToBP_CataractOverlap (Variables|/Script/Engine.ChildActorComponent|GetChildActor (Variables|Default|GetCataractOverlap))))
      (LocalVariables|SetSlicePoint (Transformation|GetActorLocation _asbp_cataract_overlap))
      (LocalVariables|SetCataract (Default|GetCataract _asbp_cataract_overlap))
      (LocalVariables|SetComponentToSlice (Default|GetSliceComponent _asbp_cataract_overlap)))
    (:then_1
      (LocalVariables|GetCataract
        (:then
          (LocalVariables|GetComponentToSlice
            (:then
              (if (Variables|Slice|GetSliceAlongAxis)
                (CallFunction|SlicewithDirection (LocalVariables|GetCataract) (LocalVariables|GetComponentToSlice) (- (LocalVariables|GetSlicePoint) (Default|GetDynamicMeshWorldLocation (LocalVariables|GetCataract))))
                (else
                  (CallFunction|SlicewithFreePlane (LocalVariables|GetCataract) (LocalVariables|GetComponentToSlice))))
              (return))
            (:else)))
        (:else)))))