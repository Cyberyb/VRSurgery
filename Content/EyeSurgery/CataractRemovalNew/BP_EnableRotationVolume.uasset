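; Volume actor in the cataract removal eye surgery game that lets a specific tool rotate only while it is inside the volume.
; It disables rotation on the assigned AffectedRotateTool at BeginPlay, then enables it when that tool begins overlapping the sphere and disables it again when the overlap ends.
; UpdateAffectedRotatedTool swaps in a new tool and starts it with rotation disabled.
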(event OnComponentBeginOverlap(Sphere)
  (params (OverlappedComponent :type Primitive%20Component%20Object%20Reference) (OtherActor :type Actor%20Object%20Reference) (OtherComp :type Primitive%20Component%20Object%20Reference) (OtherBodyIndex :type Integer) (bFromSweep :type Boolean) (SweepResult :type Hit%20Result%20Structure%20%28by%20ref%29))
  (bind _affectedrotatetool (Variables|Default|GetAffectedRotateTool)
    (:then
      (if (== _affectedrotatetool OtherActor)
        (Default|EnableRotation _affectedrotatetool)))
    (:else)))

(event OnComponentEndOverlap(Sphere)
  (params (OverlappedComponent :type Primitive%20Component%20Object%20Reference) (OtherActor :type Actor%20Object%20Reference) (OtherComp :type Primitive%20Component%20Object%20Reference) (OtherBodyIndex :type Integer))
  (bind _affectedrotatetool (Variables|Default|GetAffectedRotateTool)
    (:then
      (if (== _affectedrotatetool OtherActor)
        (Default|DisableRotation _affectedrotatetool)))
    (:else)))

(event EventBeginPlay
  (bind _affectedrotatetool (Variables|Default|GetAffectedRotateTool)
    (:then
      (Default|DisableRotation _affectedrotatetool))
    (:else)))

(fn ConstructionScript)

(fn UpdateAffectedRotatedTool
  (params (NewRotateTool :type BP%20Rotate%20Tool%20Object%20Reference))
  (bind _output_get (Variables|Default|SetAffectedRotateTool NewRotateTool))
  (Default|DisableRotation _output_get))