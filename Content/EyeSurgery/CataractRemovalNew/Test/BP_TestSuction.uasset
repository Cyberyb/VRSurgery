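; Test suction tool for the cataract removal surgery prototype, which carves material out of a target cataract using mesh booleans.
; The construction script copies a cube static mesh into its DynamicMesh component to serve as the cutting shape.
; Every Tick, while TargetCataract is valid, it passes that mesh and its world transform to the cataract's ApplyBooleanToAll as a Subtract.
; The overlap event is empty, so cutting does not depend on contact detection.
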(event OnComponentBeginOverlap(DynamicMesh)
  (params (OverlappedComponent :type Primitive%20Component%20Object%20Reference) (OtherActor :type Actor%20Object%20Reference) (OtherComp :type Primitive%20Component%20Object%20Reference) (OtherBodyIndex :type Integer) (bFromSweep :type Boolean) (SweepResult :type Hit%20Result%20Structure%20%28by%20ref%29)))

(event EventBeginPlay)

(event EventTick
  (params (DeltaSeconds :type Float%20%28single-precision%29))
  (bind _targetcataract (Variables|Default|GetTargetCataract))
  (Utilities|IsValid _targetcataract
    (:Is%20Valid
      (bind _returnvalue (DynamicMeshComponent|GetDynamicMesh (Variables|Default|GetDynamicMesh)))
      (Default|ApplyBooleantoAll _targetcataract _returnvalue (Transformation|GetWorldTransform (Variables|Default|GetDynamicMesh)) "Subtract"))))

(event Input|ActionEvents|InputActionSuction
  (params (Key :type Key%20Structure :default "None")))

(fn ConstructionScript
  (bind _returnvalue (DynamicMeshComponent|GetDynamicMesh (Variables|Default|GetDynamicMesh)))
  (GeometryScript|StaticMesh|CopyMeshFromStaticMesh :FromStaticMeshAsset "/Engine/BasicShapes/Cube.Cube" :ToDynamicMesh _returnvalue :Debug 0))