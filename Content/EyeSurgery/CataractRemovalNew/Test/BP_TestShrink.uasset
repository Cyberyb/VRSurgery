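; Test Blueprint in the cataract removal folder that progressively shrinks any scene components marked for shrinking.
; MarkShrink and UnmarkShrink maintain the component set, which Tick iterates while printing its count.
; Shrink scales Dynamic Mesh geometry multiplicatively through Geometry Script and subtracts from relative scale for other components.
; The fixed per-tick step is frame-rate dependent and unclamped.
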(event OnComponentBeginOverlap(Sphere)
  (params (OverlappedComponent :type Primitive%20Component%20Object%20Reference) (OtherActor :type Actor%20Object%20Reference) (OtherComp :type Primitive%20Component%20Object%20Reference) (OtherBodyIndex :type Integer) (bFromSweep :type Boolean) (SweepResult :type Hit%20Result%20Structure%20%28by%20ref%29)))

(event EventTick
  (params (DeltaSeconds :type Float%20%28single-precision%29))
  (bind _comptoshrink (Variables|Default|GetCompToShrink))
  (Development|PrintString (Utilities|String|ToString(Integer) (Utilities|Set|Length _comptoshrink)))
  (bind _result (Utilities|Set|ToArray _comptoshrink))
  (for _array_element _result
    (CallFunction|Shrink _array_element "0.050000,0.050000,0.050000")))

(fn ConstructionScript)

(fn MarkShrink
  (params (SceneComponent :type Scene%20Component%20Object%20Reference))
  (Utilities|Set|Add (Variables|Default|GetCompToShrink) SceneComponent))

(fn UnmarkShrink
  (params (SceneComponent :type Scene%20Component%20Object%20Reference))
  (Utilities|Set|Remove (Variables|Default|GetCompToShrink) SceneComponent))

(fn Shrink
  (params (SceneComponent :type Scene%20Component%20Object%20Reference) (DeltaScale :type Vector))
  (bind _relativescale3d (Variables|/Script/Engine.SceneComponent|GetRelativeScale3D SceneComponent))
  (bind _returnvalue (- _relativescale3d DeltaScale))
  (bind _asdynamic_mesh_component (Utilities|Casting|CastToDynamicMeshComponent SceneComponent)
    (:then
      (bind _returnvalue_2 (DynamicMeshComponent|GetDynamicMesh _asdynamic_mesh_component))
      (Class|GeometryScriptLibraryMeshTransformFunctions|ScaleMesh _returnvalue_2 (- "1.000000,1.000000,1.000000" DeltaScale) 0))
    (:CastFailed
      (Transformation|SetRelativeScale3D SceneComponent _returnvalue)))
  (return _returnvalue))