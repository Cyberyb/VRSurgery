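; VR cataract surgery suction tool that carves away the dynamic cataract mesh while enabled, triggered and overlapping it.
; A hidden, simplified sphere dynamic mesh is boolean-subtracted from the cataract at the suction range every tick, followed by small-component removal and simplification to limit triangle growth.
; SuctionRange overlaps track the cataract and its mesh components.
; Grab input sets the trigger or toggles tool mode, and BeginPlay updates the tip board.
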(event OnComponentBeginOverlap(SuctionRange)
  (params (OverlappedComponent :type Primitive%20Component%20Object%20Reference) (OtherActor :type Actor%20Object%20Reference) (OtherComp :type Primitive%20Component%20Object%20Reference) (OtherBodyIndex :type Integer) (bFromSweep :type Boolean) (SweepResult :type Hit%20Result%20Structure%20%28by%20ref%29))
  (bind _asbp_dynamic_cataract (Utilities|Casting|CastToBP_DynamicCataract OtherActor))
  (Variables|Default|SetCataract _asbp_dynamic_cataract)
  (bind _as动态网格体组件 (Utilities|Casting|CastToDynamicMeshComponent OtherComp))
  (Utilities|Set|Add (Variables|Default|GetOverlappingComp) _as动态网格体组件))

(event OnComponentEndOverlap(SuctionRange)
  (params (OverlappedComponent :type Primitive%20Component%20Object%20Reference) (OtherActor :type Actor%20Object%20Reference) (OtherComp :type Primitive%20Component%20Object%20Reference) (OtherBodyIndex :type Integer))
  (bind _as动态网格体组件 (Utilities|Casting|CastToDynamicMeshComponent OtherComp))
  (Utilities|Set|Remove (Variables|Default|GetOverlappingComp) _as动态网格体组件))

(event GrabKeyInput(Comp_Grab)
  (params (MComp :type BP%20M%20Comp%20Object%20Reference) (Key :type Enum_Controller_Buttons%20Enum :default "NewEnumerator1") (Set :type Boolean))
  (switch Utilities|FlowControl|Switch|SwitchonEnum_Controller_Buttons Key
    (:NewEnumerator0
      (bind _output_get (Variables|Default|SetTriggered Set))
      (if _output_get
        _))
    (:NewEnumerator3
      (if Set
        (bind _returnvalue (Actor|GetActorOfClass "/Game/EyeSurgery/BluePrint/Object/Helpers/BP_ToolModeHP.BP_ToolModeHP_C"))
        (Utilities|IsValid _returnvalue
          (:Is%20Valid
            (Default|CallToggleMode _returnvalue "NewEnumerator0" (Variables|/Game/AFCore/Blueprints/VR/MotionComponents/BP_MComp.BP_MComp_C|GetSide MComp))))))))

(event EventBeginPlay
  (bind _returnvalue (Actor|GetActorOfClass "/Game/EyeSurgery/BluePrint/UI/BP_TipBoard.BP_TipBoard_C"))
  (Utilities|IsValid _returnvalue
    (:Is%20Valid
      (Default|UpdateToolTip _returnvalue "NewEnumerator0" false))))

(event EventTick
  (params (DeltaSeconds :type Float%20%28single-precision%29))
  (bind _cataract (Variables|Default|GetCataract))
  (if (Variables|Default|GetEnabled)
    (if (and (CallFunction|IsOverlappingwithCataract) (Variables|Default|GetTriggered))
      (Utilities|IsValid _cataract
        (:Is%20Valid
          (bind _returnvalue (DynamicMeshComponent|GetDynamicMesh (Variables|Default|GetDynamicMesh)))
          (Default|ApplyBooleantoAll _cataract _returnvalue (Transformation|GetWorldTransform (Variables|Default|GetSuctionRange)) "Subtract")
          (Default|DeleteSmallComponents _cataract 2.0 2.0)
          ;[1 1 1] Direct simplification from target mesh
          (Default|SimplifyAll (Variables|Default|GetCataract)))))))

(fn ConstructionScript
  (Utilities|FlowControl|Sequence
    (:then_0
      (bind _returnvalue (DynamicMeshComponent|GetDynamicMesh (Variables|Default|GetDynamicMesh)))
      (bind _output_get (LocalVariables|SetMesh _returnvalue))
      (GeometryScript|StaticMesh|CopyMeshFromStaticMesh :FromStaticMeshAsset "/Engine/BasicShapes/Sphere.Sphere" :ToDynamicMesh _output_get :Debug 0
        (:Success
          (Rendering|SetVisibility (Variables|Default|GetDynamicMesh) false false))))
    (:then_1
      ;[1 1 1] Mitigate triangle count of target mesh after boolean operation
      (Class|GeometryScriptLibraryMeshSimplifyFunctions|ApplySimplifytoTriangleCount :TargetMesh (LocalVariables|GetMesh) :TriangleCount (Variables|Default|GetToolMeshTriangleCount) :Debug 0))))

(fn IsOverlappingwithCataract
  (return (Utilities|Set|IsNotEmpty (Variables|Default|GetOverlappingComp))))

(fn IsTriggered
  (return (Variables|Default|GetTriggered)))

(fn Enable
  (Variables|Default|SetEnabled true))

(fn Disable
  (Variables|Default|SetEnabled false))