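; Tool for the cataract removal eye surgery that rotates the target cataract as the tool's contact point moves around it.
; While enabled, each tick turns the contact point's movement around the cataract's dynamic mesh location into an axis-angle rotation via cross product and angle between vectors.
; Per-axis lock flags zero components of that rotation before it is applied through TransformAllComponent, and the previous contact location updates every tick.
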(event EventTick
  (params (DeltaSeconds :type Float%20%28single-precision%29))
  (if (Variables|Default|GetEnabled)
    (Utilities|ApplyRotation
      (:Out
        _)))
  (CallFunction|UpdatePrevLocation))

(fn ConstructionScript
  (Variables|Default|SetPrevLocation (Transformation|GetWorldLocation (Variables|Default|GetContactPoint))))

(fn ComputeRotation
  (Utilities|FlowControl|Sequence
    (:then_0
      (LocalVariables|SetCurrLocation (Transformation|GetWorldLocation (Variables|Default|GetContactPoint)))
      (LocalVariables|SetRotationCenter (Default|GetWorldDynamicMeshLocation (Variables|Default|GetCataractToRotate))))
    (:then_1
      (return (Math|Rotator|MakeRotator (.OutX (Utilities|Mask (.Roll (Math|Rotator|BreakRotator (Math|Vector|RotatorfromAxisandAngle (Math|Vector|CrossProduct (- (Variables|Default|GetPrevLocation) (LocalVariables|GetRotationCenter)) (- (LocalVariables|GetCurrLocation) (LocalVariables|GetRotationCenter))) (CallFunction|AngleBetweenTwoVectors (- (Variables|Default|GetPrevLocation) (LocalVariables|GetRotationCenter)) (- (LocalVariables|GetCurrLocation) (LocalVariables|GetRotationCenter)))))) (.Pitch (Math|Rotator|BreakRotator (Math|Vector|RotatorfromAxisandAngle (Math|Vector|CrossProduct (- (Variables|Default|GetPrevLocation) (LocalVariables|GetRotationCenter)) (- (LocalVariables|GetCurrLocation) (LocalVariables|GetRotationCenter))) (CallFunction|AngleBetweenTwoVectors (- (Variables|Default|GetPrevLocation) (LocalVariables|GetRotationCenter)) (- (LocalVariables|GetCurrLocation) (LocalVariables|GetRotationCenter)))))) (.Yaw (Math|Rotator|BreakRotator (Math|Vector|RotatorfromAxisandAngle (Math|Vector|CrossProduct (- (Variables|Default|GetPrevLocation) (LocalVariables|GetRotationCenter)) (- (LocalVariables|GetCurrLocation) (LocalVariables|GetRotationCenter))) (CallFunction|AngleBetweenTwoVectors (- (Variables|Default|GetPrevLocation) (LocalVariables|GetRotationCenter)) (- (LocalVariables|GetCurrLocation) (LocalVariables|GetRotationCenter)))))) (not (Variables|Default|GetLockX)) (not (Variables|Default|GetLockY)) (not (Variables|Default|GetLockZ)))) (.OutY (Utilities|Mask (.Roll (Math|Rotator|BreakRotator (Math|Vector|RotatorfromAxisandAngle (Math|Vector|CrossProduct (- (Variables|Default|GetPrevLocation) (LocalVariables|GetRotationCenter)) (- (LocalVariables|GetCurrLocation) (LocalVariables|GetRotationCenter))) (CallFunction|AngleBetweenTwoVectors (- (Variables|Default|GetPrevLocation) (LocalVariables|GetRotationCenter)) (- (LocalVariables|GetCurrLocation) (LocalVariables|GetRotationCenter)))))) (.Pitch (Math|Rotator|BreakRotator (Math|Vector|RotatorfromAxisandAngle (Math|Vector|CrossProduct (- (Variables|Default|GetPrevLocation) (LocalVariables|GetRotationCenter)) (- (LocalVariables|GetCurrLocation) (LocalVariables|GetRotationCenter))) (CallFunction|AngleBetweenTwoVectors (- (Variables|Default|GetPrevLocation) (LocalVariables|GetRotationCenter)) (- (LocalVariables|GetCurrLocation) (LocalVariables|GetRotationCenter)))))) (.Yaw (Math|Rotator|BreakRotator (Math|Vector|RotatorfromAxisandAngle (Math|Vector|CrossProduct (- (Variables|Default|GetPrevLocation) (LocalVariables|GetRotationCenter)) (- (LocalVariables|GetCurrLocation) (LocalVariables|GetRotationCenter))) (CallFunction|AngleBetweenTwoVectors (- (Variables|Default|GetPrevLocation) (LocalVariables|GetRotationCenter)) (- (LocalVariables|GetCurrLocation) (LocalVariables|GetRotationCenter)))))) (not (Variables|Default|GetLockX)) (not (Variables|Default|GetLockY)) (not (Variables|Default|GetLockZ)))) (.OutZ (Utilities|Mask (.Roll (Math|Rotator|BreakRotator (Math|Vector|RotatorfromAxisandAngle (Math|Vector|CrossProduct (- (Variables|Default|GetPrevLocation) (LocalVariables|GetRotationCenter)) (- (LocalVariables|GetCurrLocation) (LocalVariables|GetRotationCenter))) (CallFunction|AngleBetweenTwoVectors (- (Variables|Default|GetPrevLocation) (LocalVariables|GetRotationCenter)) (- (LocalVariables|GetCurrLocation) (LocalVariables|GetRotationCenter)))))) (.Pitch (Math|Rotator|BreakRotator (Math|Vector|RotatorfromAxisandAngle (Math|Vector|CrossProduct (- (Variables|Default|GetPrevLocation) (LocalVariables|GetRotationCenter)) (- (LocalVariables|GetCurrLocation) (LocalVariables|GetRotationCenter))) (CallFunction|AngleBetweenTwoVectors (- (Variables|Default|GetPrevLocation) (LocalVariables|GetRotationCenter)) (- (LocalVariables|GetCurrLocation) (LocalVariables|GetRotationCenter)))))) (.Yaw (Math|Rotator|BreakRotator (Math|Vector|RotatorfromAxisandAngle (Math|Vector|CrossProduct (- (Variables|Default|GetPrevLocation) (LocalVariables|GetRotationCenter)) (- (LocalVariables|GetCurrLocation) (LocalVariables|GetRotationCenter))) (CallFunction|AngleBetweenTwoVectors (- (Variables|Default|GetPrevLocation) (LocalVariables|GetRotationCenter)) (- (LocalVariables|GetCurrLocation) (LocalVariables|GetRotationCenter)))))) (not (Variables|Default|GetLockX)) (not (Variables|Default|GetLockY)) (not (Variables|Default|GetLockZ)))))))))

(fn UpdatePrevLocation
  (Variables|Default|SetPrevLocation (Transformation|GetWorldLocation (Variables|Default|GetContactPoint))))

(fn EnableRotation
  (Variables|Default|SetEnabled true))

(fn DisableRotation
  (Variables|Default|SetEnabled false))