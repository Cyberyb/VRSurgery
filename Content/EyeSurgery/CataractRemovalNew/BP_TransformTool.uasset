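; Surgical tool for the cataract removal procedure that rotates or translates dynamic mesh pieces of a cataract by following its tip's per-frame motion.
; Rotate mode turns all pieces by the tip's swept angle around the mesh center, with axis locks and a multiplier, while inside a BP_RotateLimiter.
; Translate mode moves the last overlapped mesh component by the tip's offset.
; Paired DoOnce nodes signal rotation begin, and end on disable.
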(event OnComponentBeginOverlap(TransformTip)
  (params (OverlappedComponent :type Primitive%20Component%20Object%20Reference) (OtherActor :type Actor%20Object%20Reference) (OtherComp :type Primitive%20Component%20Object%20Reference) (OtherBodyIndex :type Integer) (bFromSweep :type Boolean) (SweepResult :type Hit%20Result%20Structure%20%28by%20ref%29))
  (Utilities|FlowControl|Sequence
    (:then_0
      (Utilities|Casting|CastToBP_RotateLimiter OtherActor)
      (Variables|Default|SetInsideLimiter true))
    (:then_1
      (bind _as动态网格体组件 (Utilities|Casting|CastToDynamicMeshComponent OtherComp))
      (Variables|Default|SetMeshComponentToMove _as动态网格体组件))))

(event OnComponentEndOverlap(TransformTip)
  (params (OverlappedComponent :type Primitive%20Component%20Object%20Reference) (OtherActor :type Actor%20Object%20Reference) (OtherComp :type Primitive%20Component%20Object%20Reference) (OtherBodyIndex :type Integer))
  (Utilities|Casting|CastToBP_RotateLimiter OtherActor)
  (Variables|Default|SetInsideLimiter false))

(event Custom|RotationEnabled
  (Utilities|FlowControl|DoOnce false
    (:Completed
      (Default|CallRotateBegins)
      (Utilities|FlowControl|DoOnce false) ; enters at Reset
    )))

(event Custom|RotationDisabled
  (Utilities|FlowControl|DoOnce false
    (:Completed
      (Default|CallRotateEnds)
      (Utilities|FlowControl|DoOnce false) ; enters at Reset
    )))

(event EventTick
  (params (DeltaSeconds :type Float%20%28single-precision%29))
  (bind _mode (Variables|Default|GetMode))
  (if (Variables|Default|GetEnabled)
    (switch Utilities|FlowControl|Switch|SwitchonE_TransformMode _mode
      (:NewEnumerator0
        (if (Variables|Default|GetInsideLimiter)
          (Utilities|ApplyRotation
            (:Out
              (CallFunction|RotationEnabled)))))
      (:NewEnumerator1
        (Utilities|ApplyOffset)))
    (else
      (switch Utilities|FlowControl|Switch|SwitchonE_TransformMode _mode
        (:NewEnumerator0
          (CallFunction|RotationDisabled))
        (:NewEnumerator1
          _))))
  (CallFunction|UpdatePrevLocation))

(fn ConstructionScript
  (Variables|Default|SetPrevLocation (Transformation|GetWorldLocation (Variables|Default|GetTransformTip))))

(fn UpdatePrevLocation
  (Variables|Default|SetPrevLocation (Transformation|GetWorldLocation (Variables|Default|GetTransformTip))))

(fn Enable
  (Variables|Default|SetEnabled true))

(fn Disable
  (Variables|Default|SetEnabled false))

(fn IsInsideLimiter
  (return (Variables|Default|GetInsideLimiter)))

(fn ComputeRotation
  (Utilities|FlowControl|Sequence
    (:then_0
      (LocalVariables|SetCurrLocation (Transformation|GetWorldLocation (Variables|Default|GetTransformTip)))
      (LocalVariables|SetRotationCenter (Default|GetDynamicMeshWorldLocation (Variables|Rotation|GetCataractToTransform))))
    (:then_1
      (return (Math|Rotator|MakeRotator (.OutX (Utilities|Float3Mask (.Roll (Math|Rotator|BreakRotator (Math|Vector|RotatorfromAxisandAngle (Math|Vector|CrossProduct (- (Variables|Default|GetPrevLocation) (LocalVariables|GetRotationCenter)) (- (LocalVariables|GetCurrLocation) (LocalVariables|GetRotationCenter))) (CallFunction|AngleBetweenTwoVectors (- (Variables|Default|GetPrevLocation) (LocalVariables|GetRotationCenter)) (- (LocalVariables|GetCurrLocation) (LocalVariables|GetRotationCenter)))))) (.Pitch (Math|Rotator|BreakRotator (Math|Vector|RotatorfromAxisandAngle (Math|Vector|CrossProduct (- (Variables|Default|GetPrevLocation) (LocalVariables|GetRotationCenter)) (- (LocalVariables|GetCurrLocation) (LocalVariables|GetRotationCenter))) (CallFunction|AngleBetweenTwoVectors (- (Variables|Default|GetPrevLocation) (LocalVariables|GetRotationCenter)) (- (LocalVariables|GetCurrLocation) (LocalVariables|GetRotationCenter)))))) (.Yaw (Math|Rotator|BreakRotator (Math|Vector|RotatorfromAxisandAngle (Math|Vector|CrossProduct (- (Variables|Default|GetPrevLocation) (LocalVariables|GetRotationCenter)) (- (LocalVariables|GetCurrLocation) (LocalVariables|GetRotationCenter))) (CallFunction|AngleBetweenTwoVectors (- (Variables|Default|GetPrevLocation) (LocalVariables|GetRotationCenter)) (- (LocalVariables|GetCurrLocation) (LocalVariables|GetRotationCenter)))))) (not (Variables|Rotation|GetLockX)) (not (Variables|Rotation|GetLockY)) (not (Variables|Rotation|GetLockZ)))) (.OutY (Utilities|Float3Mask (.Roll (Math|Rotator|BreakRotator (Math|Vector|RotatorfromAxisandAngle (Math|Vector|CrossProduct (- (Variables|Default|GetPrevLocation) (LocalVariables|GetRotationCenter)) (- (LocalVariables|GetCurrLocation) (LocalVariables|GetRotationCenter))) (CallFunction|AngleBetweenTwoVectors (- (Variables|Default|GetPrevLocation) (LocalVariables|GetRotationCenter)) (- (LocalVariables|GetCurrLocation) (LocalVariables|GetRotationCenter)))))) (.Pitch (Math|Rotator|BreakRotator (Math|Vector|RotatorfromAxisandAngle (Math|Vector|CrossProduct (- (Variables|Default|GetPrevLocation) (LocalVariables|GetRotationCenter)) (- (LocalVariables|GetCurrLocation) (LocalVariables|GetRotationCenter))) (CallFunction|AngleBetweenTwoVectors (- (Variables|Default|GetPrevLocation) (LocalVariables|GetRotationCenter)) (- (LocalVariables|GetCurrLocation) (LocalVariables|GetRotationCenter)))))) (.Yaw (Math|Rotator|BreakRotator (Math|Vector|RotatorfromAxisandAngle (Math|Vector|CrossProduct (- (Variables|Default|GetPrevLocation) (LocalVariables|GetRotationCenter)) (- (LocalVariables|GetCurrLocation) (LocalVariables|GetRotationCenter))) (CallFunction|AngleBetweenTwoVectors (- (Variables|Default|GetPrevLocation) (LocalVariables|GetRotationCenter)) (- (LocalVariables|GetCurrLocation) (LocalVariables|GetRotationCenter)))))) (not (Variables|Rotation|GetLockX)) (not (Variables|Rotation|GetLockY)) (not (Variables|Rotation|GetLockZ)))) (.OutZ (Utilities|Float3Mask (.Roll (Math|Rotator|BreakRotator (Math|Vector|RotatorfromAxisandAngle (Math|Vector|CrossProduct (- (Variables|Default|GetPrevLocation) (LocalVariables|GetRotationCenter)) (- (LocalVariables|GetCurrLocation) (LocalVariables|GetRotationCenter))) (CallFunction|AngleBetweenTwoVectors (- (Variables|Default|GetPrevLocation) (LocalVariables|GetRotationCenter)) (- (LocalVariables|GetCurrLocation) (LocalVariables|GetRotationCenter)))))) (.Pitch (Math|Rotator|BreakRotator (Math|Vector|RotatorfromAxisandAngle (Math|Vector|CrossProduct (- (Variables|Default|GetPrevLocation) (LocalVariables|GetRotationCenter)) (- (LocalVariables|GetCurrLocation) (LocalVariables|GetRotationCenter))) (CallFunction|AngleBetweenTwoVectors (- (Variables|Default|GetPrevLocation) (LocalVariables|GetRotationCenter)) (- (LocalVariables|GetCurrLocation) (LocalVariables|GetRotationCenter)))))) (.Yaw (Math|Rotator|BreakRotator (Math|Vector|RotatorfromAxisandAngle (Math|Vector|CrossProduct (- (Variables|Default|GetPrevLocation) (LocalVariables|GetRotationCenter)) (- (LocalVariables|GetCurrLocation) (LocalVariables|GetRotationCenter))) (CallFunction|AngleBetweenTwoVectors (- (Variables|Default|GetPrevLocation) (LocalVariables|GetRotationCenter)) (- (LocalVariables|GetCurrLocation) (LocalVariables|GetRotationCenter)))))) (not (Variables|Rotation|GetLockX)) (not (Variables|Rotation|GetLockY)) (not (Variables|Rotation|GetLockZ)))))))))

(fn ComputeOffset
  (return (- (Transformation|GetWorldLocation (Variables|Default|GetTransformTip)) (Variables|Default|GetPrevLocation))))

(fn SwitchMode
  (params (NewMode :type E_TransformMode%20Enum :default "NewEnumerator0"))
  (Variables|Default|SetMode NewMode)
  (return))