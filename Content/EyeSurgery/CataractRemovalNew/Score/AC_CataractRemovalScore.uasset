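; Actor component that scores a cataract removal in the eye surgery game by comparing a recorded attempt to ExpectedRecord.
; ComputeScore returns two all-or-nothing scores: operation order and mesh count.
; SameSequence compares operations index by index without checking array lengths.
; As written, the mesh count score is awarded when MaxComponentCount differs from the expected value.
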(event EventBeginPlay)

(event EventTick
  (params (DeltaSeconds :type Float%20%28single-precision%29)))

(fn ComputeScore
  (params (Record :type F%20Cataract%20Removal%20Rec%20Structure))
  (bind _expectedrecord (Variables|Default|GetExpectedRecord))
  (Utilities|FlowControl|Sequence
    (:then_0
      (LocalVariables|SetCntScore (select (!= (.maxcomponentcount Record) (.maxcomponentcount _expectedrecord)) 5e+01 0.0)))
    (:then_1
      (bind _same (CallFunction|SameSequence (.operations Record) (.operations _expectedrecord)))
      (LocalVariables|SetOpScore (select _same 5e+01 0.0)))
    (:then_2
      (return (LocalVariables|GetOpScore) (LocalVariables|GetCntScore)))))

(fn SameSequence
  (params (Operations1 :type Array%20of%20E_CataractRemovalOp%20Enums :default "NewEnumerator4") (Operations2 :type Array%20of%20E_CataractRemovalOp%20Enums :default "NewEnumerator4"))
  (bind (_array_element _array_index) (Utilities|Array|ForEachLoopwithBreak Operations1)
    (:LoopBody
      (if (not (Utilities|Enum|Equal(Enum) _array_element (Utilities|Array|Get(acopy) Operations2 _array_index)))
        (return false)))
    (:Completed
      (return true))))