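; BP_SliceTool is a grabbable surgical tool that slices or rotates the dynamic-mesh cataract in the eye surgery game.
; Each tick picks its behavior: slicing when it and a nearby suction tool are both triggered, rotation when triggered alone, otherwise idle.
; In slice mode, tip overlaps cut one or all cataract components on a cooldown.
; The cut plane follows either the tool's rotation or an angle around a chosen axis.
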(event OnComponentBeginOverlap(TipCollision)
  (params (OverlappedComponent :type Primitive%20Component%20Object%20Reference) (OtherActor :type Actor%20Object%20Reference) (OtherComp :type Primitive%20Component%20Object%20Reference) (OtherBodyIndex :type Integer) (bFromSweep :type Boolean) (SweepResult :type Hit%20Result%20Structure%20%28by%20ref%29))
  (if (Utilities|Enum|Equal(Enum) (Variables|Default|GetBehavior) "NewEnumerator1")
    (bind _asbp_dynamic_cataract (Utilities|Casting|CastToBP_DynamicCataract OtherActor))
    (bind _as动态网格体组件 (Utilities|Casting|CastToDynamicMeshComponent OtherComp))
    ;[1 1 1] Cooldown
    (Utilities|FlowControl|DoOnce false
      (:Completed
        (Utilities|Time|SetTimerbyEvent (delegate Custom|EnableSlicing) (Variables|Slice|GetSliceCooldown))
        (if (Variables|Slice|GetSliceAlongAxis)
          (CallFunction|SlicewithDirection _asbp_dynamic_cataract _as动态网格体组件 (- (Transformation|GetWorldLocation (Variables|Default|GetTipCollision)) (Default|GetWorldDynamicMeshLocation _asbp_dynamic_cataract)))
          (else
            (CallFunction|SlicewithFreePlane _asbp_dynamic_cataract _as动态网格体组件)))))))

(event GrabKeyInput(Comp_Grab)
  (params (MComp :type BP%20M%20Comp%20Object%20Reference) (Key :type Enum_Controller_Buttons%20Enum :default "NewEnumerator1") (Set :type Boolean))
  (switch Utilities|FlowControl|Switch|SwitchonEnum_Controller_Buttons Key
    (:NewEnumerator0
      (Variables|Slice|SetTriggered Set))))

(event OnComponentBeginOverlap(SliceModeDetection)
  (params (OverlappedComponent :type Primitive%20Component%20Object%20Reference) (OtherActor :type Actor%20Object%20Reference) (OtherComp :type Primitive%20Component%20Object%20Reference) (OtherBodyIndex :type Integer) (bFromSweep :type Boolean) (SweepResult :type Hit%20Result%20Structure%20%28by%20ref%29))
  (bind _asbp_suction_tool (Utilities|Casting|CastToBP_SuctionTool OtherActor))
  (Variables|Default|SetNearSuctionTool _asbp_suction_tool))

(event OnComponentEndOverlap(SliceModeDetection)
  (params (OverlappedComponent :type Primitive%20Component%20Object%20Reference) (OtherActor :type Actor%20Object%20Reference) (OtherComp :type Primitive%20Component%20Object%20Reference) (OtherBodyIndex :type Integer))
  (Utilities|Casting|CastToBP_SuctionTool OtherActor)
  (Variables|Default|SetNearSuctionTool 0))

(event Custom|EnableSlicing
  ;[1 1 1] Cooldown
  (Utilities|FlowControl|DoOnce false) ; enters at Reset
)

(event EventBeginPlay)

(event Collision|EventActorBeginOverlap
  (params (OtherActor :type Actor%20Object%20Reference)))

(event EventTick
  (params (DeltaSeconds :type Float%20%28single-precision%29))
  (|CallParentFunction DeltaSeconds)
  (Utilities|UpdateToolBehavior
    (:Out
      (Utilities|SetRotationMode
        (:Out
          (Development|PrintString (Utilities|String|EnumtoString (Variables|Default|GetBehavior))))))))

(fn ConstructionScript
  (bind _returnvalue (Actor|GetActorOfClass "/Game/EyeSurgery/CataractRemovalNew/BP_DynamicCataract.BP_DynamicCataract_C"))
  (Utilities|IsValid _returnvalue
    (:Is%20Valid
      (Variables|Default|SetCataractToRotate _returnvalue))))

(fn SlicewithFreePlane
  (params (Cataract :type BP%20Dynamic%20Cataract%20Object%20Reference) (ComponentToSlice :type Dynamic%20Mesh%20Component%20Object%20Reference))
  (bind _returnvalue (Transformation|GetActorRotation))
  (bind _returnvalue_2 (Transformation|GetActorLocation Cataract))
  (bind _gapwidth (Variables|Slice|GetGapWidth))
  (bind _tipcollision (Variables|Default|GetTipCollision))
  (bind _returnvalue_3 (Transformation|GetWorldLocation _tipcollision))
  (bind _returnvalue_4 (- _returnvalue_3 _returnvalue_2))
  (if (Variables|Slice|GetSliceThroughAllComponents)
    (Default|SliceAll Cataract (Math|Transform|MakeTransform _returnvalue_4 _returnvalue "1.000000,1.000000,1.000000") (Utilities|Struct|MakeGeometryScriptMeshPlaneSliceOptions true true _gapwidth 1.0))
    (else
      (Default|SliceComponent Cataract ComponentToSlice (Math|Transform|MakeTransform _returnvalue_4 _returnvalue "1.000000,1.000000,1.000000") (Utilities|Struct|MakeGeometryScriptMeshPlaneSliceOptions true true _gapwidth 1.0)))))

(fn SlicewithDirection
  (params (Cataract :type BP%20Dynamic%20Cataract%20Object%20Reference) (ComponentToSlice :type Dynamic%20Mesh%20Component%20Object%20Reference) (PlaneVec :type Vector))
  (bind _rotation (CallFunction|GetSliceRotationAlongY PlaneVec))
  (bind _rotation_2 (CallFunction|GetSliceRotationAlongZ PlaneVec))
  (bind _rotation_3 (CallFunction|GetSliceRotationAlongX PlaneVec))
  (bind _totalmeshtransform (Variables|/Game/EyeSurgery/CataractRemovalNew/BP_DynamicCataract.BP_DynamicCataract_C|GetTotalMeshTransform Cataract))
  (bind _slicedirection (Variables|Slice|GetSliceDirection))
  (bind _gapwidth (Variables|Slice|GetGapWidth))
  (bind _returnvalue (Utilities|Select :Index _slicedirection :NewEnumerator0 _rotation_3 :NewEnumerator1 _rotation :NewEnumerator2 _rotation_2))
  (bind _returnvalue_2 (Math|Transform|MakeTransform (.location _totalmeshtransform) _returnvalue))
  (if (Variables|Slice|GetSliceThroughAllComponents)
    (Default|SliceAll Cataract _returnvalue_2 (Utilities|Struct|MakeGeometryScriptMeshPlaneSliceOptions true true _gapwidth 1.0))
    (else
      (Default|SliceComponent Cataract ComponentToSlice _returnvalue_2 (Utilities|Struct|MakeGeometryScriptMeshPlaneSliceOptions true true _gapwidth 1.0)))))

(fn GetSliceRotationAlongX
  (params (PlaneVec :type Vector))
  (bind (_x _y _z) (Math|Vector|BreakVector PlaneVec))
  (return (Math|Rotator|MakeRotator (* (CallFunction|AngleBetweenTwoVectors (Math|Vector|MakeVector 0.0 _y _z) "0,1.000000, 0") (* (Math|Float|Sign(Float) _z) -1.0)) 0.0 0.0)))

(fn GetSliceRotationAlongY
  (params (PlaneVec :type Vector))
  (bind (_x _y _z) (Math|Vector|BreakVector PlaneVec))
  (return (Math|Rotator|MakeRotator 0.0 (* (CallFunction|AngleBetweenTwoVectors (Math|Vector|MakeVector _x 0.0 _z) "1.000000,0.000000, 0") (Math|Float|Sign(Float) _z)) 0.0)))

(fn GetSliceRotationAlongZ
  (params (PlaneVec :type Vector))
  (bind (_x _y) (Math|Vector|BreakVector PlaneVec))
  (return (Math|Rotator|MakeRotator 9e+01 0.0 (* (CallFunction|AngleBetweenTwoVectors (Math|Vector|MakeVector _x _y 0.0) "1.000000,0.000000, 0") (Math|Float|Sign(Float) _y)))))

(fn SuctionToolIsNear
  (return (Utilities|IsValid (Variables|Default|GetNearSuctionTool))))

(fn SliceToolTriggered
  (return (Variables|Slice|GetTriggered)))

(fn SuctionToolTriggered
  (bind _nearsuctiontool (Variables|Default|GetNearSuctionTool)
    (:then
      (return (Default|IsTriggered _nearsuctiontool)))
    (:else
      (return false))))