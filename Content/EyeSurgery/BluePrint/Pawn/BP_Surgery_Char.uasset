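; Player pawn for the eye surgery scene, built on a parent with motion controllers, that keeps the view confined to the operating area.
; On BeginPlay it restricts movement abilities and caches the level's BP_CameraRange actor.
; Each tick it clamps the main camera's world pitch and yaw to a narrow band, preserving roll.
; When the camera leaves the range sphere, it nudges it one unit per tick back toward the center.
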(event EventBeginPlay
  (|CallParentFunction)
  (CallFunction|RestrictMovementAbilities true)
  (bind _returnvalue (Actor|GetActorOfClass "/Game/EyeSurgery/BluePrint/Object/Helpers/BP_CameraRange.BP_CameraRange_C"))
  (Variables|Default|SetCameraRangeRef _returnvalue))

(event Collision|EventActorBeginOverlap
  (params (OtherActor :type Actor%20Object%20Reference)))

(event EventTick
  (params (DeltaSeconds :type Float%20%28single-precision%29))
  (bind _maincamera (Variables|Default|GetMainCamera))
  (bind _maincamera_2 (Variables|Default|GetMainCamera))
  (bind _camerarangeref (Variables|Default|GetCameraRangeRef))
  (bind _returnvalue (Transformation|GetWorldRotation _maincamera))
  (bind _returnvalue_2 (Transformation|GetWorldLocation _maincamera_2))
  (bind _sphere (Variables|/Game/EyeSurgery/BluePrint/Object/Helpers/BP_CameraRange.BP_CameraRange_C|GetSphere _camerarangeref))
  (bind _returnvalue_3 (Transformation|GetWorldLocation _sphere))
  (|CallParentFunction DeltaSeconds)
  (Transformation|SetWorldRotation _maincamera (Math|Rotator|MakeRotator (.roll _returnvalue) (Math|Float|Clamp(Float) (.pitch _returnvalue) -1e+01 1e+01) (Math|Float|Clamp(Float) (.yaw _returnvalue) -1e+01 1e+01)) false false)
  (if (> (Math|Vector|Distance(Vector) _returnvalue_3 _returnvalue_2) (Variables|/Script/Engine.SphereComponent|GetSphereRadius _sphere))
    (Transformation|SetWorldLocation _maincamera_2 (+ (Math|Vector|Normalize (- _returnvalue_3 _returnvalue_2)) _returnvalue_2) false false)))

(fn ConstructionScript
  (|CallParentFunction))