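; BP_Eye_VR_Char is the eye-surgery VR character, adding a toggle for the world-space menu board.
; The ShoulderRight input spawns BP_Board_Menu ahead of and above player pawn 0, rotated 180 degrees from it, or destroys any existing boards.
; BeginPlay and Tick are disabled stubs, and an unconnected Comp_PawnUI call to spawn W_ToolsMenu never runs.
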(event EventBeginPlay
  (|CallParentFunction) ; 此节点被禁用，将不会被调用。\n从引脚连出引线来编译功能。
)

(event Collision|EventActorBeginOverlap
  (params (OtherActor :type Actor%20Object%20Reference)))

(event EventTick
  (params (DeltaSeconds :type Float%20%28single-precision%29))
  (|CallParentFunction DeltaSeconds) ; 此节点被禁用，将不会被调用。\n从引脚连出引线来编译功能。
)

(event Input|ActionEvents|InputActionShoulderRight
  (params (Key :type Key%20Structure :default "None"))
  (bind _returnvalue (Game|Player|GetPlayerPawn 0))
  (bind _returnvalue_2 (Transformation|GetActorTransform _returnvalue))
  ;[1 1 1] 按菜单键生成Menu界面
  (:Pressed
    (bind _outactors (Actor|GetAllActorsOfClass "/Game/EyeSurgery/BluePrint/UI/BP_Board_Menu.BP_Board_Menu_C"))
    (if (Utilities|Array|IsEmpty _outactors)
      (Game|SpawnActorfromClass "/Game/EyeSurgery/BluePrint/UI/BP_Board_Menu.BP_Board_Menu_C" (Math|Transform|MakeTransform (+ (Math|Vector|MakeVector (.x (.location _returnvalue_2)) (.y (.location _returnvalue_2)) (+ (.z (.location _returnvalue_2)) 75.0)) (* (Transformation|GetActorForwardVector _returnvalue) 1e+02)) (Math|Rotator|CombineRotators (.rotation _returnvalue_2) "0,180.000000, 0") (.scale _returnvalue_2)) "Undefined" 0 0)
      (else
        (Actor|DestroyActor _outactors)))))

(event Input|ActionEvents|InputActionShoulderLeft
  (params (Key :type Key%20Structure :default "None"))
  ;[1 1 1] 按菜单键生成Menu界面
)

(fn ConstructionScript
  (|CallParentFunction))