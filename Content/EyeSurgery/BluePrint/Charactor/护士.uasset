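; Nurse (护士) character for the EyeSurgery game that turns to face the player when its Comp_Switch component changes state.
; The state change prints a debug "Hello", casts the player pawn to BP_Eye_DT_Char and restarts RotateTimeline.
; Each timeline update eases the capsule from its current rotation toward a look-at rotation on the player, with yaw offset by -90 degrees.
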(event OnStateChanged(Comp_Switch)
  (params (SourceInfo :type Struct%20Component%20Source%20Info%20Structure) (Value :type Boolean))
  (bind _capsulecomponent (Variables|Collision|GetCapsuleComponent))
  (Development|PrintString "Hello")
  (bind _asbp_eye_dt_char (Utilities|Casting|CastToBP_Eye_DT_Char (Game|Player|GetPlayerPawn 0)))
  (bind _插值旋转 (Timeline|RotateTimeline PlayFromStart)
    (:Update
      (Transformation|SetWorldRotation _capsulecomponent (Math|Interpolation|Ease "SinusoidalInOut" _插值旋转 (Transformation|GetWorldRotation (Variables|Collision|GetCapsuleComponent)) (Math|Rotator|MakeRotator (.roll (Math|Rotator|FindLookatRotation (Transformation|GetWorldLocation _capsulecomponent) (Transformation|GetWorldLocation (Variables|/Script/Engine.Actor|GetRootComponent _asbp_eye_dt_char)))) (.pitch (Math|Rotator|FindLookatRotation (Transformation|GetWorldLocation _capsulecomponent) (Transformation|GetWorldLocation (Variables|/Script/Engine.Actor|GetRootComponent _asbp_eye_dt_char)))) (- (.yaw (Math|Rotator|FindLookatRotation (Transformation|GetWorldLocation _capsulecomponent) (Transformation|GetWorldLocation (Variables|/Script/Engine.Actor|GetRootComponent _asbp_eye_dt_char)))) 9e+01)) true) false false))))

(event EventBeginPlay)

(event Collision|EventActorBeginOverlap
  (params (OtherActor :type Actor%20Object%20Reference)))

(event EventTick
  (params (DeltaSeconds :type Float%20%28single-precision%29)))

(fn ConstructionScript)