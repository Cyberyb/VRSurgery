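; BP_SurgeryVoice triggers the voice lines for each step of a cataract surgery sequence, from incision through lens insertion to incision sealing.
; On BeginPlay it finds and caches the BP_VoiceManage actor, then plays the first step's narration.
; PlayVoice maps a step ID to PlayNextSound calls on that manager, spacing multi-line steps with hard-coded Delays.
; Some timed chains, including a longer phacoemulsification sequence, are left unconnected and never run.
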(event Custom|PlayVoice
  (params (VoiceID :type Integer))
  (bind _voicemanageref (Variables|Default|GetVoiceManageRef))
  (bind _voicemanageref_2 (Variables|Default|GetVoiceManageRef))
  (switch int VoiceID
    (:0
      ;[1 1 1] Step1切口
      (Default|PlayNextSound _voicemanageref "/Game/EyeSurgery/Sounds/手术/Step1/1.1")
      (Utilities|FlowControl|Delay 5.0)
      (Default|PlayNextSound _voicemanageref "/Game/EyeSurgery/Sounds/手术/Step1/2.2"))
    (:1
      ;[1 1 1] Step2注射粘弹剂
      (Default|PlayNextSound (Variables|Default|GetVoiceManageRef) "/Game/EyeSurgery/Sounds/手术/Step2/1.1"))
    (:2
      ;[1 1 1] Step3撕嚢1
      (Default|PlayNextSound (Variables|Default|GetVoiceManageRef) "/Game/EyeSurgery/Sounds/手术/Step3/2.2"))
    (:3
      ;[1 1 1] Step3撕嚢2
      (Default|PlayNextSound (Variables|Default|GetVoiceManageRef) "/Game/EyeSurgery/Sounds/手术/Step3/3.3"))
    (:4
      ;[1 1 1] Step3撕嚢3
      (Default|PlayNextSound (Variables|Default|GetVoiceManageRef) "/Game/EyeSurgery/Sounds/手术/Step3/4.4"))
    (:5
      ;[1 1 1] Step4水分离
      (Default|PlayNextSound _voicemanageref_2 "/Game/EyeSurgery/Sounds/手术/Step4/1.1")
      (Utilities|FlowControl|Delay 6.6)
      (Default|PlayNextSound _voicemanageref_2 "/Game/EyeSurgery/Sounds/手术/Step4/2.2")
      (Utilities|FlowControl|Delay 4.4)
      (Default|PlayNextSound _voicemanageref_2 "/Game/EyeSurgery/Sounds/手术/Step4/3.3"))
    (:6
      ;[1 1 1] Step5超声乳化1
      (Default|PlayNextSound (Variables|Default|GetVoiceManageRef) "/Game/EyeSurgery/Sounds/手术/Step5/5月10日_1_.5月10日_1_"))
    (:7
      ;[1 1 1] Step6吸取皮质
      (Default|PlayNextSound (Variables|Default|GetVoiceManageRef) "/Game/EyeSurgery/Sounds/手术/Step6/2.2"))
    (:8
      ;[1 1 1] Step7注射粘弹剂
      (Default|PlayNextSound (Variables|Default|GetVoiceManageRef) "/Game/EyeSurgery/Sounds/手术/Step7/1.1"))
    (:9
      ;[1 1 1] Step8注入晶状体
      (Default|PlayNextSound (Variables|Default|GetVoiceManageRef) "/Game/EyeSurgery/Sounds/手术/Step8/1.1"))
    (:10
      ;[1 1 1] Step9抽吸粘弹剂
      (Default|PlayNextSound (Variables|Default|GetVoiceManageRef) "/Game/EyeSurgery/Sounds/手术/Step9/2.2"))
    (:11
      ;[1 1 1] Step10水密切口
      (Default|PlayNextSound (Variables|Default|GetVoiceManageRef) "/Game/EyeSurgery/Sounds/手术/Step10/1.1"))))

(event EventBeginPlay
  (Utilities|FlowControl|Sequence
    (:then_0
      (bind _returnvalue (Actor|GetActorOfClass "/Game/EyeSurgery/BluePrint/Voice/BP_VoiceManage.BP_VoiceManage_C"))
      (Utilities|IsValid _returnvalue
        (:Is%20Valid
          (Variables|Default|SetVoiceManageRef _returnvalue))))
    (:then_1
      (CallFunction|PlayVoice))))

(event Collision|EventActorBeginOverlap
  (params (OtherActor :type Actor%20Object%20Reference)))

(event EventTick
  (params (DeltaSeconds :type Float%20%28single-precision%29)))

(fn ConstructionScript)