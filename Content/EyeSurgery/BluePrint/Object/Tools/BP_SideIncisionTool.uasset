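; BP_SideIncisionTool is an eye surgery tool that cuts a side incision on BP_TestEyeball, shown as a decal.
; On tip overlap it spawns an attached incision decal, placed at the tip with the reference decal's rotation, optionally only once.
; Each tick, the tip's farthest distance from its entry point becomes Depth, which lerps decal scale up to a maximum.
; Ending overlap clears the tracked eyeball, decal and depth.
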(event OnComponentBeginOverlap(TipCollision)
  (params (OverlappedComponent :type Primitive%20Component%20Object%20Reference) (OtherActor :type Actor%20Object%20Reference) (OtherComp :type Primitive%20Component%20Object%20Reference) (OtherBodyIndex :type Integer) (bFromSweep :type Boolean) (SweepResult :type Hit%20Result%20Structure%20%28by%20ref%29))
  (bind _asbp_test_eyeball (Utilities|Casting|CastToBP_TestEyeball OtherActor))
  (if (not (and (Variables|Incision|GetSpawnOnlyOnce) (Variables|Default|GetHaveSpawned)))
    (bind _newdecal (CallFunction|SpawnDecalonEyeball _asbp_test_eyeball "/Game/EyeSurgery/Incision/MI_Incision.MI_Incision" (Variables|/Script/Engine.DecalComponent|GetDecalSize (Variables|Default|GetRefDecal)) "Side"))
    (Utilities|PrepareforIncision _asbp_test_eyeball _newdecal 0.0
      (:Out
        (Variables|Default|SetHaveSpawned true)
        (Utilities|InitializeSpawnedDecalwithRef)
        (Utilities|ScaleSpawnedDecal (Variables|Incision|GetInitialScale))))))

(event OnComponentEndOverlap(TipCollision)
  (params (OverlappedComponent :type Primitive%20Component%20Object%20Reference) (OtherActor :type Actor%20Object%20Reference) (OtherComp :type Primitive%20Component%20Object%20Reference) (OtherBodyIndex :type Integer))
  (Utilities|Casting|CastToBP_TestEyeball OtherActor)
  (Utilities|PrepareforIncision 0 0 0.0))

(event EventTick
  (params (DeltaSeconds :type Float%20%28single-precision%29))
  (Variables|Default|GetEyeball
    (:then
      (Variables|Default|GetSpawnedDecal
        (:then
          (Utilities|UpdateDepth
            (:Out
              (Utilities|ScaleSpawnedDecal (CallFunction|LerpScalebyDepth)))))
        (:else)))
    (:else)))

(fn ConstructionScript
  (Variables|Default|SetHaveSpawned false))

(fn ComputeLerpAlpha
  (params (AVal :type Float%20%28double-precision%29) (BVal :type Float%20%28double-precision%29) (PVal :type Float%20%28double-precision%29))
  (return (/ (- PVal AVal) (- BVal AVal))))

(fn LerpScalebyDepth
  (bind _maxdepth (Variables|Incision|GetMaxDepth))
  (return (Math|Float|Lerp (Variables|Incision|GetInitialScale) (Variables|Incision|GetMaxScale) (CallFunction|ComputeLerpAlpha 0.0 _maxdepth (Math|Float|Clamp(Float) (Variables|Default|GetDepth) 0.0 _maxdepth)))))

(fn TipWorldLocation
  (return (Transformation|GetWorldLocation (Variables|Default|GetTipCollision))))

(fn SpawnDecalonEyeball
  (params (Eyeball :type BP%20Test%20Eyeball%20Object%20Reference) (DecalMaterial :type Material%20Interface%20Object%20Reference) (DecalSize :type Vector) (Tag :type Name))
  (bind _newdecal (Default|SpawnDecalAttached Eyeball DecalMaterial DecalSize Tag))
  (return _newdecal))