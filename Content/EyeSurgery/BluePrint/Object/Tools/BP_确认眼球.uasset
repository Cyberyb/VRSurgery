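; Selectable eyeball-confirmation actor for the eye surgery procedure, reacting to the current task stage when pressed.
; In the pre-anesthesia stage (麻醉前), selection clears the highlight and swaps the confirmation mark's material to M_TagAfter.
; In the disinfection and draping stage (消毒铺巾), it reports task completion to the task manager.
; On success it starts the next task, plays voice audio and disables its own selection and highlight.
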(event PressedSelect(Comp_Select_Comp)
  (params (Pawn :type BP%20Pawn%20Base%20Object%20Reference) (SourceActor :type Actor%20Object%20Reference) (ImpactLocation :type Vector :default "0, 0, 0") (ImpactComponent :type Actor%20Component%20Object%20Reference))
  (bind _taskmanageref (Variables|Default|GetTaskManageRef))
  (bind _comp_highlight (Variables|Default|GetComp_Highlight))
  (bind _taskmanageref_2 (Variables|Default|GetTaskManageRef))
  (Utilities|IsValid _taskmanageref
    (:Is%20Valid
      (switch name (.Value (Utilities|Map|Find (Variables|/Game/EyeSurgery/DataAssets/Task/BP_TaskManage.BP_TaskManage_C|GetLevel2NameMap _taskmanageref) (Variables|/Game/EyeSurgery/DataAssets/Task/BP_TaskManage.BP_TaskManage_C|GetTaskArrayPDA _taskmanageref)))
        (:麻醉前
          (Variables|/Game/AFCore/Blueprints/Components/State/Comp_Highlight.Comp_Highlight_C|SetState _comp_highlight (Utilities|Struct|MakeStruct_Component_Binary "(InteractingPawn_9_73348001489683A296EE00B9C4DAAEE1=None,InteractingActor_11_52252C714CABB09D93F211B6CCAED861=None,SourceObject_12_CFB163304D2BD3A56E60338325318CA3=None,SourceIdentifier_14_C1E04B914773FC0E2DE8DEB2E24C888A=\"\")" false))
          (Rendering|Material|SetMaterial (Variables|Default|Get标识确认) 0 "/Game/VR-Space/Materials/M_TagAfter.M_TagAfter"))
        (:消毒铺巾
          (bind _isfinished (Default|TaskFinished _taskmanageref_2 2))
          (if _isfinished
            (Default|TaskInit _taskmanageref_2 3)
            (Default|PlayNextSound (Variables|Default|GetVoiceManageRef) "/Game/EyeSurgery/Sounds/消毒铺巾/Step4/1.1")
            (Variables|/Game/AFCore/Blueprints/Components/Interaction/Comp_Select.Comp_Select_C|SetSelectEnabled (Variables|Default|GetComp_Select_Comp) false)
            (Variables|/Game/AFCore/Blueprints/Components/State/Comp_Highlight.Comp_Highlight_C|SetState _comp_highlight (Utilities|Struct|MakeStruct_Component_Binary "(InteractingPawn_9_73348001489683A296EE00B9C4DAAEE1=None,InteractingActor_11_52252C714CABB09D93F211B6CCAED861=None,SourceObject_12_CFB163304D2BD3A56E60338325318CA3=None,SourceIdentifier_14_C1E04B914773FC0E2DE8DEB2E24C888A=\"\")" false))))))))

(event EventBeginPlay)

(event Collision|EventActorBeginOverlap
  (params (OtherActor :type Actor%20Object%20Reference)))

(event EventTick
  (params (DeltaSeconds :type Float%20%28single-precision%29)))

(fn ConstructionScript)