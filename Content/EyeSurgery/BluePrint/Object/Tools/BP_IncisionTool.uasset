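; BP_IncisionTool is an eye-surgery tool that leaves an incision decal on the test eyeball when its tip touches it.
; On tip overlap it adds and places a decal at the contact point, optionally only once, and records the start location.
; Each tick it tracks the furthest tip distance from that point as depth, scaling the decal between initial and maximum size.
; Ending the overlap clears the eyeball and resets depth.
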(event OnComponentBeginOverlap(TipCollision)
  (params (OverlappedComponent :type Primitive%20Component%20Object%20Reference) (OtherActor :type Actor%20Object%20Reference) (OtherComp :type Primitive%20Component%20Object%20Reference) (OtherBodyIndex :type Integer) (bFromSweep :type Boolean) (SweepResult :type Hit%20Result%20Structure%20%28by%20ref%29))
  (bind _asbp_test_eyeball (Utilities|Casting|CastToBP_TestEyeball OtherActor))
  (if (not (and (Variables|Incision|GetSpawnOnlyOnce) (Variables|Default|GetHaveSpawned)))
    (bind _output_get (Variables|Default|SetEyeball _asbp_test_eyeball))
    (bind _newdecal (Default|AddDecal _output_get))
    (bind _output_get_2 (Variables|Default|SetSpawnedDecal _newdecal))
    (Default|PlaceDecal _output_get _output_get_2 (Transformation|GetWorldLocation (Variables|Default|GetTipCollision)))
    (Utilities|UpdateStartLocation
      (:Out
        (Default|ScaleDecal (Variables|Default|GetEyeball) (Variables|Default|GetSpawnedDecal) (Variables|Incision|GetInitialScale))
        (Variables|Default|SetHaveSpawned true)))))

(event OnComponentEndOverlap(TipCollision)
  (params (OverlappedComponent :type Primitive%20Component%20Object%20Reference) (OtherActor :type Actor%20Object%20Reference) (OtherComp :type Primitive%20Component%20Object%20Reference) (OtherBodyIndex :type Integer))
  (Utilities|Casting|CastToBP_TestEyeball OtherActor)
  (Variables|Default|SetEyeball 0)
  (Variables|Default|SetDepth 0.0))

(event EventTick
  (params (DeltaSeconds :type Float%20%28single-precision%29))
  (Variables|Default|GetEyeball
    (:then
      (Utilities|UpdateDepth
        (:Out
          (Default|ScaleDecal (Variables|Default|GetEyeball) (Variables|Default|GetSpawnedDecal) (CallFunction|LerpScalebyDepth)))))
    (:else)))

(fn ConstructionScript)

(fn ComputeLerpAlpha
  (params (AVal :type Float%20%28double-precision%29) (BVal :type Float%20%28double-precision%29) (PVal :type Float%20%28double-precision%29))
  (return (/ (- PVal AVal) (- BVal AVal))))

(fn LerpScalebyDepth
  (bind _maxdepth (Variables|Incision|GetMaxDepth))
  (return (Math|Float|Lerp (Variables|Incision|GetInitialScale) (Variables|Incision|GetMaxScale) (CallFunction|ComputeLerpAlpha 0.0 _maxdepth (Math|Float|Clamp(Float) (Variables|Default|GetDepth) 0.0 _maxdepth)))))

(fn TipWorldLocation
  (return (Transformation|GetWorldLocation (Variables|Default|GetTipCollision))))