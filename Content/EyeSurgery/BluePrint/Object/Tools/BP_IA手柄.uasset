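; BP_IA手柄 is the irrigation/aspiration (IA) handpiece tool in the eye surgery game, used to suck away soft lens material.
; Comp_Grab's Trigger key sets Triggered, and a Sphere overlap while triggered stores the touched actor, unfiltered, and enables suction.
; While both flags hold, Tick shrinks that actor by a fixed per-frame step through a shared, unclamped ScaleFloat.
; Suction is never disabled here, and the pull-toward-tip offset is disconnected.
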(event GrabKeyInput(Comp_Grab)
  (params (MComp :type BP%20M%20Comp%20Object%20Reference) (Key :type Enum_Controller_Buttons%20Enum :default "NewEnumerator1") (Set :type Boolean))
  (switch Utilities|FlowControl|Switch|SwitchonEnum_Controller_Buttons Key
    (:NewEnumerator0
      (Variables|Default|SetTriggered Set))))

(event OnComponentBeginOverlap(Sphere)
  (params (OverlappedComponent :type Primitive%20Component%20Object%20Reference) (OtherActor :type Actor%20Object%20Reference) (OtherComp :type Primitive%20Component%20Object%20Reference) (OtherBodyIndex :type Integer) (bFromSweep :type Boolean) (SweepResult :type Hit%20Result%20Structure%20%28by%20ref%29))
  (if (Variables|Default|GetTriggered)
    (Variables|Default|SetSoftLensToSuck OtherActor)
    (Variables|Default|SetEnableToSuck true)))

(event Custom|SuckSoftLens
  (params (DeltaScale :type Float%20%28double-precision%29))
  (bind _output_get (Variables|Default|SetScaleFloat (- (Variables|Default|GetScaleFloat) DeltaScale)))
  (Transformation|SetActorScale3D (Variables|Default|GetSoftLensToSuck) (Math|Conversions|ToVector(Float) _output_get)))

(event EventBeginPlay)

(event Collision|EventActorBeginOverlap
  (params (OtherActor :type Actor%20Object%20Reference)))

(event EventTick
  (params (DeltaSeconds :type Float%20%28single-precision%29))
  (if (and (Variables|Default|GetTriggered) (Variables|Default|GetEnableToSuck))
    (CallFunction|SuckSoftLens 0.01)))

(fn ConstructionScript)