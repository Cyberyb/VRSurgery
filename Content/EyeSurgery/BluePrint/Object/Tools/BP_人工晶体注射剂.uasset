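; VR grab tool for the eye-surgery game: an artificial lens injector that delivers the lens.
; On BeginPlay it caches the level's BP_LensPosHelper, and the first Trigger input while grabbed starts that helper's sequence, guarded by DoOnce.
; Tick then follows the helper's stage, first pinning the lens to the injector's Sphere component, then handing it once to the helper's root transform and ending the update.
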(event GrabKeyInput(Comp_Grab)
  (params (MComp :type BP%20M%20Comp%20Object%20Reference) (Key :type Enum_Controller_Buttons%20Enum :default "NewEnumerator1") (Set :type Boolean))
  (switch Utilities|FlowControl|Switch|SwitchonEnum_Controller_Buttons Key
    (:NewEnumerator0
      (Utilities|FlowControl|Sequence
        (:then_0
          (Variables|Animate|SetIsTriggered Set))
        (:then_1
          (Utilities|FlowControl|DoOnce false
            (:Completed
              (Variables|Default|SetInjected true)
              (Default|PlaySequence (Variables|Default|GetLensPosHelper)))))))))

(event EventBeginPlay
  (bind _returnvalue (Actor|GetActorOfClass "/Game/EyeSurgery/BluePrint/Object/Helpers/BP_LensPosHelper.BP_LensPosHelper_C"))
  (Utilities|IsValid _returnvalue
    (:Is%20Valid
      (Variables|Default|SetLensPosHelper _returnvalue))))

(event Collision|EventActorBeginOverlap
  (params (OtherActor :type Actor%20Object%20Reference)))

(event EventTick
  (params (DeltaSeconds :type Float%20%28single-precision%29))
  (bind _lensposhelper (Variables|Default|GetLensPosHelper))
  (if (Variables|Default|GetInjected)
    (switch int (Variables|/Game/EyeSurgery/BluePrint/Object/Helpers/BP_LensPosHelper.BP_LensPosHelper_C|GetStage (Variables|Default|GetLensPosHelper))
      (:1
        (Default|SetLensTransform (Variables|Default|GetLensPosHelper) (Transformation|GetWorldTransform (Variables|Default|GetSphere))))
      (:2
        (Utilities|FlowControl|DoOnce false
          (:Completed
            (Default|SetLensTransform _lensposhelper (Transformation|GetWorldTransform (Variables|/Game/EyeSurgery/BluePrint/Object/Helpers/BP_LensPosHelper.BP_LensPosHelper_C|GetDefaultSceneRoot _lensposhelper)))
            (Variables|Default|SetInjected false)))))))

(fn ConstructionScript)