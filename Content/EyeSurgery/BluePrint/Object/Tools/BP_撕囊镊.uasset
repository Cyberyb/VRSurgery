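; Grabbable capsulorhexis forceps for an eye surgery sim, tearing the lens capsule while the trigger is held inside BP_CollisionHepler.
; Tick scrubs the helper's tear sequence in two steps: downward distance from the center, then angle around it.
; Progress only moves forward, and step two rejects large jumps to enforce a continuous circular tear.
; Voice cues play along the way; starting height and elapsed time form the score, recorded before the task-finish check.
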(event GrabKeyInput(Comp_Grab)
  (params (MComp :type BP%20M%20Comp%20Object%20Reference) (Key :type Enum_Controller_Buttons%20Enum :default "NewEnumerator1") (Set :type Boolean))
  (switch Utilities|FlowControl|Switch|SwitchonEnum_Controller_Buttons Key
    (:NewEnumerator0
      (Utilities|FlowControl|Sequence
        (:then_0
          (Variables|Animate|SetIsTriggered Set))
        (:then_1
          (if (Variables|Default|GetCanTrigger)
            (Variables|Default|SetCanTear Set)
            (Utilities|FlowControl|DoOnce false
              (:Completed
                (bind _collisionhelper (Variables|Default|GetCollisionHelper)
                  (:then
                    (Utilities|IsValid (Variables|/Game/EyeSurgery/BluePrint/Object/Helpers/BP_CollisionHepler.BP_CollisionHepler_C|GetGC_Tear _collisionhelper)
                      (:Is%20Valid
                        (Rendering|SetVisibility (Variables|/Script/GeometryCache.GeometryCacheActor|GetGeometryCacheComponent (Variables|/Game/EyeSurgery/BluePrint/Object/Helpers/BP_CollisionHepler.BP_CollisionHepler_C|GetGC_Tear _collisionhelper)) true false)
                        (bind _step (CallFunction|GetTearStep))
                        (Variables|Default|SetStep _step))))
                  (:else))))))))))

(event OnComponentBeginOverlap(Sphere)
  (params (OverlappedComponent :type Primitive%20Component%20Object%20Reference) (OtherActor :type Actor%20Object%20Reference) (OtherComp :type Primitive%20Component%20Object%20Reference) (OtherBodyIndex :type Integer) (bFromSweep :type Boolean) (SweepResult :type Hit%20Result%20Structure%20%28by%20ref%29))
  (if (== (Utilities|GetClass OtherActor) "/Game/EyeSurgery/BluePrint/Object/Helpers/BP_CollisionHepler.BP_CollisionHepler_C")
    (Variables|Default|SetCanTrigger true)
    (bind _returnvalue (Actor|GetActorOfClass "/Game/EyeSurgery/BluePrint/Object/Helpers/BP_CollisionHepler.BP_CollisionHepler_C"))
    (Utilities|IsValid _returnvalue
      (:Is%20Valid
        (Variables|Default|SetCollisionHelper _returnvalue)))))

(event OnComponentEndOverlap(Sphere)
  (params (OverlappedComponent :type Primitive%20Component%20Object%20Reference) (OtherActor :type Actor%20Object%20Reference) (OtherComp :type Primitive%20Component%20Object%20Reference) (OtherBodyIndex :type Integer))
  (if (== (Utilities|GetClass OtherActor) "/Game/EyeSurgery/BluePrint/Object/Helpers/BP_CollisionHepler.BP_CollisionHepler_C")
    (Variables|Default|SetCanTrigger false)))

(event EventBeginPlay
  (|CallParentFunction)
  (bind _returnvalue (Actor|GetActorOfClass "/Game/EyeSurgery/BluePrint/Object/BP_SurgeryVoice.BP_SurgeryVoice_C"))
  (Utilities|IsValid _returnvalue
    (:Is%20Valid
      (Variables|Default|SetSurgeryVoice _returnvalue))))

(event Collision|EventActorBeginOverlap
  (params (OtherActor :type Actor%20Object%20Reference))
  (|CallParentFunction OtherActor) ; 此节点被禁用，将不会被调用。\n从引脚连出引线来编译功能。
)

(event EventTick
  (params (DeltaSeconds :type Float%20%28single-precision%29))
  (bind _sphere (Variables|Default|GetSphere))
  (bind _collisionhelper (Variables|Default|GetCollisionHelper))
  (bind _collisionhelper_2 (Variables|Default|GetCollisionHelper))
  (bind _returnvalue (Transformation|GetWorldLocation _sphere))
  (bind _tearsequence (Variables|/Game/EyeSurgery/BluePrint/Object/Helpers/BP_CollisionHepler.BP_CollisionHepler_C|GetTearSequence _collisionhelper))
  (bind _mainsphere (Variables|/Game/EyeSurgery/BluePrint/Object/Helpers/BP_CollisionHepler.BP_CollisionHepler_C|GetMainSphere _collisionhelper_2))
  (bind _returnvalue_2 (Transformation|GetWorldLocation _mainsphere))
  (bind _sequenceplayer (Variables|/Script/LevelSequence.LevelSequenceActor|GetSequencePlayer _tearsequence))
  (bind _returnvalue_3 (- _returnvalue _returnvalue_2))
  (|CallParentFunction DeltaSeconds)
  (if (and (Variables|Default|GetCanTrigger) (Variables|Default|GetCanTear))
    (switch int (Variables|Default|GetStep)
      (:1
        (Utilities|FlowControl|Sequence
          (:then_0
            (Utilities|FlowControl|DoOnce false
              (:Completed
                (Default|PlayVoice (Variables|Default|GetSurgeryVoice) 3)
                (CallFunction|CalculateSubScore))))
          (:then_1
            ;[1 1 1] Step1
            (bind _distance (CallFunction|CalculateDistance))
            (Components|Timeline|SetPlaybackPosition (Variables|/Script/LevelSequence.LevelSequenceActor|GetSequencePlayer (Variables|/Game/EyeSurgery/BluePrint/Object/Helpers/BP_CollisionHepler.BP_CollisionHepler_C|GetTearSequence (Variables|Default|GetCollisionHelper))) (Utilities|Struct|MakeMovieSceneSequencePlaybackParams (Utilities|Struct|MakeFrameTime (Utilities|Struct|MakeFrameNumber (Math|Integer|Max(Integer) (Math|Float|Floor (* (Math|Float|Min(Float) (/ _distance (Components|Sphere|GetScaledSphereRadius (Variables|/Game/EyeSurgery/BluePrint/Object/Helpers/BP_CollisionHepler.BP_CollisionHepler_C|GetMainSphere (Variables|Default|GetCollisionHelper)))) 1.0) 1e+02)) (Variables|Default|GetStep1Max))) 0.0) 0.0 "" "Frame" "Play" false))
            (Variables|Default|SetStep1Max (Math|Integer|Max(Integer) (Math|Float|Floor (* (Math|Float|Min(Float) (/ _distance (Components|Sphere|GetScaledSphereRadius (Variables|/Game/EyeSurgery/BluePrint/Object/Helpers/BP_CollisionHepler.BP_CollisionHepler_C|GetMainSphere (Variables|Default|GetCollisionHelper)))) 1.0) 1e+02)) (Variables|Default|GetStep1Max)))
            (if (>= (Math|Float|Floor (* (Math|Float|Min(Float) (/ _distance (Components|Sphere|GetScaledSphereRadius (Variables|/Game/EyeSurgery/BluePrint/Object/Helpers/BP_CollisionHepler.BP_CollisionHepler_C|GetMainSphere (Variables|Default|GetCollisionHelper)))) 1.0) 1e+02)) 65)
              (Variables|Default|SetStep 2)
              (Default|PlayVoice (Variables|Default|GetSurgeryVoice) 4)))))
      (:2
        ;[1 1 1] Step2
        (bind _angel (CallFunction|CalculateAngel (Math|Vector2D|MakeVector2D (.y _returnvalue_3) (.z _returnvalue_3)) "(X=0.000000,Y=-1.000000)" false))
        (Utilities|IsValid _tearsequence
          (:Is%20Valid
            (Components|Timeline|SetPlaybackPosition _sequenceplayer (Utilities|Struct|MakeMovieSceneSequencePlaybackParams (Utilities|Struct|MakeFrameTime (Utilities|Struct|MakeFrameNumber (Math|Integer|Max(Integer) (Math|Integer|SelectInt (+ (Math|Float|Truncate (* (/ _angel 3.6e+02) (- (Class|MovieSceneSequencePlayer|GetFrameDuration _sequenceplayer) 70))) 70) (Variables|Default|GetStep2Loc) (< (+ (Math|Float|Truncate (* (/ _angel 3.6e+02) (- (Class|MovieSceneSequencePlayer|GetFrameDuration _sequenceplayer) 70))) 70) (+ (Variables|Default|GetStep2Loc) 10))) (Variables|Default|GetStep2Max))) 0.0) 0.0 "" "Frame" "Play" false))
            (Variables|Default|SetStep2Loc (Math|Integer|Max(Integer) (Math|Integer|SelectInt (+ (Math|Float|Truncate (* (/ _angel 3.6e+02) (- (Class|MovieSceneSequencePlayer|GetFrameDuration _sequenceplayer) 70))) 70) (Variables|Default|GetStep2Loc) (< (+ (Math|Float|Truncate (* (/ _angel 3.6e+02) (- (Class|MovieSceneSequencePlayer|GetFrameDuration _sequenceplayer) 70))) 70) (+ (Variables|Default|GetStep2Loc) 10))) (Variables|Default|GetStep2Max)))
            (Variables|Default|SetStep2Max (Math|Integer|Max(Integer) (Math|Integer|SelectInt (+ (Math|Float|Truncate (* (/ _angel 3.6e+02) (- (Class|MovieSceneSequencePlayer|GetFrameDuration _sequenceplayer) 70))) 70) (Variables|Default|GetStep2Loc) (< (+ (Math|Float|Truncate (* (/ _angel 3.6e+02) (- (Class|MovieSceneSequencePlayer|GetFrameDuration _sequenceplayer) 70))) 70) (+ (Variables|Default|GetStep2Loc) 10))) (Variables|Default|GetStep2Max)))
            (if (>= (Math|Integer|Max(Integer) (Math|Integer|SelectInt (+ (Math|Float|Truncate (* (/ _angel 3.6e+02) (- (Class|MovieSceneSequencePlayer|GetFrameDuration _sequenceplayer) 70))) 70) (Variables|Default|GetStep2Loc) (< (+ (Math|Float|Truncate (* (/ _angel 3.6e+02) (- (Class|MovieSceneSequencePlayer|GetFrameDuration _sequenceplayer) 70))) 70) (+ (Variables|Default|GetStep2Loc) 10))) (Variables|Default|GetStep2Max)) 300)
              (Rendering|SetVisibility (Variables|/Script/GeometryCache.GeometryCacheActor|GetGeometryCacheComponent (Variables|/Game/EyeSurgery/BluePrint/Object/Helpers/BP_CollisionHepler.BP_CollisionHepler_C|GetGC_Tear (Variables|Default|GetCollisionHelper))) false false)
              (Utilities|FlowControl|DoOnce false
                (:Completed
                  (CallFunction|CalculateScore)
                  (bind _returnvalue_4 (Actor|GetActorOfClass "/Game/EyeSurgery/BluePrint/Object/Helpers/BP_TaskFinisHP.BP_TaskFinisHP_C"))
                  (Utilities|IsValid _returnvalue_4
                    (:Is%20Valid
                      (Default|CheckFinished _returnvalue_4 2))))))))))))

(fn ConstructionScript
  (|CallParentFunction))

(fn CalculateAngel
  (params (StartPos :type Vector%202D%20Structure) (EndPos :type Vector%202D%20Structure) (ClockWise :type Boolean))
  (bind _returnvalue (Math|Vector2D|DotProduct(2D) StartPos EndPos))
  (bind _returnvalue_2 (Class|KismetMathLibrary|CrossProduct2D StartPos EndPos))
  (bind _returnvalue_3 (Class|KismetMathLibrary|DegAtan2 _returnvalue_2 _returnvalue))
  (bind _returnvalue_4 (< _returnvalue_2 0.0))
  (bind _returnvalue_5 (Math|Float|Absolute(Float) _returnvalue_3))
  (bind _returnvalue_6 (- 3.6e+02 _returnvalue_5))
  (bind _returnvalue_7 (select _returnvalue_4 _returnvalue_6 _returnvalue_3))
  (return (select ClockWise _returnvalue_7 (- 3.6e+02 _returnvalue_7))))

(fn CalculateDistance
  (bind _collisionhelper (Variables|Default|GetCollisionHelper))
  (bind _sphere (Variables|Default|GetSphere))
  (bind _returnvalue (Transformation|GetWorldLocation _sphere))
  (bind _mainsphere (Variables|/Game/EyeSurgery/BluePrint/Object/Helpers/BP_CollisionHepler.BP_CollisionHepler_C|GetMainSphere _collisionhelper))
  (bind _returnvalue_2 (Transformation|GetWorldLocation _mainsphere))
  (bind _returnvalue_3 (- (.z _returnvalue_2) (.z _returnvalue)))
  (bind _returnvalue_4 (Math|Float|Max(Float) _returnvalue_3 0.0))
  (Development|PrintString (Utilities|String|ToString(Float) _returnvalue_4))
  (return _returnvalue_4))

(fn GetTearStep
  (bind _collisionhelper (Variables|Default|GetCollisionHelper)
    (:then
      (if (< (.value (.frame (Sequencer|Player|GetCurrentTime (Variables|/Script/LevelSequence.LevelSequenceActor|GetSequencePlayer (Variables|/Game/EyeSurgery/BluePrint/Object/Helpers/BP_CollisionHepler.BP_CollisionHepler_C|GetTearSequence _collisionhelper))))) 70)
        (return 1)
        (else
          (return 2))))
    (:else)))

(fn CalculateScore
  (bind _returnvalue (Actor|GetActorOfClass "/Game/EyeSurgery/BluePrint/Object/Helpers/BP_ScoreManage.BP_ScoreManage_C"))
  (Utilities|IsValid _returnvalue
    (:Is%20Valid
      (Default|RecordScore _returnvalue "NewEnumerator2" (Math|Integer|Clamp(Integer) (+ (Math|Float|Truncate (Math|Float|Max(Float) (- 5e+01 (Math|Float|Max(Float) (- (- (Utilities|Time|GetTimeSeconds) (Variables|分数|GetStartTime)) (Variables|分数|GetTimeThresh)) 0.0)) 0.0)) (Variables|Score|GetSubScore)) 0 100))
      (return))))

(fn CalculateSubScore
  (Variables|Score|SetSubScore (Math|Float|Truncate (Math|Float|Max(Float) (- 5e+01 (Math|Float|Absolute(Float) (- (.z (Transformation|GetWorldLocation (Variables|/Game/EyeSurgery/BluePrint/Object/Helpers/BP_CollisionHepler.BP_CollisionHepler_C|GetMainSphere (Variables|Default|GetCollisionHelper)))) (.z (Transformation|GetWorldLocation (Variables|Default|GetSphere)))))) 0.0)))
  (Variables|分数|SetStartTime (Utilities|Time|GetTimeSeconds))
  (return))