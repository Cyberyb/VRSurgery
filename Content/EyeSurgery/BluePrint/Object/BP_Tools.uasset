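; BP_Tools is a grabbable surgical tool actor for the VR eye surgery game, tying its grab state to the tools board menu.
; On pickup it records the laser component's grabbed tool, then after a short delay disables that hand's W_ToolsMenu button.
; On release it destroys the tool after a delay and re-enables the button.
; Key-driven tool switching, menu paging and overlap-based controller blocking remain as disconnected, unused logic.
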(event GrabKeyInput(Comp_Grab)
  (params (MComp :type BP%20M%20Comp%20Object%20Reference) (Key :type Enum_Controller_Buttons%20Enum :default "NewEnumerator1") (Set :type Boolean)))

(event GrabActorPickedUp(Comp_Grab)
  (params (GrabbingPawn :type BP%20Pawn%20Base%20Object%20Reference) (GrabbingActor :type Actor%20Object%20Reference))
  ;[1 1 1] 抓取时记录Tool并禁用工具获取按钮
  (bind _asbp_mcomp_laser (Utilities|Casting|CastToBP_MComp_Laser GrabbingActor))
  (Utilities|IsValid (Variables|/Game/AFCore/Blueprints/VR/MotionComponents/BP_MComp_Laser.BP_MComp_Laser_C|GetGrabbedActor _asbp_mcomp_laser)
    (:Is%20Valid
      (Variables|Default|SetGrabbedTool (Variables|/Game/AFCore/Blueprints/VR/MotionComponents/BP_MComp_Laser.BP_MComp_Laser_C|GetGrabbedActor _asbp_mcomp_laser))
      (Utilities|FlowControl|Delay 0.2)
      (bind _returnvalue (Actor|GetActorOfClass "/Game/EyeSurgery/BluePrint/UI/BP_ToolsBoard.BP_ToolsBoard_C"))
      (bind _asw_tools_menu (Utilities|Casting|CastToW_ToolsMenu (UserInterface|GetWidget (Variables|/Game/AFCore/Blueprints/UI/Static/BP_Board.BP_Board_C|GetComp_Widget _returnvalue))))
      (Default|DeactivateButton _asw_tools_menu (Variables|/Game/AFCore/Blueprints/VR/MotionComponents/BP_MComp.BP_MComp_C|GetSide _asbp_mcomp_laser)))))

(event OnComponentBeginOverlap(StaticMeshComponent)
  (params (OverlappedComponent :type Primitive%20Component%20Object%20Reference) (OtherActor :type Actor%20Object%20Reference) (OtherComp :type Primitive%20Component%20Object%20Reference) (OtherBodyIndex :type Integer) (bFromSweep :type Boolean) (SweepResult :type Hit%20Result%20Structure%20%28by%20ref%29)))

(event OnComponentEndOverlap(StaticMeshComponent)
  (params (OverlappedComponent :type Primitive%20Component%20Object%20Reference) (OtherActor :type Actor%20Object%20Reference) (OtherComp :type Primitive%20Component%20Object%20Reference) (OtherBodyIndex :type Integer)))

(event GrabActorReleased(Comp_Grab)
  (params (ReleasingPawn :type BP%20Pawn%20Base%20Object%20Reference) (ReleasingActor :type Actor%20Object%20Reference) (LastRelease :type Boolean))
  (bind _grabbedtool (Variables|Default|GetGrabbedTool))
  ;[1 1 1] 释放时销毁Tool并激活工具获取按钮
  (bind _asbp_mcomp_laser (Utilities|Casting|CastToBP_MComp_Laser ReleasingActor))
  (Utilities|IsValid _grabbedtool
    (:Is%20Valid
      (Utilities|FlowControl|Delay 0.1)
      (Actor|DestroyActor _grabbedtool)
      (bind _returnvalue (Actor|GetActorOfClass "/Game/EyeSurgery/BluePrint/UI/BP_ToolsBoard.BP_ToolsBoard_C"))
      (bind _asw_tools_menu (Utilities|Casting|CastToW_ToolsMenu (UserInterface|GetWidget (Variables|/Game/AFCore/Blueprints/UI/Static/BP_Board.BP_Board_C|GetComp_Widget _returnvalue))))
      (Default|ActivateButton _asw_tools_menu (Variables|/Game/AFCore/Blueprints/VR/MotionComponents/BP_MComp.BP_MComp_C|GetSide _asbp_mcomp_laser)))))

(event Custom|CorrectControllerLocation)

(event EventBeginPlay
  (bind _asbp_surgery_char (Utilities|Casting|CastToBP_Surgery_Char (Game|Player|GetPlayerPawn 0)))
  (Variables|Default|SetMotion%20Controller%20Right (Variables|/Game/AFCore/Blueprints/Pawn/VR/BP_Pawn_VR.BP_Pawn_VR_C|GetMotionControllerRight _asbp_surgery_char))
  (Variables|Default|SetMotion%20Controller%20Left (Variables|/Game/AFCore/Blueprints/Pawn/VR/BP_Pawn_VR.BP_Pawn_VR_C|GetMotionControllerLeft _asbp_surgery_char)))

(event Collision|EventActorBeginOverlap
  (params (OtherActor :type Actor%20Object%20Reference)))

(event EventTick
  (params (DeltaSeconds :type Float%20%28single-precision%29)))

(fn ConstructionScript)

(fn GetFrontTran
  (bind _returnvalue (Actor|GetActorOfClass "/Game/EyeSurgery/BluePrint/Pawn/BP_Surgery_Char.BP_Surgery_Char_C"))
  (return "0, 0, 0" (+ (.location (Transformation|GetWorldTransform (Variables|/Game/AFCore/Blueprints/Pawn/BP_Pawn_Base.BP_Pawn_Base_C|GetMainCamera _returnvalue))) (* (Math|Vector|GetForwardVector (Variables|/Game/AFCore/Blueprints/Pawn/BP_Pawn_Base.BP_Pawn_Base_C|GetMainCamera _returnvalue)) 15.0)) (Math|Rotator|CombineRotators (.rotation (Transformation|GetWorldTransform (Variables|/Game/AFCore/Blueprints/Pawn/BP_Pawn_Base.BP_Pawn_Base_C|GetMainCamera _returnvalue))) "0,180.000000, 0")))