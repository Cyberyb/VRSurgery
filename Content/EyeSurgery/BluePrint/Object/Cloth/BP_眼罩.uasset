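; BP_眼罩 is the eye shield Blueprint in the eye surgery project, an attachable object that advances the procedure once placed.
; When its anchor connector attaches and the voice manager reference is valid, it plays the next voice clip.
; It then finds the tagged tape (胶带) actors and enables grabbing on their grab components, unlocking the taping step.
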(event ConnectorAttached(Comp_Connector_Anchor)
  (params (Connector :type Comp%20Connector%20Object%20Reference) (AttachedToActor :type Actor%20Object%20Reference) (AttachedToComponent :type Scene%20Component%20Object%20Reference))
  (bind _voicemanageref (Variables|Default|GetVoiceManageRef)
    (:then
      (Default|PlayNextSound _voicemanageref "/Game/EyeSurgery/Sounds/手术后安全核查/Step3/3.3")
      (bind _outactors (Actor|GetAllActorsOfClasswithTag "/Game/EyeSurgery/BluePrint/Object/Cloth/BP_胶带.BP_胶带_C" "胶带"))
      (for _array_element _outactors
        (Default|SetGrabEnabled (Variables|/Game/VR-Space/Draping/BP_DrapeToSnap.BP_DrapeToSnap_C|GetComp_Grab _array_element) true)))
    (:else)))

(event EventBeginPlay
  (|CallParentFunction) ; 此节点被禁用，将不会被调用。\n从引脚连出引线来编译功能。
)

(event Collision|EventActorBeginOverlap
  (params (OtherActor :type Actor%20Object%20Reference))
  (|CallParentFunction OtherActor) ; 此节点被禁用，将不会被调用。\n从引脚连出引线来编译功能。
)

(event EventTick
  (params (DeltaSeconds :type Float%20%28single-precision%29))
  (|CallParentFunction DeltaSeconds) ; 此节点被禁用，将不会被调用。\n从引脚连出引线来编译功能。
)

(fn ConstructionScript
  (|CallParentFunction))