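; Adhesive tape (胶带) actor for the eye surgery game that reports when the taping step is complete.
; When its connector anchor attaches, it flags itself as attached and sums that flag across all tape actors in the level.
; A total of two plays the next sound through the voice manager, finishes the tape task in the task manager and, on success, initializes the following task.
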(event ConnectorAttached(Comp_Connector_Anchor)
  (params (Connector :type Comp%20Connector%20Object%20Reference) (AttachedToActor :type Actor%20Object%20Reference) (AttachedToComponent :type Scene%20Component%20Object%20Reference))
  (Variables|Default|SetAttached 1)
  (bind _outactors (Actor|GetAllActorsOfClass "BP_胶带_C"))
  (bind _array_element (Utilities|Array|ForEachLoopwithBreak _outactors)
    (:LoopBody
      (Variables|Default|SetSum (+ (Variables|BP_胶带_C|GetAttached _array_element) (Variables|Default|GetSum))))
    (:Completed
      (if (== (Variables|Default|GetSum) 2)
        (bind _voicemanageref (Variables|Default|GetVoiceManageRef)
          (:then
            (Default|PlayNextSound _voicemanageref "/Game/EyeSurgery/Sounds/手术后安全核查/Step4/1.1")
            (bind _taskmanageref (Variables|Default|GetTaskManageRef)
              (:then
                (bind _isfinished (Default|TaskFinished _taskmanageref 2))
                (if _isfinished
                  (Default|TaskInit _taskmanageref 3)))
              (:else)))
          (:else))))))

(event EventBeginPlay
  (|CallParentFunction) ; 此节点被禁用，将不会被调用。\n从引脚连出引线来编译功能。
)

(event Collision|EventActorBeginOverlap
  (params (OtherActor :type Actor%20Object%20Reference))
  (|CallParentFunction OtherActor) ; 此节点被禁用，将不会被调用。\n从引脚连出引线来编译功能。
)

(event EventTick
  (params (DeltaSeconds :type Float%20%28single-precision%29))
  (|CallParentFunction DeltaSeconds) ; 此节点被禁用，将不会被调用。\n从引脚连出引线来编译功能。
)

(fn ConstructionScript
  (|CallParentFunction))