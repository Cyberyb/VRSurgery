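; Gauze actor for the eye surgery game that reports grab and attach events to voice and task managers.
; Picking it up through its grab component plays a voice line.
; Attaching its anchor connector plays another voice line, then asks the task manager to finish the current task and initializes the next one if that succeeds.
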(event GrabActorPickedUp(Comp_Grab)
  (params (GrabbingPawn :type BP%20Pawn%20Base%20Object%20Reference) (GrabbingActor :type Actor%20Object%20Reference))
  (bind _voicemanageref (Variables|Default|GetVoiceManageRef)
    (:then
      (Default|PlayNextSound _voicemanageref "/Game/EyeSurgery/Sounds/手术后安全核查/Step2/2.2"))
    (:else)))

(event ConnectorAttached(Comp_Connector_Anchor)
  (params (Connector :type Comp%20Connector%20Object%20Reference) (AttachedToActor :type Actor%20Object%20Reference) (AttachedToComponent :type Scene%20Component%20Object%20Reference))
  (bind _voicemanageref (Variables|Default|GetVoiceManageRef)
    (:then
      (Default|PlayNextSound _voicemanageref "/Game/EyeSurgery/Sounds/手术后安全核查/Step3/1.1")
      (bind _taskmanageref (Variables|Default|GetTaskManageRef)
        (:then
          (bind _isfinished (Default|TaskFinished _taskmanageref 1))
          (if _isfinished
            (Default|TaskInit _taskmanageref 2)))
        (:else)))
    (:else)))

(event EventBeginPlay
  (|CallParentFunction) ; 此节点被禁用，将不会被调用。\n从引脚连出引线来编译功能。
)

(event Collision|EventActorBeginOverlap
  (params (OtherActor :type Actor%20Object%20Reference))
  (|CallParentFunction OtherActor) ; 此节点被禁用，将不会被调用。\n从引脚连出引线来编译功能。
)

(event EventTick
  (params (DeltaSeconds :type Float%20%28single-precision%29))
  (|CallParentFunction DeltaSeconds) ; 此节点被禁用，将不会被调用。\n从引脚连出引线来编译功能。
)

(fn ConstructionScript
  (|CallParentFunction))