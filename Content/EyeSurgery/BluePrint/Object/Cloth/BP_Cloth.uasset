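; BP_Cloth is a selectable cloth object in an eye surgery simulation that destroys itself when pressed.
; After a short error-avoiding delay, it counts actors tagged 铺巾 (surgical drape) to detect whether only one remains.
; For the last one, it first has BP_VoiceManage play a sound and enables grabbing on BP_眼罩 (eye shield), unlocking that object.
; That final destroy only happens if the voice manager is valid.
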(event PressedSelect(Comp_Select_Comp)
  (params (Pawn :type BP%20Pawn%20Base%20Object%20Reference) (SourceActor :type Actor%20Object%20Reference) (ImpactLocation :type Vector :default "0, 0, 0") (ImpactComponent :type Actor%20Component%20Object%20Reference))
  ;[1 1 1] 不Delay会出错
  (Utilities|FlowControl|Delay 0.1)
  (bind _outactors (Actor|GetAllActorswithTag "铺巾"))
  (if (== (Utilities|Array|Length _outactors) 1)
    (bind _returnvalue (Actor|GetActorOfClass "/Game/EyeSurgery/BluePrint/Voice/BP_VoiceManage.BP_VoiceManage_C"))
    (Utilities|IsValid _returnvalue
      (:Is%20Valid
        (Default|PlayNextSound _returnvalue "/Game/EyeSurgery/Sounds/手术后安全核查/Step3/2.2")
        (bind _returnvalue_2 (Actor|GetActorOfClass "/Game/EyeSurgery/BluePrint/Object/Cloth/BP_眼罩.BP_眼罩_C"))
        (Default|SetGrabEnabled (Variables|/Game/VR-Space/Draping/BP_DrapeToSnap.BP_DrapeToSnap_C|GetComp_Grab _returnvalue_2) true)
        (Actor|DestroyActor)))
    (else
      (Actor|DestroyActor))))

(event EventBeginPlay)

(event Collision|EventActorBeginOverlap
  (params (OtherActor :type Actor%20Object%20Reference)))

(event EventTick
  (params (DeltaSeconds :type Float%20%28single-precision%29)))

(fn ConstructionScript)