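; Manager for the surgical drape-snapping steps in a VR eye surgery simulation.
; Each drape-attached event marks that tag's slot in DrapeDetect, counts filled slots and spawns the next tagged drape until the sequence ends.
; Certain counts finish or start tasks through the task manager and play timed voice lines.
; Spawning writes the new tag to the connector IDs of every BP_DrapeToSnap in the level, not just the newest.
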(event Custom|ChangeDrapeArray
  (params (Tag :type Name))
  (bind _tagstodrape (Variables|Default|GetTagsToDrape))
  (bind (_value _returnvalue) (Utilities|Map|Find _tagstodrape Tag))
  (if _returnvalue
    (Utilities|Array|SetArrayElem (Variables|Default|GetDrapeDetect) _value true)
    (CallFunction|CheckDrapeArray)
    (if (< _value (- (Utilities|Array|Length (Variables|Default|GetTagsArray)) 1))
      (CallFunction|SpawnDrape (Utilities|Array|Get(acopy) (Variables|Default|GetTagsArray) (+ _value 1)))
      (Variables|Default|SetDrapeSum 0))))

(event Custom|CheckDrapeArray
  (bind _taskmanageref (Variables|Default|GetTaskManageRef))
  (bind _voicemanageref (Variables|Default|GetVoiceManageRef))
  ;[1 1 1] 根据Snap的情况完成任务或播放语音
  (for _array_element (Variables|Default|GetDrapeDetect)
    (if _array_element
      (Math|Integer|IncrementInt (Variables|Default|GetDrapeSum))))
  (switch int (Variables|Default|GetDrapeSum)
    (:2
      (Default|PlayNextSound _voicemanageref "/Game/EyeSurgery/Sounds/消毒铺巾/Step4/2.2"))
    (:3
      (bind _isfinished (Default|TaskFinished _taskmanageref 3))
      (if _isfinished
        (Default|TaskInit _taskmanageref 4)
        (Default|PlayNextSound _voicemanageref "/Game/EyeSurgery/Sounds/消毒铺巾/Step5/1.1")
        (Utilities|FlowControl|Delay 2.0)
        (Default|PlayNextSound _voicemanageref "/Game/EyeSurgery/Sounds/消毒铺巾/Step5/2.2")))
    (:4
      (Default|TaskFinished _taskmanageref 4)
      (Default|PlayNextSound _voicemanageref "/Game/EyeSurgery/Sounds/消毒铺巾/Step6/1.1")
      (Utilities|FlowControl|Delay 2.5)
      (Default|PlayNextSound _voicemanageref "/Game/EyeSurgery/Sounds/消毒铺巾/Step6/2.2"))
    (:8
      (Default|TaskFinished _taskmanageref 5)
      (Default|PlayNextSound _voicemanageref "/Game/EyeSurgery/Sounds/消毒铺巾/Step7/1.1")
      (Utilities|FlowControl|Delay 3.4)
      (Default|PlayNextSound _voicemanageref "/Game/EyeSurgery/Sounds/消毒铺巾/Step7/2.2"))
    (:9
      (bind _isfinished_2 (Default|TaskFinished _taskmanageref 6))
      (if _isfinished_2
        (Default|TaskInit _taskmanageref 7)
        (Default|PlayNextSound _voicemanageref "/Game/EyeSurgery/Sounds/消毒铺巾/Step8/1.1")
        (Utilities|FlowControl|Delay 3.5)
        (Default|PlayNextSound _voicemanageref "/Game/EyeSurgery/Sounds/消毒铺巾/Step8/2.2")))))

(event Custom|SpawnDrape
  (params (DrapeTag :type Name))
  ;[1 1 1] 生成对应类型的Drape
  (bind _asbp_eye_vr_char (Utilities|Casting|CastToBP_Eye_VR_Char (Game|Player|GetPlayerPawn 0)))
  (Default|SpawnActor (Variables|Default|GetComp_SpawnActor) _asbp_eye_vr_char "/Game/VR-Space/Draping/BP_DrapeToSnap.BP_DrapeToSnap_C" false)
  (CallFunction|ChangeDrapeType DrapeTag))

(event EventBeginPlay
  (EventDispatchers|BindEventtoDrapeAttached (delegate Custom|ChangeDrapeArray)))

(fn ConstructionScript)

(fn ChangeDrapeType
  (params (DrapeTag :type Name))
  (bind _outactors (Actor|GetAllActorsOfClass "/Game/VR-Space/Draping/BP_DrapeToSnap.BP_DrapeToSnap_C"))
  (for _array_element _outactors
    (bind _output_get (Variables|/Game/VR-Space/Draping/BP_DrapeToSnap.BP_DrapeToSnap_C|SetConnectorID _array_element DrapeTag))
    (Variables|/Game/AFCore/Blueprints/Components/Snapping/Comp_Connector_Anchor.Comp_Connector_Anchor_C|SetConnectorID (Variables|/Game/VR-Space/Draping/BP_DrapeToSnap.BP_DrapeToSnap_C|GetComp_Connector_Anchor _array_element) _output_get)))