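; Eye-drop bottle actor for the eye surgery game, a grabbable prop that releases drops and cues sounds.
; GenerateDrops, bound to the V key, spawns a BP_Drip at the Export component with a fixed flipped rotation.
; Pickup through Comp_Grab plays a BP_VoiceManage sound, and DripFinished plays a confirmation sound after a short delay.
; The grab Trigger input branches on controller side, with no actions attached.
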(event GrabKeyInput(Comp_Grab)
  (params (MComp :type BP%20M%20Comp%20Object%20Reference) (Key :type Enum_Controller_Buttons%20Enum :default "NewEnumerator1") (Set :type Boolean))
  (switch Utilities|FlowControl|Switch|SwitchonEnum_Controller_Buttons Key
    (:NewEnumerator0
      (switch Utilities|FlowControl|Switch|SwitchonEnum_Side (Variables|/Game/AFCore/Blueprints/VR/MotionComponents/BP_MComp.BP_MComp_C|GetSide MComp)))))

(event GrabActorPickedUp(Comp_Grab)
  (params (GrabbingPawn :type BP%20Pawn%20Base%20Object%20Reference) (GrabbingActor :type Actor%20Object%20Reference))
  (bind _returnvalue (Actor|GetActorOfClass "/Game/EyeSurgery/BluePrint/Voice/BP_VoiceManage.BP_VoiceManage_C"))
  (Utilities|IsValid _returnvalue
    (:Is%20Valid
      (Default|PlayNextSound _returnvalue "/Game/EyeSurgery/Sounds/麻醉前安全核查/Step1/4.4"))))

(event Custom|GenerateDrops
  (Game|SpawnActorfromClass "/Game/EyeSurgery/BluePrint/Object/Animate/BP_Drip.BP_Drip_C" (Math|Transform|MakeTransform (Transformation|GetWorldLocation (Variables|Default|GetExport)) "0, 0,180.000000" "1.000000,1.000000,1.000000") "Undefined" 0 0))

(event Custom|DripFinished
  (Utilities|FlowControl|Delay 3.5)
  (Default|PlayNextSound (stale GrabActorPickedUp(Comp_Grab) _returnvalue) "/Game/EyeSurgery/Sounds/麻醉前安全核查/Step1/Confirmation_of_the_operation.Confirmation_of_the_operation"))

(event EventBeginPlay
  (Input|EnableInput (Game|GetPlayerController 0)))

(event Collision|EventActorBeginOverlap
  (params (OtherActor :type Actor%20Object%20Reference)))

(event EventTick
  (params (DeltaSeconds :type Float%20%28single-precision%29)))

(event Input|KeyboardEvents|V
  (params (Key :type Key%20Structure :default "None"))
  (:Pressed
    (CallFunction|GenerateDrops)))

(fn ConstructionScript)