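; BP_Drip is an eye-drop droplet actor for an eye surgery procedure, destroying itself on any hit and printing what it struck.
; Landing on BP_EyeDorpHit plays the next voice line through BP_VoiceManage and swaps the eye-open patient mesh's material.
; It then updates the patient button on the pre-anesthesia (麻醉前) widget hosted by BP_BaseBoard and calls DripFinished on the eye-drop actor (眼药水).
; All targets are found through GetActorOfClass lookups.
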(event EventBeginPlay)

(event Collision|EventHit
  (params (MyComp :type Primitive%20Component%20Object%20Reference) (Other :type Actor%20Object%20Reference) (OtherComp :type Primitive%20Component%20Object%20Reference) (bSelfMoved :type Boolean) (HitLocation :type Vector :default "0, 0, 0") (HitNormal :type Vector :default "0, 0, 0") (NormalImpulse :type Vector :default "0, 0, 0") (Hit :type Hit%20Result%20Structure%20%28by%20ref%29))
  (bind _hitactor (Collision|BreakHitResult Hit))
  (Actor|DestroyActor)
  (Development|PrintString (Utilities|GetDisplayName _hitactor))
  (if (== (Utilities|GetClass _hitactor) "/Game/EyeSurgery/BluePrint/Object/Helpers/BP_EyeDorpHit.BP_EyeDorpHit_C")
    (bind _returnvalue (Actor|GetActorOfClass "/Game/EyeSurgery/BluePrint/Voice/BP_VoiceManage.BP_VoiceManage_C"))
    (Utilities|IsValid _returnvalue
      (:Is%20Valid
        (Default|PlayNextSound _returnvalue "/Game/EyeSurgery/Sounds/麻醉前安全核查/Step1/5.5")
        (bind _returnvalue_2 (Actor|GetActorOfClass "/Game/VR-Space/人物资产/vr眼科人物模型/患者-睁眼.患者-睁眼_C"))
        (Rendering|Material|SetMaterial (Variables|/Game/VR-Space/人物资产/vr眼科人物模型/患者-睁眼.患者-睁眼_C|GetSM_MERGED_StaticMeshActor_ok _returnvalue_2) 0 "/Game/人物资产/消毒人/M_SM_MERGED_StaticMeshActor_ok6mm.M_SM_MERGED_StaticMeshActor_ok6mm")
        (bind _returnvalue_3 (Actor|GetActorOfClass "/Game/EyeSurgery/BluePrint/UI/BP_BaseBoard.BP_BaseBoard_C"))
        (bind _asw_麻醉前 (Utilities|Casting|CastToW_麻醉前 (Default|GetWidgetObject (Variables|/Game/AFCore/Blueprints/UI/Static/BP_Board.BP_Board_C|GetComp_Widget _returnvalue_3))))
        (Utilities|IsValid _asw_麻醉前
          (:Is%20Valid
            (Default|DeactivateButton (Variables|/Game/EyeSurgery/BluePrint/Widget/W_麻醉前.W_麻醉前_C|GetWidget_Button_Patient _asw_麻醉前) false false)
            (bind _returnvalue_4 (Actor|GetActorOfClass "/Game/EyeSurgery/BluePrint/Object/Animate/BP_眼药水.BP_眼药水_C"))
            (Utilities|IsValid _returnvalue_4
              (:Is%20Valid
                (Default|DripFinished _returnvalue_4)))))))))

(fn ConstructionScript)