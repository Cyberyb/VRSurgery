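; BP_PosLable is a position registry for the EyeSurgery game that moves the player pawn to predefined spots in a level.
; On BeginPlay it resolves a level number by looking up its LevelDA in LevelMap.
; TransferPawn switches on that number and, for level 1 only, sets the player pawn's location to the valid actor mapped to the requested index in PositionsMap, without sweep or rotation change.
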(event EventBeginPlay
  (bind _levelda (Variables|Default|GetLevelDA))
  (bind _levelmap (Variables|Default|GetLevelMap))
  (bind (_value _returnvalue) (Utilities|Map|Find _levelmap _levelda))
  (if _returnvalue
    (Variables|Default|SetLevelNum _value)))

(event Collision|EventActorBeginOverlap
  (params (OtherActor :type Actor%20Object%20Reference)))

(event EventTick
  (params (DeltaSeconds :type Float%20%28single-precision%29)))

(fn ConstructionScript)

(fn TransferPawn
  (params (PosNum :type Integer))
  (bind _positionsmap (Variables|Default|GetPositionsMap))
  (bind _value (Utilities|Map|Find _positionsmap PosNum))
  (switch int (Variables|Default|GetLevelNum)
    (:1
      (Utilities|IsValid _value
        (:Is%20Valid
          (Transformation|SetActorLocation (Game|Player|GetPlayerPawn 0) (Transformation|GetActorLocation _value) false false))))))