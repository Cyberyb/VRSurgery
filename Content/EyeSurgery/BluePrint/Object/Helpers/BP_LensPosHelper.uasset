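; BP_LensPosHelper is an eye surgery helper actor that positions a lens geometry cache and drives its level sequence animation.
; PlaySequence plays LensSequence up to a frame bias short of its end, and Tick sets Stage to 2 once playback reaches frame 25.
; SetLensTransform moves the GCLens geometry cache component to a given world transform, adding a 90-degree yaw offset.
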(event Custom|PlaySequence
  (bind _lenssequence (Variables|Default|GetLensSequence))
  (bind _sequenceplayer (Variables|/Script/LevelSequence.LevelSequenceActor|GetSequencePlayer _lenssequence))
  (Class|MovieSceneSequencePlayer|Playto _sequenceplayer (Utilities|Struct|MakeMovieSceneSequencePlaybackParams (Utilities|Struct|MakeFrameTime (Utilities|Struct|MakeFrameNumber (- (Class|MovieSceneSequencePlayer|GetFrameDuration _sequenceplayer) (Variables|Default|GetFrameBias))) 0.0) 0.0 "" "Frame" "Play" false)))

(event EventBeginPlay)

(event Collision|EventActorBeginOverlap
  (params (OtherActor :type Actor%20Object%20Reference)))

(event EventTick
  (params (DeltaSeconds :type Float%20%28single-precision%29))
  (if (>= (.value (.frame (Sequencer|Player|GetCurrentTime (Variables|/Script/LevelSequence.LevelSequenceActor|GetSequencePlayer (Variables|Default|GetLensSequence))))) 25)
    (Variables|Default|SetStage 2)))

(fn ConstructionScript)

(fn SetLensTransform
  (params (NewTransform :type Transform))
  (bind (_location _rotation _scale) (Math|Transform|BreakTransform NewTransform))
  (bind _gc_lens (Variables|Default|GetGC_Lens))
  (Utilities|IsValid _gc_lens
    (:Is%20Valid
      (Transformation|SetWorldTransform (Variables|/Script/GeometryCache.GeometryCacheActor|GetGeometryCacheComponent _gc_lens) (Math|Transform|MakeTransform _location (Math|Rotator|MakeRotator (.roll _rotation) (.pitch _rotation) (+ (.yaw _rotation) 9e+01)) _scale) false false))))