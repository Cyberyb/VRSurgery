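; Helper for the VR eye surgery game that switches the mode of the phacoemulsification handpiece (超声乳化手柄).
; It binds to a toggle-mode event on BeginPlay, then finds the laser component on the left or right motion controller.
; That laser releases its held tool and grabs a newly spawned suction or shrink tool at the same transform, chosen by a flipping boolean.
; The tip board then updates to the new mode.
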(event Custom|ToggleToolMode
  (params (Tool :type E_ToolMode%20Enum :default "NewEnumerator0") (Side :type Enum_Side%20Enum :default "NewEnumerator0"))
  (bind _phacoemulsificationmode (Variables|Default|GetPhacoemulsificationMode))
  (Development|PrintString (Utilities|String|EnumtoString Tool))
  (switch Utilities|FlowControl|Switch|SwitchonE_ToolMode Tool
    (:NewEnumerator0
      (CallFunction|ChangePHAMode Side _phacoemulsificationmode)
      (bind _returnvalue (Actor|GetActorOfClass "/Game/EyeSurgery/BluePrint/UI/BP_TipBoard.BP_TipBoard_C"))
      (Utilities|IsValid _returnvalue
        (:Is%20Valid
          (Default|UpdateToolTip _returnvalue "NewEnumerator0" _phacoemulsificationmode))))))

(event EventBeginPlay
  (EventDispatchers|BindEventtoToggleMode (delegate Custom|ToggleToolMode)))

(event Collision|EventActorBeginOverlap
  (params (OtherActor :type Actor%20Object%20Reference)))

(event EventTick
  (params (DeltaSeconds :type Float%20%28single-precision%29)))

(fn ConstructionScript)

(fn ChangePHAMode
  (params (Side :type Enum_Side%20Enum :default "NewEnumerator0") (Mode :type Boolean))
  (switch Utilities|FlowControl|Switch|SwitchonEnum_Side Side
    (:NewEnumerator0
      (bind _returnvalue (Actor|GetActorOfClass "/Game/AFCore/Blueprints/VR/MotionControllers/Controller/BP_MotionController_Controller_Eye_Left.BP_MotionController_Controller_Eye_Left_C"))
      (bind _asbp_mcomp_laser (Utilities|Casting|CastToBP_MComp_Laser (Variables|/Script/Engine.ChildActorComponent|GetChildActor (Variables|/Game/AFCore/Blueprints/VR/MotionControllers/Controller/BP_MotionController_Controller_Eye_Left.BP_MotionController_Controller_Eye_Left_C|GetMComp_Grab _returnvalue))))
      (LocalVariables|SetLaser _asbp_mcomp_laser))
    (:NewEnumerator1
      (bind _returnvalue_2 (Actor|GetActorOfClass "/Game/AFCore/Blueprints/VR/MotionControllers/Controller/BP_MotionController_Controller_Eye_Right.BP_MotionController_Controller_Eye_Right_C"))
      (bind _asbp_mcomp_laser_2 (Utilities|Casting|CastToBP_MComp_Laser (Variables|/Script/Engine.ChildActorComponent|GetChildActor (Variables|/Game/AFCore/Blueprints/VR/MotionControllers/Controller/BP_MotionController_Controller_Eye_Right.BP_MotionController_Controller_Eye_Right_C|GetMComp_LaserPointer _returnvalue_2))))
      (LocalVariables|SetLaser _asbp_mcomp_laser_2)))
  (bind _laser (LocalVariables|GetLaser)
    (:then
      (bind _output_get (LocalVariables|SetGrabbedTool (Variables|/Game/AFCore/Blueprints/VR/MotionComponents/BP_MComp_Laser.BP_MComp_Laser_C|GetGrabbedActor _laser)))
      (Default|GrabbingActorReleaseActor _laser)
      (bind _asactor (Utilities|Casting|CastToActorClass (Class|KismetMathLibrary|SelectClass "/Game/EyeSurgery/CataractRemovalNew/BP_SuctionTool.BP_SuctionTool_C" "/Game/EyeSurgery/CataractRemovalNew/BP_ShrinkTool.BP_ShrinkTool_C" Mode)))
      (bind _returnvalue_3 (Game|SpawnActorfromClass _asactor (Math|Transform|MakeTransform (Transformation|GetActorLocation _output_get) (Transformation|GetActorRotation _output_get) "1.000000,1.000000,1.000000") "Undefined" 0 0))
      (Default|SearchandGrabActor _laser _returnvalue_3)
      (bind _output_get_2 (Variables|Default|SetPhacoemulsificationMode (not Mode)))
      (return _output_get_2))
    (:else)))