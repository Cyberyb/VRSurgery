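; BP_TearHepler is an eye-surgery helper that scrubs a paused tear Level Sequence by following the capsule-tearing forceps (BP_撕嚢镊) around its Sphere.
; Overlap events on the Sphere track the forceps and cache their detection sphere.
; While overlapped, Tick converts the forceps' offset in the world YZ plane into a 0–360° angle from downward, via cross/dot atan2.
; That angle sets the proportional playback frame.
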(event OnComponentBeginOverlap(Sphere)
  (params (OverlappedComponent :type Primitive%20Component%20Object%20Reference) (OtherActor :type Actor%20Object%20Reference) (OtherComp :type Primitive%20Component%20Object%20Reference) (OtherBodyIndex :type Integer) (bFromSweep :type Boolean) (SweepResult :type Hit%20Result%20Structure%20%28by%20ref%29))
  (if (== (Utilities|GetClass OtherActor) "/Game/EyeSurgery/BluePrint/Object/Tools/BP_撕嚢镊.BP_撕嚢镊_C")
    (Development|PrintString "Overlaping!!!")
    (Variables|Default|SetOverlapped true)
    (bind _returnvalue (Actor|GetActorOfClass "/Game/EyeSurgery/BluePrint/Object/Tools/BP_撕嚢镊.BP_撕嚢镊_C"))
    (Variables|Default|SetDetectSphere (Variables|/Game/EyeSurgery/BluePrint/Object/Tools/BP_撕嚢镊.BP_撕嚢镊_C|GetSphere _returnvalue))
    (else
      (Development|PrintString "Not Correct!!!"))))

(event OnComponentEndOverlap(Sphere)
  (params (OverlappedComponent :type Primitive%20Component%20Object%20Reference) (OtherActor :type Actor%20Object%20Reference) (OtherComp :type Primitive%20Component%20Object%20Reference) (OtherBodyIndex :type Integer))
  (if (== (Utilities|GetClass OtherActor) "/Game/EyeSurgery/BluePrint/Object/Tools/BP_撕嚢镊.BP_撕嚢镊_C")
    (Variables|Default|SetOverlapped false)))

(event EventBeginPlay
  (Sequencer|Player|Pause (Variables|/Script/LevelSequence.LevelSequenceActor|GetSequencePlayer (Variables|Default|GetTearSequence))))

(event Collision|EventActorBeginOverlap
  (params (OtherActor :type Actor%20Object%20Reference)))

(event EventTick
  (params (DeltaSeconds :type Float%20%28single-precision%29))
  (if (Variables|Default|GetOverlapped)
    (bind _detectsphere (Variables|Default|GetDetectSphere)
      (:then
        (bind _angel (CallFunction|CalculateAngel (Math|Vector2D|MakeVector2D (.Y (Math|Vector|BreakVector (- (Transformation|GetWorldLocation _detectsphere) (Transformation|GetWorldLocation (Variables|Default|GetSphere))))) (.Z (Math|Vector|BreakVector (- (Transformation|GetWorldLocation _detectsphere) (Transformation|GetWorldLocation (Variables|Default|GetSphere)))))) "(X=0.000000,Y=-1.000000)"))
        (bind _tearsequence (Variables|Default|GetTearSequence)
          (:then
            (Development|PrintString (Utilities|String|ToString(Integer) (Math|Float|Truncate (* (/ _angel 3.6e+02) (Class|MovieSceneSequencePlayer|GetFrameDuration (Variables|/Script/LevelSequence.LevelSequenceActor|GetSequencePlayer _tearsequence))))))
            (Components|Timeline|SetPlaybackPosition (Variables|/Script/LevelSequence.LevelSequenceActor|GetSequencePlayer _tearsequence) (Utilities|Struct|MakeMovieSceneSequencePlaybackParams (Utilities|Struct|MakeFrameTime (Utilities|Struct|MakeFrameNumber (Math|Float|Truncate (* (/ _angel 3.6e+02) (Class|MovieSceneSequencePlayer|GetFrameDuration (Variables|/Script/LevelSequence.LevelSequenceActor|GetSequencePlayer _tearsequence))))) 0.0) 0.0 "" "Frame" "Play" false)))
          (:else)))
      (:else))))

(fn ConstructionScript)

(fn CalculateAngel
  (params (StartPos :type Vector%202D%20Structure) (EndPos :type Vector%202D%20Structure))
  (bind _returnvalue (Math|Vector2D|DotProduct(2D) StartPos EndPos))
  (bind _returnvalue_2 (Class|KismetMathLibrary|CrossProduct2D StartPos EndPos))
  (bind _returnvalue_3 (Class|KismetMathLibrary|DegAtan2 _returnvalue_2 _returnvalue))
  (return (select (< _returnvalue_2 0.0) (- 3.6e+02 (Math|Float|Absolute(Float) _returnvalue_3)) _returnvalue_3)))