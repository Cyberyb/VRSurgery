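; Helper actor that exports an eye surgery session's scores to an Excel workbook.
; SaveToExcel builds a workbook through InsertScore, saves it under the project's Scores folder with a timestamp name, and returns a path rebuilt from the current time.
; InsertScore calls AddScoreTitle for user, time and column headers, then writes each BP_ScoreManage task name and score to a row offset by TaskID.
; The event graph is inactive.
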(event EventBeginPlay)

(event Collision|EventActorBeginOverlap
  (params (OtherActor :type Actor%20Object%20Reference)))

(event EventTick
  (params (DeltaSeconds :type Float%20%28single-precision%29)))

(fn ConstructionScript)

(fn InsertScore
  (params (WorkBook :type Excel%20Workbook%20Object%20Reference) (WorkSheet :type Excel%20Worksheet%20Object%20Reference))
  (bind _returnvalue (Class|ExcelWorkbook|Sheetat WorkBook))
  (CallFunction|AddScoreTitle WorkBook)
  (bind _returnvalue_2 (Actor|GetActorOfClass "/Game/EyeSurgery/BluePrint/Object/Helpers/BP_ScoreManage.BP_ScoreManage_C"))
  (Utilities|IsValid _returnvalue_2
    (:Is%20Valid
      (for _array_element (Variables|/Game/EyeSurgery/BluePrint/Object/Helpers/BP_ScoreManage.BP_ScoreManage_C|GetSurgeryScore _returnvalue_2)
        (Class|ExcelCell|SetString (Class|ExcelWorksheet|Cellat _returnvalue 1 (+ (.taskid _array_element) 4)) (Utilities|String|EnumtoString (.taskname _array_element)))
        (Class|ExcelCell|SetString (Class|ExcelWorksheet|Cellat _returnvalue 2 (+ (.taskid _array_element) 4)) (Utilities|String|ToString(Integer) (.score _array_element))))
      (return WorkBook))))

(fn AddScoreTitle
  (params (WorkBook :type Excel%20Workbook%20Object%20Reference))
  (bind _returnvalue (Class|ExcelWorkbook|Sheetat WorkBook))
  (bind _returnvalue_2 (Math|DateTime|Now))
  (bind _gameinstance (CallFunction|GetMainGameInstance self))
  ;[1 1 1] 用户名
  (Class|ExcelCell|SetString (Class|ExcelWorksheet|Cellat _returnvalue 1 1) "用户名：")
  (Class|ExcelCell|SetString (Class|ExcelWorksheet|Cellat _returnvalue 2 1) (Variables|/Game/AFCore/Blueprints/Game/BP_GameInstance_Main.BP_GameInstance_Main_C|GetCurUser _gameinstance))
  ;[1 1 1] 时间
  (Class|ExcelCell|SetString (Class|ExcelWorksheet|Cellat _returnvalue 1 2) "时间：")
  (Class|ExcelCell|SetString (Class|ExcelWorksheet|Cellat _returnvalue 2 2) (Utilities|String|Append (Utilities|String|ToString(Integer) (.year _returnvalue_2)) "/" (Utilities|String|ToString(Integer) (.month _returnvalue_2)) "/" (Utilities|String|ToString(Integer) (.day _returnvalue_2)) " " (Utilities|String|ToString(Integer) (.hour _returnvalue_2)) ":" (Utilities|String|ToString(Integer) (.minute _returnvalue_2)) ":" (Utilities|String|ToString(Integer) (.second _returnvalue_2))))
  ;[1 1 1] Title
  (Class|ExcelCell|SetString (Class|ExcelWorksheet|Cellat _returnvalue 1 3) "项目名称")
  (Class|ExcelCell|SetString (Class|ExcelWorksheet|Cellat _returnvalue 2 3) "百分制成绩"))

(fn SavetoExcel
  (bind _returnvalue (Math|DateTime|Now))
  (bind _returnvalue_2 (Utilities|String|ToString(Integer) (.month _returnvalue)))
  (bind _returnvalue_3 (Utilities|String|ToString(Integer) (.day _returnvalue)))
  (bind _returnvalue_4 (Utilities|String|ToString(Integer) (.hour _returnvalue)))
  (bind _returnvalue_5 (Utilities|String|ToString(Integer) (.minute _returnvalue)))
  (bind _returnvalue_6 (Utilities|String|ToString(Integer) (.second _returnvalue)))
  (bind _returnvalue_7 (Utilities|String|ToString(Integer) (.year _returnvalue)))
  (bind _returnvalue_8 (Utilities|String|Append _returnvalue_7 _returnvalue_2 _returnvalue_3 _returnvalue_4 _returnvalue_5 _returnvalue_6 ".xlsx"))
  (bind _returnvalue_9 (Utilities|String|Append "Scores/" _returnvalue_8))
  (bind _returnvalue_10 (Game|ConstructObjectfromClass "/Script/DirectExcel.ExcelWorkbook"))
  (bind _outbook (CallFunction|InsertScore _returnvalue_10))
  (bind _returnvalue_11 (Class|ExcelWorkbook|Saveas _outbook _returnvalue_9 "ProjectDir"))
  (if _returnvalue_11
    (Development|PrintString "Save Excel Success!")
    (return _returnvalue_9)))