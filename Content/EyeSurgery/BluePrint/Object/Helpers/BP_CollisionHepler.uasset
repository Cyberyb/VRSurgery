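; Helper actor for the eye surgery game that spawns and fades a viscoelastic agent (粘弹剂) decal.
; SpawnVisDecal stores the decal it places; FadeDecal sets its fade-out and starts a timeline driving opacity through a shared Material Parameter Collection.
; CalculateAngel separately returns the 0–360 degree angle between two 2D vectors.
; MainSphere overlap, BeginPlay and Tick handlers are empty, with leftover unconnected scaling and class-check nodes.
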(event OnComponentBeginOverlap(MainSphere)
  (params (OverlappedComponent :type Primitive%20Component%20Object%20Reference) (OtherActor :type Actor%20Object%20Reference) (OtherComp :type Primitive%20Component%20Object%20Reference) (OtherBodyIndex :type Integer) (bFromSweep :type Boolean) (SweepResult :type Hit%20Result%20Structure%20%28by%20ref%29)))

(event OnComponentEndOverlap(MainSphere)
  (params (OverlappedComponent :type Primitive%20Component%20Object%20Reference) (OtherActor :type Actor%20Object%20Reference) (OtherComp :type Primitive%20Component%20Object%20Reference) (OtherBodyIndex :type Integer)))

(event Custom|FadeOutDecal
  (params (Decal :type Decal%20Component%20Object%20Reference))
  (bind _新建轨道_0 (Timeline|不透明度 Play)
    (:Update
      (Rendering|Material|SetScalarParameterValue "/Game/VR-Space/Surgery/Material/MSC_粘弹剂.MSC_粘弹剂" "不透明度" _新建轨道_0 :!class /Script/Engine.KismetMaterialLibrary))))

(event EventBeginPlay)

(event Collision|EventActorBeginOverlap
  (params (OtherActor :type Actor%20Object%20Reference)))

(event EventTick
  (params (DeltaSeconds :type Float%20%28single-precision%29)))

(fn ConstructionScript)

(fn CalculateAngel
  (params (StartPos :type Vector%202D%20Structure) (EndPos :type Vector%202D%20Structure))
  (bind _returnvalue (Math|Vector2D|DotProduct(2D) StartPos EndPos))
  (bind _returnvalue_2 (Class|KismetMathLibrary|CrossProduct2D StartPos EndPos))
  (bind _returnvalue_3 (Class|KismetMathLibrary|DegAtan2 _returnvalue_2 _returnvalue))
  (return (select (< _returnvalue_2 0.0) (- 3.6e+02 (Math|Float|Absolute(Float) _returnvalue_3)) _returnvalue_3)))

(fn SpawnVisDecal
  (params (Location :type Vector))
  (bind _returnvalue (Rendering|Decal|SpawnDecalatLocation "/Game/VR-Space/Surgery/Material/M_粘弹剂.M_粘弹剂" "6.000000,14.000000,14.000000" Location "0.000000,180.000000,180.000000" 0.0))
  (Variables|Default|SetDecals _returnvalue))

(fn FadeDecal
  (bind _decals (Variables|Default|GetDecals))
  (Utilities|IsValid _decals
    (:Is%20Valid
      (Rendering|Components|Decal|SetFadeOut _decals 0.0 2.0 true)
      (CallFunction|FadeOutDecal _decals))))