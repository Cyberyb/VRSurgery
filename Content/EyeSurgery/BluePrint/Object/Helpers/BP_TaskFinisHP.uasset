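; Helper Blueprint that handles step completion in a staged cataract surgery simulation, from incision through lens implantation to sealing the wound.
; CheckFinished switches on a task ID, calls TaskManage.TaskFinished and plays a SurgeryVoice clip when it succeeds, except the incision step, which plays unconditionally.
; The final step instead calls ShowScoreBoard, which finds the BP_ScoreTipBoard actor and makes its widget visible.
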(event EventBeginPlay)

(event Collision|EventActorBeginOverlap
  (params (OtherActor :type Actor%20Object%20Reference)))

(event EventTick
  (params (DeltaSeconds :type Float%20%28single-precision%29)))

(fn ConstructionScript)

(fn CheckFinished
  (params (TaskID :type Integer))
  (switch int TaskID
    (:0
      ;[1 1 1] 切口
      (Default|TaskFinished (Variables|Default|GetTaskManage))
      (Default|PlayVoice (Variables|Default|GetSurgeryVoice) 1))
    (:1
      ;[1 1 1] 注射粘弹剂1
      (bind _isfinished (Default|TaskFinished (Variables|Default|GetTaskManage) 1))
      (if _isfinished
        (Default|PlayVoice (Variables|Default|GetSurgeryVoice) 2)))
    (:2
      ;[1 1 1] 撕嚢
      (bind _isfinished_2 (Default|TaskFinished (Variables|Default|GetTaskManage) 2))
      (if _isfinished_2
        (Default|PlayVoice (Variables|Default|GetSurgeryVoice) 5)))
    (:3
      ;[1 1 1] 水分离
      (bind _isfinished_3 (Default|TaskFinished (Variables|Default|GetTaskManage) 3))
      (if _isfinished_3
        (Default|PlayVoice (Variables|Default|GetSurgeryVoice) 6)))
    (:4
      ;[1 1 1] 刻槽劈核
      (bind _isfinished_4 (Default|TaskFinished (Variables|Default|GetTaskManage) 4))
      (if _isfinished_4
        (Default|PlayVoice (Variables|Default|GetSurgeryVoice) 7)))
    (:5
      ;[1 1 1] 吸取皮质
      (bind _isfinished_5 (Default|TaskFinished (Variables|Default|GetTaskManage) 5))
      (if _isfinished_5
        (Default|PlayVoice (Variables|Default|GetSurgeryVoice) 8)))
    (:6
      ;[1 1 1] 注射粘弹剂
      (bind _isfinished_6 (Default|TaskFinished (Variables|Default|GetTaskManage) 6))
      (if _isfinished_6
        (Default|PlayVoice (Variables|Default|GetSurgeryVoice) 9)))
    (:7
      ;[1 1 1] 注射晶状体
      (bind _isfinished_7 (Default|TaskFinished (Variables|Default|GetTaskManage) 7))
      (if _isfinished_7
        (Default|PlayVoice (Variables|Default|GetSurgeryVoice) 10)))
    (:8
      ;[1 1 1] 抽吸粘弹剂
      (bind _isfinished_8 (Default|TaskFinished (Variables|Default|GetTaskManage) 8))
      (if _isfinished_8
        (Default|PlayVoice (Variables|Default|GetSurgeryVoice) 11)))
    (:9
      ;[1 1 1] 水密切口
      (bind _isfinished_9 (Default|TaskFinished (Variables|Default|GetTaskManage) 9))
      (if _isfinished_9
        (CallFunction|ShowScoreBoard)))))

(fn ShowScoreBoard
  (bind _returnvalue (Actor|GetActorOfClass "/Game/EyeSurgery/BluePrint/UI/BP_ScoreTipBoard.BP_ScoreTipBoard_C"))
  (Utilities|IsValid _returnvalue
    (:Is%20Valid
      (Default|SetWidgetVisibility (Variables|/Game/AFCore/Blueprints/UI/Static/BP_Board.BP_Board_C|GetComp_Widget _returnvalue) true))))