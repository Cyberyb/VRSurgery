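; BP_ScoreManage is a helper actor that records scores for tasks in an eye surgery simulation.
; RecordScore uses FindItembyName to search the SurgeryScore array for the entry matching a task name enum, sets its score through a struct reference, and prints the task and score.
; Unknown tasks are ignored, and the event graph holds only disabled default events.
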(event EventBeginPlay)

(event Collision|EventActorBeginOverlap
  (params (OtherActor :type Actor%20Object%20Reference)))

(event EventTick
  (params (DeltaSeconds :type Float%20%28single-precision%29)))

(fn ConstructionScript)

(fn RecordScore
  (params (TaskName :type E_SurgeryTaskName%20Enum :default "NewEnumerator0") (Score :type Integer))
  (bind (_scoreref _found) (CallFunction|FindItembyName TaskName))
  (if _found
    (bind _structout (Utilities|Struct|SetmembersinS_SurgeryScore _scoreref Score))
    (Development|PrintString (Utilities|String|Append (Utilities|String|Append "当前任务：" (Utilities|String|EnumtoString (.taskname _structout))) (Utilities|String|Append "  分数：" (Utilities|String|ToString(Integer) (.score _structout)))))))

(fn FindItembyName
  (params (TaskName :type E_SurgeryTaskName%20Enum :default "NewEnumerator0"))
  (bind _surgeryscore (Variables|Default|GetSurgeryScore))
  (bind (_array_element _array_index) (Utilities|Array|ForEachLoopwithBreak (Variables|Default|GetSurgeryScore))
    (:LoopBody
      (if (Utilities|Enum|Equal(Enum) (.taskname _array_element) TaskName)
        (return (Utilities|Array|Get(acopy) _surgeryscore _array_index) true)))
    (:Completed
      (return (Utilities|Array|Get(acopy) _surgeryscore) false))))