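; BP_夹子Manage is a clamp manager in the EyeSurgery VR game that completes task 7 once both clamp positions have clamps attached.
; CheckState checks both Attached flags, then reports to TaskManageRef.
; On success it spawns a W_Tips widget through the VR pawn's UI component, announcing completion and a return to the start screen.
; After a short delay, or immediately if the pawn cast fails, it initializes task 8.
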(event Custom|CheckState
  (bind _taskmanageref (Variables|Default|GetTaskManageRef))
  (if (and (Variables|/Game/EyeSurgery/BluePrint/Object/BP_巾钳位置.BP_巾钳位置_C|GetAttached (Variables|Default|Get夹子位置1)) (Variables|/Game/EyeSurgery/BluePrint/Object/BP_巾钳位置.BP_巾钳位置_C|GetAttached (Variables|Default|Get夹子位置2)))
    (bind _isfinished (Default|TaskFinished _taskmanageref 7))
    (if _isfinished
      (bind _asbp_eye_vr_char (Utilities|Casting|CastToBP_Eye_VR_Char (Game|Player|GetPlayerPawn 0))
        (:then
          (bind _widgetobject (Default|SpawnElement (Variables|/Game/EyeSurgery/BluePrint/Pawn/BP_Eye_VR_Char.BP_Eye_VR_Char_C|GetComp_PawnUI _asbp_eye_vr_char) "/Game/EyeSurgery/BluePrint/Widget/W_Tips.W_Tips_C" "NewEnumerator0" false 0.0 false 1.0))
          (bind _asw_tips (Utilities|Casting|CastToW_Tips _widgetobject))
          (Default|SetTipCpntent _asw_tips "恭喜您完成任务！正在前往开始界面")
          (Utilities|FlowControl|Delay 2.0))
        (:CastFailed
          _))
      (Default|TaskInit _taskmanageref 8))))

(event EventBeginPlay)

(event Collision|EventActorBeginOverlap
  (params (OtherActor :type Actor%20Object%20Reference)))

(event EventTick
  (params (DeltaSeconds :type Float%20%28single-precision%29)))

(fn ConstructionScript)