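; Utility function library for the EyeSurgery game, offering math helpers and global shortcuts for task completion and score recording.
; Math helpers sum and average float arrays and compute the centroid of a point array, with no empty-array guard.
; TaskFinished and RecordScore look up BP_TaskFinisHP and BP_ScoreManage by class and forward calls to them; only the former checks that the actor is valid.
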(fn SumOfFloatArray
  (params (Array :type Array%20of%20Floats%20%28double-precision%29))
  (LocalVariables|SetRes 0.0)
  (for _array_element Array
    (LocalVariables|SetRes (+ _array_element (LocalVariables|GetRes))))
  (return (LocalVariables|GetRes)))

(fn AvgOfFloatArray
  (params (Array :type Array%20of%20Floats%20%28double-precision%29))
  (return (/ (CallFunction|SumOfFloatArray Array) (Utilities|Array|Length Array))))

(fn CenterPoint
  (params (Points :type Array%20of%20Vectors))
  (Utilities|FlowControl|Sequence
    (:then_0
      (LocalVariables|SetSum "0, 0, 0"))
    (:then_1
      (for _array_element Points
        (LocalVariables|SetSum (+ _array_element (LocalVariables|GetSum))))
      (return (/ (LocalVariables|GetSum) (Utilities|Array|Length Points))))))

(fn TaskFinished
  (params (TaskID :type Integer))
  (bind _returnvalue (Actor|GetActorOfClass 0 "/Game/EyeSurgery/BluePrint/Object/Helpers/BP_TaskFinisHP.BP_TaskFinisHP_C"))
  (Utilities|IsValid _returnvalue
    (:Is%20Valid
      (Default|CheckFinished _returnvalue TaskID))))

(fn RecordScore
  (params (TaskName :type E_SurgeryTaskName%20Enum :default "NewEnumerator0") (Score :type Integer))
  (bind _returnvalue (Actor|GetActorOfClass 0 "/Game/EyeSurgery/BluePrint/Object/Helpers/BP_ScoreManage.BP_ScoreManage_C"))
  (Default|RecordScore _returnvalue TaskName Score))