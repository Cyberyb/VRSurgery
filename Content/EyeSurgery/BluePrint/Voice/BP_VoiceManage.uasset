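; Voice manager actor for the eye surgery game that plays 2D voice clips for the current procedure stage.
; After a short delay at BeginPlay, it looks up the task in TaskManageRef's Level2NameMap and plays opening clips for lens pickup, pre-anesthesia, pre-surgery or post-surgery.
; PlayNextSound pauses any playing clip before starting and storing a new one, so voices never overlap; PauseCurSound pauses the current one.
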(event EventBeginPlay
  (bind _taskmanageref (Variables|Default|GetTaskManageRef))
  (Utilities|FlowControl|Delay 2.0)
  (Utilities|IsValid _taskmanageref
    (:Is%20Valid
      (switch name (.Value (Utilities|Map|Find (Variables|/Game/EyeSurgery/DataAssets/Task/BP_TaskManage.BP_TaskManage_C|GetLevel2NameMap _taskmanageref) (Variables|/Game/EyeSurgery/DataAssets/Task/BP_TaskManage.BP_TaskManage_C|GetTaskArrayPDA _taskmanageref)))
        (:人工晶状体领取
          (CallFunction|PlayNextSound "/Game/EyeSurgery/Sounds/人工晶状体准备/Step1/1.1_0"))
        (:麻醉前
          (CallFunction|PlayNextSound "/Game/EyeSurgery/Sounds/麻醉前安全核查/Step1/1.1"))
        (:手术前
          (CallFunction|PlayNextSound "/Game/EyeSurgery/Sounds/手术前安全核查/Step1/1.1")
          (Utilities|FlowControl|Delay 6.5)
          (CallFunction|PlayNextSound "/Game/EyeSurgery/Sounds/手术前安全核查/Step1/2.2"))
        (:手术后
          (CallFunction|PlayNextSound "/Game/EyeSurgery/Sounds/手术后安全核查/Step1/1.1"))))))

(event Collision|EventActorBeginOverlap
  (params (OtherActor :type Actor%20Object%20Reference)))

(event EventTick
  (params (DeltaSeconds :type Float%20%28single-precision%29)))

(fn ConstructionScript)

(fn PlayNextSound
  (params (Source :type Sound%20Base%20Object%20Reference))
  (Utilities|IsValid (Variables|Default|GetLastSound)
    (:Is%20Valid
      (if (Audio|Components|Audio|IsPlaying (Variables|Default|GetLastSound))
        (Class|AudioComponent|SetPaused (Variables|Default|GetLastSound) true)))
    (:Is%20Not%20Valid
      _))
  (Utilities|IsValid Source
    (:Is%20Valid
      (bind _returnvalue (Audio|CreateSound2D Source 1.0 1.0 0.0 0))
      (Audio|Components|Audio|Play _returnvalue 0.0)
      (bind _output_get (Variables|Default|SetLastSound _returnvalue))
      (return _output_get))))

(fn PauseCurSound
  (bind _lastsound (Variables|Default|GetLastSound))
  (Utilities|IsValid _lastsound
    (:Is%20Valid
      (if (Audio|Components|Audio|IsPlaying _lastsound)
        (Class|AudioComponent|SetPaused _lastsound true)))))