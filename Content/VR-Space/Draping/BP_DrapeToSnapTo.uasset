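; BP_DrapeToSnapTo is a snap target for drape pieces in the VR draping space, with its mesh and allowed connector IDs set at construction.
; When an actor attaches, it hides that actor and unhides itself, then calls SnapComplete with the connector ID if the actor is a BP_DrapeToSnap.
; Its anchor component reports attachment to the level's BP_DrapeManage, found at BeginPlay, using the target's first actor tag.
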(event ActorGotAttached(Comp_Anchor)
  (params (Anchor :type Comp%20Anchor%20Object%20Reference) (Actor :type Actor%20Object%20Reference) (Connector :type Comp%20Connector%20Anchor%20Object%20Reference))
  (Default|CallDrapeAttached (Variables|Default|GetDrapeManageRef) (Utilities|Array|Get(acopy) (Variables|Actor|GetTags))))

(event ActorAttached(Comp_Attach)
  (params (NewlyAttachedActor :type Actor%20Object%20Reference))
  (Rendering|SetActorHiddenInGame NewlyAttachedActor true)
  (Rendering|SetActorHiddenInGame false)
  (bind _asbp_drape_to_snap (Utilities|Casting|CastToBP_DrapeToSnap NewlyAttachedActor))
  (Default|CallSnapComplete (Variables|/Game/VR-Space/Draping/BP_DrapeToSnap.BP_DrapeToSnap_C|GetConnectorID _asbp_drape_to_snap)))

(event EventBeginPlay
  (bind _returnvalue (Actor|GetActorOfClass "/Game/EyeSurgery/BluePrint/Object/BP_DrapeManage.BP_DrapeManage_C"))
  (Utilities|IsValid _returnvalue
    (:Is%20Valid
      (Variables|Default|SetDrapeManageRef _returnvalue))))

(event Collision|EventActorBeginOverlap
  (params (OtherActor :type Actor%20Object%20Reference)))

(event EventTick
  (params (DeltaSeconds :type Float%20%28single-precision%29)))

(fn ConstructionScript
  (bind _drapemesh (Variables|Default|GetDrapeMesh)
    (:then
      (Components|StaticMesh|SetStaticMesh (Variables|Default|GetMesh) _drapemesh)
      (Variables|/Game/AFCore/Blueprints/Components/Snapping/Comp_Anchor.Comp_Anchor_C|SetConnectorIDsToAllow (Variables|Default|GetComp_Anchor) (Variables|Default|GetConnectorIDsToAllow)))
    (:else
      (Development|PrintString "DrapeToSnapTo has invalid mesh" true true "(R=1.000000,G=0.000000,B=0.084041,A=1.000000)"))))