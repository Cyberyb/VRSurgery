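; BP_DrapeToSnap is a drape actor in the VR draping area, set up for snapping through a connector anchor component.
; Its construction script applies the chosen drape mesh and passes the connector ID and search radius to the anchor, printing a warning if the mesh is invalid.
; On BeginPlay it finds and caches the task manager, then the voice manager, without using either in these graphs.
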(event EventBeginPlay
  (bind _returnvalue (Actor|GetActorOfClass "/Game/EyeSurgery/DataAssets/Task/BP_TaskManage.BP_TaskManage_C"))
  (Utilities|IsValid _returnvalue
    (:Is%20Valid
      (Variables|Default|SetTaskManageRef _returnvalue)
      (bind _returnvalue_2 (Actor|GetActorOfClass "/Game/EyeSurgery/BluePrint/Voice/BP_VoiceManage.BP_VoiceManage_C"))
      (Utilities|IsValid _returnvalue_2
        (:Is%20Valid
          (Variables|Default|SetVoiceManageRef _returnvalue_2))))))

(event Collision|EventActorBeginOverlap
  (params (OtherActor :type Actor%20Object%20Reference)))

(event EventTick
  (params (DeltaSeconds :type Float%20%28single-precision%29)))

(fn ConstructionScript
  (bind _drapemesh (Variables|Default|GetDrapeMesh)
    (:then
      (Components|StaticMesh|SetStaticMesh (Variables|Default|GetMesh) _drapemesh)
      (Variables|/Game/AFCore/Blueprints/Components/Snapping/Comp_Connector_Anchor.Comp_Connector_Anchor_C|SetConnectorID (Variables|Default|GetComp_Connector_Anchor) (Variables|Default|GetConnectorID))
      (Variables|/Game/AFCore/Blueprints/Components/Snapping/Comp_Connector_Anchor.Comp_Connector_Anchor_C|SetSearchRadius (Variables|Default|GetComp_Connector_Anchor) (Variables|Default|GetSearchRadius)))
    (:else
      (Development|PrintString "DrapeToSnap has invalid mesh" true true "(R=1.000000,G=0.000000,B=0.031421,A=1.000000)"))))