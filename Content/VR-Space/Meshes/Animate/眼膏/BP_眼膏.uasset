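; BP_眼膏 is a grabbable VR eye-ointment actor that drives a step of a voice-guided task.
; Comp_Grab plays a voice line through VoiceManageRef on pickup and tracks the trigger state in IsPressed.
; When its skeletal mesh begins overlapping BP_眼膏检测 with the trigger held, it reports the first task finished to TaskManageRef, then on success initializes the next task and plays another voice line.
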(event GrabKeyInput(Comp_Grab)
  (params (MComp :type BP%20M%20Comp%20Object%20Reference) (Key :type Enum_Controller_Buttons%20Enum :default "NewEnumerator1") (Set :type Boolean))
  (switch Utilities|FlowControl|Switch|SwitchonEnum_Controller_Buttons Key
    (:NewEnumerator0
      (Variables|Default|SetIsPressed Set))))

(event GrabActorPickedUp(Comp_Grab)
  (params (GrabbingPawn :type BP%20Pawn%20Base%20Object%20Reference) (GrabbingActor :type Actor%20Object%20Reference))
  (bind _voicemanageref (Variables|Default|GetVoiceManageRef)
    (:then
      (Default|PlayNextSound _voicemanageref "/Game/EyeSurgery/Sounds/手术后安全核查/Step1/2.2"))
    (:else)))

(event OnComponentBeginOverlap(SkeletalMeshComponent)
  (params (OverlappedComponent :type Primitive%20Component%20Object%20Reference) (OtherActor :type Actor%20Object%20Reference) (OtherComp :type Primitive%20Component%20Object%20Reference) (OtherBodyIndex :type Integer) (bFromSweep :type Boolean) (SweepResult :type Hit%20Result%20Structure%20%28by%20ref%29))
  (if (and (== (Utilities|GetClass OtherActor) "/Game/EyeSurgery/BluePrint/Object/Helpers/BP_眼膏检测.BP_眼膏检测_C") (Variables|Default|GetIsPressed))
    (bind _taskmanageref (Variables|Default|GetTaskManageRef)
      (:then
        (bind _isfinished (Default|TaskFinished _taskmanageref))
        (if _isfinished
          (Default|TaskInit _taskmanageref 1)
          (bind _voicemanageref (Variables|Default|GetVoiceManageRef)
            (:then
              (Default|PlayNextSound _voicemanageref "/Game/EyeSurgery/Sounds/手术后安全核查/Step2/1.1"))
            (:else))))
      (:else))))

(event EventBeginPlay)

(event Collision|EventActorBeginOverlap
  (params (OtherActor :type Actor%20Object%20Reference)))

(event EventTick
  (params (DeltaSeconds :type Float%20%28single-precision%29)))

(fn ConstructionScript)