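; BP_Eye_Charactor is an interactive character actor, apparently for a VR ophthalmology scene, with gaze and select components whose event handlers are still empty.
; On BeginPlay it caches the task and voice managers.
; SpawnPawnUI places widgets through the player pawn's Comp_PawnUI, replacing existing ones.
; SwitchByLevel looks up level number and name from the task manager's current task asset, but its event-graph call is unconnected.
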(event GazeTriggered(Comp_Gaze_Comp)
  (params (Pawn :type BP%20Pawn%20Base%20Object%20Reference) (ImpactLocation :type Vector :default "0, 0, 0") (Set :type Boolean))
  ;[1 1 1] 注视事件
)

(event PressedSelect(Comp_Select_Comp)
  (params (Pawn :type BP%20Pawn%20Base%20Object%20Reference) (SourceActor :type Actor%20Object%20Reference) (ImpactLocation :type Vector :default "0, 0, 0") (ImpactComponent :type Actor%20Component%20Object%20Reference))
  ;[1 1 1] 选择事件
)

(event EventBeginPlay
  (bind _returnvalue (Actor|GetActorOfClass "/Game/EyeSurgery/DataAssets/Task/BP_TaskManage.BP_TaskManage_C"))
  (Variables|任务管理|SetTaskManageRef _returnvalue)
  (bind _returnvalue_2 (Actor|GetActorOfClass "/Game/EyeSurgery/BluePrint/Voice/BP_VoiceManage.BP_VoiceManage_C"))
  (Variables|Default|SetVoiceManageRef _returnvalue_2))

(event Collision|EventActorBeginOverlap
  (params (OtherActor :type Actor%20Object%20Reference)))

(event EventTick
  (params (DeltaSeconds :type Float%20%28single-precision%29)))

(fn ConstructionScript)

(fn SpawnPawnUI
  (params (Widget :type Widget%20Base%20Class%20Reference) (Distance :type Enum_UI_Distance%20Enum :default "NewEnumerator0") (AddArcAngle :type Boolean) (ScaleParam :type Float%20%28double-precision%29))
  (bind _returnvalue (Game|Player|GetPlayerPawn 0))
  (bind _returnvalue_2 (Actor|GetComponentbyClass _returnvalue "/Game/AFCore/Blueprints/Components/UI/Comp_PawnUI.Comp_PawnUI_C"))
  (Utilities|IsValid _returnvalue_2
    (:Is%20Valid
      (Default|SpawnElement _returnvalue_2 Widget Distance true 0.0 AddArcAngle ScaleParam))
    (:Is%20Not%20Valid
      (Development|PrintText "Comp Pawn UI Not Valid"))))

(fn SwitchbyLevel
  (bind _taskmanageref (Variables|任务管理|GetTaskManageRef))
  (bind _taskarraypda (Variables|/Game/EyeSurgery/DataAssets/Task/BP_TaskManage.BP_TaskManage_C|GetTaskArrayPDA _taskmanageref))
  (bind _level2intmap (Variables|/Game/EyeSurgery/DataAssets/Task/BP_TaskManage.BP_TaskManage_C|GetLevel2IntMap _taskmanageref))
  (bind _level2namemap (Variables|/Game/EyeSurgery/DataAssets/Task/BP_TaskManage.BP_TaskManage_C|GetLevel2NameMap _taskmanageref))
  (bind (_value _returnvalue) (Utilities|Map|Find _level2namemap _taskarraypda))
  (bind (_value_2 _returnvalue_2) (Utilities|Map|Find _level2intmap _taskarraypda))
  (Utilities|IsValid _taskmanageref
    (:Is%20Valid
      (if (or _returnvalue_2 _returnvalue)
        (return _value_2 _value)))))