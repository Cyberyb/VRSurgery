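; BP_Capture is a scene-capture actor for render-target painting on the head of a BP_Patient.
; BeginPlay publishes capture size and unwrap location to MPC_Global, clears RT_Capture and creates a dynamic M_Unwrap material.
; PaintActor and the identical PaintOnStaticMesh temporarily swap in that material with brush location and radius, capture the unwrapped head with the body hidden, then restore it.
; GetUnwrapLocation returns a point just above the Background component.
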(event EventBeginPlay
  (Rendering|Material|SetScalarParameterValue "/Game/VR-Space/MeshPainting/MPC_Global.MPC_Global" "CaptureSize" (Variables|/Script/Engine.SceneCaptureComponent2D|GetOrthoWidth (Variables|Default|GetSceneCapture)) :!class /Script/Engine.KismetMaterialLibrary)
  (Rendering|Material|SetVectorParameterValue "/Game/VR-Space/MeshPainting/MPC_Global.MPC_Global" "UnwrapLocation" (Math|Conversions|ToLinearColor(Vector) (Transformation|GetWorldLocation (Variables|Default|GetDefaultSceneRoot))) :!class /Script/Engine.KismetMaterialLibrary)
  (Utilities|FlowControl|Delay 0.1)
  (Rendering|ClearRenderTarget2D "/Game/VR-Space/MeshPainting/RT_Capture.RT_Capture")
  (bind _returnvalue (Rendering|Material|CreateDynamicMaterialInstance "/Game/VR-Space/MeshPainting/M_Unwrap.M_Unwrap" "None" "None" :!class /Script/Engine.KismetMaterialLibrary))
  (Variables|Default|SetUnwrapMaterial _returnvalue))

(fn ConstructionScript)

(fn PaintActor
  (params (ActorToPaint :type Actor%20Object%20Reference) (PaintLocation :type Vector) (BrushRadius :type Float%20%28double-precision%29))
  ;[1 1 1] Validation, otherwise resulting runtime error
  (Utilities|IsValid (Variables|Default|GetUnwrapMaterial)
    (:Is%20Valid
      ;[1 1 1] Save head static mesh for later use
      (bind _asbp_patient (Utilities|Casting|CastToBP_Patient ActorToPaint))
      (LocalVariables|SetMesh (Variables|/Game/VR-Space/MeshPainting/BP_Patient.BP_Patient_C|GetHead _asbp_patient))
      (Utilities|FlowControl|Sequence
        (:then_0
          ;[1 1 1] Unwrap head
          (LocalVariables|SetOriginalMaterial (Rendering|Material|GetMaterial (LocalVariables|GetMesh) 0))
          (Rendering|Material|SetMaterial (LocalVariables|GetMesh) 0 (Variables|Default|GetUnwrapMaterial)))
        (:then_1
          ;[1 1 1] Setup Unwrap material with location to paint and brush radius
          (Rendering|Material|SetVectorParameterValue (Variables|Default|GetUnwrapMaterial) "PaintLocation" (Math|Conversions|ToLinearColor(Vector) PaintLocation) :!class /Script/Engine.MaterialInstanceDynamic)
          (Rendering|Material|SetScalarParameterValue (Variables|Default|GetUnwrapMaterial) "BrushRadius" BrushRadius :!class /Script/Engine.MaterialInstanceDynamic))
        (:then_2
          ;[1 1 1] Capture unwrapped material
          (bind _asbp_patient_2 (Utilities|Casting|CastToBP_Patient ActorToPaint))
          (Default|HideBody _asbp_patient_2)
          (Rendering|SceneCapture|CaptureScene (Variables|Default|GetSceneCapture) :!class /Script/Engine.SceneCaptureComponent2D)
          (bind _asbp_patient_3 (Utilities|Casting|CastToBP_Patient ActorToPaint))
          (Default|ShowBody _asbp_patient_3))
        (:then_3
          ;[1 1 1] Back to original material
          (Rendering|Material|SetMaterial (LocalVariables|GetMesh) 0 (LocalVariables|GetOriginalMaterial)))))))

(fn PaintonStaticMesh
  (params (ActorToPaint :type Actor%20Object%20Reference) (PaintLocation :type Vector) (BrushRadius :type Float%20%28double-precision%29))
  ;[1 1 1] Validation, otherwise resulting runtime error
  (Utilities|IsValid (Variables|Default|GetUnwrapMaterial)
    (:Is%20Valid
      ;[1 1 1] Save head static mesh for later use
      (bind _asbp_patient (Utilities|Casting|CastToBP_Patient ActorToPaint))
      (LocalVariables|SetMesh (Variables|/Game/VR-Space/MeshPainting/BP_Patient.BP_Patient_C|GetHead _asbp_patient))
      (Utilities|FlowControl|Sequence
        (:then_0
          ;[1 1 1] Unwrap head
          (LocalVariables|SetOriginalMaterial (Rendering|Material|GetMaterial (LocalVariables|GetMesh) 0))
          (Rendering|Material|SetMaterial (LocalVariables|GetMesh) 0 (Variables|Default|GetUnwrapMaterial)))
        (:then_1
          ;[1 1 1] Setup Unwrap material with location to paint and brush radius
          (Rendering|Material|SetVectorParameterValue (Variables|Default|GetUnwrapMaterial) "PaintLocation" (Math|Conversions|ToLinearColor(Vector) PaintLocation) :!class /Script/Engine.MaterialInstanceDynamic)
          (Rendering|Material|SetScalarParameterValue (Variables|Default|GetUnwrapMaterial) "BrushRadius" BrushRadius :!class /Script/Engine.MaterialInstanceDynamic))
        (:then_2
          ;[1 1 1] Capture unwrapped material
          (bind _asbp_patient_2 (Utilities|Casting|CastToBP_Patient ActorToPaint))
          (Default|HideBody _asbp_patient_2)
          (Rendering|SceneCapture|CaptureScene (Variables|Default|GetSceneCapture) :!class /Script/Engine.SceneCaptureComponent2D)
          (bind _asbp_patient_3 (Utilities|Casting|CastToBP_Patient ActorToPaint))
          (Default|ShowBody _asbp_patient_3))
        (:then_3
          ;[1 1 1] Back to original material
          (Rendering|Material|SetMaterial (LocalVariables|GetMesh) 0 (LocalVariables|GetOriginalMaterial)))))))

(fn GetUnwrapLocation
  (return (+ (Transformation|GetWorldLocation (Variables|Default|GetBackground)) "0,0,1.000000")))