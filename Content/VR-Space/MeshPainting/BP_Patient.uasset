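; BP_Patient is a VR mesh-painting patient actor with separate head, hair, hands and clothes components.
; HideBody and ShowBody toggle hair, hands and clothes visibility, leaving the head untouched.
; Two material functions clear the RT_Capture render target to black and swap the head to a first or second blend material, resetting paint between passes.
; A head hit event only prints a debug string.
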(event OnComponentHit(Head)
  (params (HitComponent :type Primitive%20Component%20Object%20Reference) (OtherActor :type Actor%20Object%20Reference) (OtherComp :type Primitive%20Component%20Object%20Reference) (NormalImpulse :type Vector :default "0, 0, 0") (Hit :type Hit%20Result%20Structure%20%28by%20ref%29))
  (Development|PrintString "Head Hit"))

(event EventBeginPlay)

(event Collision|EventActorBeginOverlap
  (params (OtherActor :type Actor%20Object%20Reference)))

(event EventTick
  (params (DeltaSeconds :type Float%20%28single-precision%29)))

(fn ConstructionScript)

(fn HideBody
  (Rendering|SetVisibility (Variables|Default|GetHair) false false)
  (Rendering|SetVisibility (Variables|Default|GetHands) false false)
  (Rendering|SetVisibility (Variables|Default|GetClothes) false false))

(fn ShowBody
  (Rendering|SetVisibility (Variables|Default|GetHair) true false)
  (Rendering|SetVisibility (Variables|Default|GetHands) true false)
  (Rendering|SetVisibility (Variables|Default|GetClothes) true false))

(fn SetMaterialforFirstPaint
  (Rendering|ClearRenderTarget2D "/Game/VR-Space/MeshPainting/RT_Capture.RT_Capture")
  (Rendering|Material|SetMaterial (Variables|Default|GetHead) 0 "/Game/VR-Space/MeshPainting/MI_HeadBlend1.MI_HeadBlend1"))

(fn SetMaterialforSecondPaint
  (Rendering|ClearRenderTarget2D "/Game/VR-Space/MeshPainting/RT_Capture.RT_Capture")
  (Rendering|Material|SetMaterial (Variables|Default|GetHead) 0 "/Game/VR-Space/MeshPainting/MI_HeadBlend2.MI_HeadBlend2"))