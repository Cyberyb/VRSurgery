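; BP_Painter is a grabbable VR cotton swab (棉签1 or 棉签2) that paints onto ActorToPaint during an eye-ointment task.
; While Sphere1 overlaps BP_眼膏检测, Tick has Capture paint at the sphere's center, using its radius as brush size.
; Pickup plays a voice line for the first swab or switches the target to its second-paint material for the second.
; Anchor reattachment completes that swab's task, starting the next task and voice line.
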(event GrabKeyInput(Comp_Grab)
  (params (MComp :type BP%20M%20Comp%20Object%20Reference) (Key :type Enum_Controller_Buttons%20Enum :default "NewEnumerator1") (Set :type Boolean))
  ;[1 1 1] Trigger键启用
  (switch Utilities|FlowControl|Switch|SwitchonEnum_Controller_Buttons Key
    (:NewEnumerator0
      (switch Utilities|FlowControl|Switch|SwitchonEnum_Side (Variables|/Game/AFCore/Blueprints/VR/MotionComponents/BP_MComp.BP_MComp_C|GetSide MComp)))))

(event OnComponentBeginOverlap(Sphere1)
  (params (OverlappedComponent :type Primitive%20Component%20Object%20Reference) (OtherActor :type Actor%20Object%20Reference) (OtherComp :type Primitive%20Component%20Object%20Reference) (OtherBodyIndex :type Integer) (bFromSweep :type Boolean) (SweepResult :type Hit%20Result%20Structure%20%28by%20ref%29))
  ;[1 1 1] 重叠启用绘图
  (if (== (Utilities|GetClass OtherActor) "/Game/EyeSurgery/BluePrint/Object/BP_眼膏检测.BP_眼膏检测_C")
    (Variables|Default|SetOverlapping true)))

(event GrabActorPickedUp(Comp_Grab)
  (params (GrabbingPawn :type BP%20Pawn%20Base%20Object%20Reference) (GrabbingActor :type Actor%20Object%20Reference))
  ;[1 1 1] 选择第一根棉签时触发语音，第二根棉签时切换Second Paint
  (switch name (Variables|Default|GetPainterTag)
    (:棉签1
      (Default|PlayNextSound (Variables|Default|GetVoiceManageRef) "/Game/EyeSurgery/Sounds/消毒铺巾/Step1/2.2"))
    (:棉签2
      (bind _actortopaint (Variables|Default|GetActorToPaint)
        (:then
          (Default|SetMaterialforSecondPaint _actortopaint))
        (:else)))))

(event OnComponentEndOverlap(Sphere1)
  (params (OverlappedComponent :type Primitive%20Component%20Object%20Reference) (OtherActor :type Actor%20Object%20Reference) (OtherComp :type Primitive%20Component%20Object%20Reference) (OtherBodyIndex :type Integer))
  ;[1 1 1] 重叠启用绘图
  (if (== (Utilities|GetClass OtherActor) "/Game/EyeSurgery/BluePrint/Object/BP_眼膏检测.BP_眼膏检测_C")
    (Variables|Default|SetOverlapping false)))

(event ConnectorAttached(Comp_Connector_Anchor)
  (params (Connector :type Comp%20Connector%20Object%20Reference) (AttachedToActor :type Actor%20Object%20Reference) (AttachedToComponent :type Scene%20Component%20Object%20Reference))
  (bind _voicemanageref (Variables|Default|GetVoiceManageRef))
  ;[1 1 1] 放回棉签时完成任务
  (bind _returnvalue (Actor|GetActorOfClass "/Game/EyeSurgery/DataAssets/Task/BP_TaskManage.BP_TaskManage_C"))
  (Utilities|IsValid _returnvalue
    (:Is%20Valid
      (switch name (Variables|Default|GetPainterTag)
        (:棉签1
          (bind _isfinished (Default|TaskFinished _returnvalue))
          (if _isfinished
            (Default|TaskInit _returnvalue 1)
            (Default|PlayNextSound _voicemanageref "/Game/EyeSurgery/Sounds/消毒铺巾/Step2/1.1")))
        (:棉签2
          (bind _isfinished_2 (Default|TaskFinished _returnvalue 1))
          (if _isfinished_2
            (Default|TaskInit _returnvalue 2)
            (Default|PlayNextSound _voicemanageref "/Game/EyeSurgery/Sounds/消毒铺巾/Step3/1.1")))))))

(event EventBeginPlay
  (bind _returnvalue (Actor|GetActorOfClass "/Game/EyeSurgery/BluePrint/Voice/BP_VoiceManage.BP_VoiceManage_C"))
  (Utilities|IsValid _returnvalue
    (:Is%20Valid
      (Variables|Default|SetVoiceManageRef _returnvalue))))

(event EventTick
  (params (DeltaSeconds :type Float%20%28single-precision%29))
  ;[1 1 1] 每帧调用画图
  (if (Variables|Default|GetOverlapping)
    (Utilities|IsValid (Variables|Default|GetCapture)
      (:Is%20Valid
        (Utilities|IsValid (Variables|Default|GetActorToPaint)
          (:Is%20Valid
            (Default|PaintActor (Variables|Default|GetCapture) (Variables|Default|GetActorToPaint) (CallFunction|GetPaintCenter) (Components|Sphere|GetScaledSphereRadius (Variables|Default|GetSphere1)))))))))

(fn ConstructionScript)

(fn GetPaintCenter
  (return (Transformation|GetWorldLocation (Variables|Default|GetSphere1))))