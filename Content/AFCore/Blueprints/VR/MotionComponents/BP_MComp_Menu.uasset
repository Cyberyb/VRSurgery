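; BP_MComp_Menu is a VR motion component that opens the tools menu for the VR pawn.
; It overrides the parent's FunctionInput event and reacts to the Tools Menu function.
; On that input it finds the pawn's Comp_PawnUI, checks it is valid, and has it spawn W_ToolsMenu, replacing any existing element.
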(event EventBeginPlay
  (|CallParentFunction) ; 此节点被禁用，将不会被调用。\n从引脚连出引线来编译功能。
)

(event Collision|EventActorBeginOverlap
  (params (OtherActor :type Actor%20Object%20Reference))
  (|CallParentFunction OtherActor) ; 此节点被禁用，将不会被调用。\n从引脚连出引线来编译功能。
)

(event EventTick
  (params (DeltaSeconds :type Float%20%28single-precision%29)))

(event EventFunctionInput
  (params (Function :type Name :default "None") (Set :type Boolean))
  (bind _vrpawn (Variables|Default|GetVRPawn))
  (bind _returnvalue (Actor|GetComponentbyClass _vrpawn "/Game/AFCore/Blueprints/Components/UI/Comp_PawnUI.Comp_PawnUI_C"))
  (|CallParentFunction Function Set)
  (switch name Function
    (:ToolsMenu
      (Utilities|IsValid _returnvalue
        (:Is%20Valid
          (Default|SpawnElement _returnvalue "/Game/EyeSurgery/BluePrint/Widget/W_ToolsMenu.W_ToolsMenu_C" "NewEnumerator0" true 0.0 false 1.0))))))

(fn ConstructionScript
  (|CallParentFunction))